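; Dialogue component that runs two-sided conversations between the player character and an owner character.
; StartDialogue resets the line index and broadcasts the times-dialogued count, leaving ReadDialogue to pick a conversation and show its lines in a lazily created widget.
; Portrait actors matched by character ID spawn far off at fixed coordinates, feed the widget and get talking flags.
; GoNext completes typing text or advances, ending the dialogue past the last line.
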(fn `CreatePortraitFromCharacterID`
  (params (CharacterID :type "/Game/GameElements/Blueprints/Characters/E_CharacterID Enum" :default "NewEnumerator0"))
  (returns (PortraitOutput :type "/Game/GameElements/Blueprints/Dialogue/BP_CharacterPortrait_Master Object Reference"))
  (switch `/Game/GameElements/Blueprints/Characters/E_CharacterID` CharacterID
    (:`NewEnumerator0`
      (bind _returnvalue (`|SpawnActorFromClass` "/Game/GameElements/Blueprints/Dialogue/BP_CharacterPortrait_Master.BP_CharacterPortrait_Master_C" (`KismetMathLibrary.MakeTransform` (9999.0 9999.0 0.0)) "AlwaysSpawn" "MultiplyWithRoot" null null))
      (return _returnvalue))
    (:`NewEnumerator1`
      (bind _returnvalue_2 (`|SpawnActorFromClass` "/Game/GameElements/Blueprints/Dialogue/BP_CharacterPortrait_Poichon.BP_CharacterPortrait_Poichon_C" (`KismetMathLibrary.MakeTransform` (9999.0 9999.0 0.0)) "AlwaysSpawn" "MultiplyWithRoot" null null))
      (return _returnvalue_2))
    (:`NewEnumerator2`
      (bind _returnvalue_3 (`|SpawnActorFromClass` "/Game/GameElements/Blueprints/Dialogue/BP_CharacterPortrait_Chapuccino.BP_CharacterPortrait_Chapuccino_C" (`KismetMathLibrary.MakeTransform` (9999.0 9999.0 0.0)) "AlwaysSpawn" "MultiplyWithRoot" null null))
      (return _returnvalue_3))
    (:`NewEnumerator3`
      (bind _returnvalue_4 (`|SpawnActorFromClass` "/Game/GameElements/Blueprints/Dialogue/BP_CharacterPortrait_Miwlk.BP_CharacterPortrait_Miwlk_C" (`KismetMathLibrary.MakeTransform` (9999.0 9999.0 0.0)) "AlwaysSpawn" "MultiplyWithRoot" null null))
      (return _returnvalue_4))))

(fn `EndDialogue`
  (bind _dialoguewidget (`self.DialogueWidget`))
  (`/Engine/EditorBlueprintResources/StandardMacros.IsValid` _dialoguewidget
    (:`Is Valid`
      (`Widget.RemoveFromParent` _dialoguewidget)
      (set `self.DialogueWidget` null)
      (`self.NullCurrentSpeaker`))
    (:`Is Not Valid`
      _))
  (`self.OnDialogueEnd`))

(fn `GoNext`
  (bind _wbp_dialoguebox (`/Game/GameElements/Blueprints/Dialogue/Widgets/WBP_Dialogue.WBP_DialogueBox` (`self.DialogueWidget`)))
  (if (`/Game/GameElements/Blueprints/Dialogue/Widgets/WBP_DialogueBox.IsTyping?` _wbp_dialoguebox)
    (`/Game/GameElements/Blueprints/Dialogue/Widgets/WBP_DialogueBox.ForceWriteText` _wbp_dialoguebox)
    (else
      (`self.ReadNextDialogueLine`))))

(fn `NullCurrentSpeaker`
  (set `/Game/GameElements/Blueprints/Dialogue/BP_CharacterPortrait_Master.IsTalking?` false (`self.OwnerPortrait`))
  (set `/Game/GameElements/Blueprints/Dialogue/BP_CharacterPortrait_Master.IsTalking?` false (`self.PlayerPortrait`)))

(fn `ReadDialogue`
  (params (DialogueIndexToRead :type Integer) (DialogueLineToReadIndex :type Integer))
  (bind (_player_ _dialogueline) (break `/Game/GameElements/Blueprints/Dialogue/F_DialogueLine` (`|GetArrayItem` (`.DialogueLines_3_12DFB60747F70F24EB2550A795904DD3` (break `/Game/GameElements/Blueprints/Dialogue/F_Dialogue` (`|GetArrayItem` (`self.Dialogues`) (`self.CurrentDialogueIndex`)))) (`self.CurrentDialogueLineIndex`))))
  (if (<= (+ DialogueIndexToRead 1) (`KismetArrayLibrary.Array_Length` (`self.Dialogues`)))
    (bind _output_get (set `self.CurrentDialogueIndex` DialogueIndexToRead))
    (if (<= (+ DialogueLineToReadIndex 1) (`KismetArrayLibrary.Array_Length` (`.DialogueLines_3_12DFB60747F70F24EB2550A795904DD3` (break `/Game/GameElements/Blueprints/Dialogue/F_Dialogue` (`|GetArrayItem` (`self.Dialogues`) _output_get)))))
      (bind _output_get_2 (set `self.CurrentDialogueLineIndex` DialogueLineToReadIndex))
      (if (== _output_get_2 0)
        (bind _dialoguewidget (`self.VerifyDialogueWidgetInstance`))
        (bind _wbp_dialoguebox (`/Game/GameElements/Blueprints/Dialogue/Widgets/WBP_Dialogue.WBP_DialogueBox` _dialoguewidget))
        (`/Game/GameElements/Blueprints/Dialogue/Widgets/WBP_DialogueBox.InitializeCharacterNames` _wbp_dialoguebox (`self.PlayerCharacter`) (`self.OwnerCharacter`) _player_)
        (`self.SetCurrentSpeaker` _player_)
        (if _player_
          (`/Game/GameElements/Blueprints/Dialogue/Widgets/WBP_DialogueBox.ReadDialogueText` _wbp_dialoguebox (`KismetTextLibrary.Conv_TextToString` _dialogueline) (`self.PlayerCharacter`))
          (else
            (`/Game/GameElements/Blueprints/Dialogue/Widgets/WBP_DialogueBox.ReadDialogueText` _wbp_dialoguebox (`KismetTextLibrary.Conv_TextToString` _dialogueline) (`self.OwnerCharacter`))))
        (else
          (bind _dialoguewidget_2 (`self.VerifyDialogueWidgetInstance`))
          (bind _wbp_dialoguebox_2 (`/Game/GameElements/Blueprints/Dialogue/Widgets/WBP_Dialogue.WBP_DialogueBox` _dialoguewidget_2))
          (`/Game/GameElements/Blueprints/Dialogue/Widgets/WBP_DialogueBox.ToggleCharacterName` _wbp_dialoguebox_2 _player_)
          (`self.SetCurrentSpeaker` _player_)
          (if _player_
            (`/Game/GameElements/Blueprints/Dialogue/Widgets/WBP_DialogueBox.ReadDialogueText` _wbp_dialoguebox_2 (`KismetTextLibrary.Conv_TextToString` _dialogueline) (`self.PlayerCharacter`))
            (else
              (`/Game/GameElements/Blueprints/Dialogue/Widgets/WBP_DialogueBox.ReadDialogueText` _wbp_dialoguebox_2 (`KismetTextLibrary.Conv_TextToString` _dialogueline) (`self.OwnerCharacter`))))))
      (else
        (`self.EndDialogue`)))
    (else
      (`self.EndDialogue`))))

(fn `ReadNextDialogueLine`
  (`self.ReadDialogue` (`self.CurrentDialogueIndex`) (+ (`self.CurrentDialogueLineIndex`) 1)))

(fn `SetCurrentSpeaker`
  (params (`PlayerSpeaking?` :type Boolean))
  (if `PlayerSpeaking?`
    (set `/Game/GameElements/Blueprints/Dialogue/BP_CharacterPortrait_Master.IsTalking?` true (`self.PlayerPortrait`))
    (else
      (set `/Game/GameElements/Blueprints/Dialogue/BP_CharacterPortrait_Master.IsTalking?` true (`self.OwnerPortrait`)))))

(fn `StartDialogue`
  (params (PlayerCharacter :type "/Game/GameElements/Blueprints/Characters/E_CharacterID Enum" :default "NewEnumerator0"))
  (bind _numberoftimesdialogued (`self.NumberOfTimesDialogued`))
  (if (> (`KismetArrayLibrary.Array_Length` (`self.Dialogues`)) 0)
    (bind _output_get (set `self.PlayerCharacter` PlayerCharacter))
    (set `self.CurrentDialogueLineIndex` 0)
    (`self.OnDialogueStart` _numberoftimesdialogued _output_get)
    (`/Engine/EditorBlueprintResources/StandardMacros.IncrementInt` _numberoftimesdialogued)))

(fn `VerifyDialogueWidgetInstance`
  (returns (DialogueWidget :type "/Game/GameElements/Blueprints/Dialogue/Widgets/WBP_Dialogue Object Reference"))
  (bind _dialoguewidget (`self.DialogueWidget`))
  (if (`KismetSystemLibrary.IsValid` _dialoguewidget)
    (return _dialoguewidget)
    (else
      (bind _returnvalue (`|CreateWidget` "/Game/GameElements/Blueprints/Dialogue/Widgets/WBP_Dialogue.WBP_Dialogue_C"))
      (bind _output_get (set `self.DialogueWidget` _returnvalue))
      (`UserWidget.AddToViewport` _output_get 0)
      (bind _portraitoutput (`self.CreatePortraitFromCharacterID` (`self.OwnerCharacter`)))
      (`/Game/GameElements/Blueprints/Dialogue/Widgets/WBP_CharacterPortrait.AssignPortrait` (`/Game/GameElements/Blueprints/Dialogue/Widgets/WBP_Dialogue.WBP_OwnerPortrait` _output_get) _portraitoutput true)
      (set `self.OwnerPortrait` _portraitoutput)
      (bind _portraitoutput_2 (`self.CreatePortraitFromCharacterID` (`self.PlayerCharacter`)))
      (`/Game/GameElements/Blueprints/Dialogue/Widgets/WBP_CharacterPortrait.AssignPortrait` (`/Game/GameElements/Blueprints/Dialogue/Widgets/WBP_Dialogue.WBP_PlayerPortrait` _output_get) _portraitoutput_2 false)
      (set `self.PlayerPortrait` _portraitoutput_2)
      (return _output_get))))