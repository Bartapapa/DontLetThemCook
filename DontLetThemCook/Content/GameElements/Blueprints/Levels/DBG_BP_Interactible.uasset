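; DBG_BP_Interactible is a debug actor for exercising the ACInteractible interaction component.
; On BeginPlay it binds handlers to the component's interaction started and ended events.
; When an interaction starts, a custom event prints the actor's name, waits briefly, then calls EndInteract on the component.
; The ended handler is an empty stub.
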(event `self.ReceiveBeginPlay`
  (bind _ac_interactible (`self.AC_Interactible`))
  (add `/Game/GameElements/Blueprints/Levels/AC_Interactible.OnInteractionStarted` _ac_interactible (`|CreateDelegate` :!event `On Interaction Started`))
  (add `/Game/GameElements/Blueprints/Levels/AC_Interactible.OnInteractionEnded` _ac_interactible (`|CreateDelegate` :!event `On Interaction Ended`)))

(event `InteractionEvent`
  (`KismetSystemLibrary.PrintString` (`KismetStringLibrary.Concat_StrStr` (`KismetSystemLibrary.GetDisplayName` self) " was interacted with!"))
  (`KismetSystemLibrary.Delay` 1.0)
  (`/Game/GameElements/Blueprints/Levels/AC_Interactible.EndInteract` (`self.AC_Interactible`)))

(fn `On Interaction Ended`
  (params (Interactible :type "/Game/GameElements/Blueprints/Levels/AC_Interactible Object Reference") (Interactor :type "/Game/GameElements/Blueprints/Characters/AC_Interactor Object Reference")))

(fn `On Interaction Started`
  (params (Interactible :type "/Game/GameElements/Blueprints/Levels/AC_Interactible Object Reference") (Interactor :type "/Game/GameElements/Blueprints/Characters/AC_Interactor Object Reference"))
  (`self.InteractionEvent`))

(fn `UserConstructionScript`)