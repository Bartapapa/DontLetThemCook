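; Groom character at a desk in the Lobby level that can turn around and later slide out of view.
; TurnAround sets a state in which Tick eases the yaw toward a target angle until a timer clears it.
; Despawn_SlideAway runs once, using a timeline to accumulate vertical offsets on the actor's current location, then hides the groom mesh when finished.
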(event `self.ReceiveBeginPlay`
  (bind (_returnvalue_x _returnvalue_y _returnvalue_z) (`KismetMathLibrary.BreakVector` (`self.K2_GetActorLocation`)))
  (set `self.ZPos` _returnvalue_z))

(event `self.ReceiveTick`
  (params (DeltaSeconds :type "Float (single-precision)"))
  (bind (_returnvalue_roll _returnvalue_pitch) (`KismetMathLibrary.BreakRotator` (`self.K2_GetActorRotation`)))
  (switch `int` (`self.State`)
    (:`1`
      (`self.K2_SetActorRotation` (`KismetMathLibrary.RInterpTo` (`self.K2_GetActorRotation`) (`KismetMathLibrary.MakeRotator` _returnvalue_roll _returnvalue_pitch (`self.ToYawRotTurnAround`)) (`GameplayStatics.GetWorldDeltaSeconds`) 1.0)))))

(event `TurnAround`
  (set `self.State` 1)
  (`KismetSystemLibrary.K2_SetTimerDelegate` (delegate `StopTurnAround`) 4.0))

(event `StopTurnAround`
  (set `self.State` 0))

(event `Despawn_SlideAway`
  (bind (_returnvalue_x _returnvalue_y _returnvalue_z) (`KismetMathLibrary.BreakVector` (`self.K2_GetActorLocation`)))
  (set `self.State` 2)
  (`/Engine/EditorBlueprintResources/StandardMacros.DoOnce` false
    (:`Completed`
      (bind (_direction _despawn) (`Timeline|Despawn`)
        (:`Update`
          (`self.K2_SetActorLocation` (`KismetMathLibrary.MakeVector` _returnvalue_x _returnvalue_y (+ _returnvalue_z (* (`self.DespawnZPos`) (- 1.0 _despawn))))))
        (:`Finished`
          (`SceneComponent.SetVisibility` (`self.GroomMesh`) false true))))))

(fn `UserConstructionScript`)