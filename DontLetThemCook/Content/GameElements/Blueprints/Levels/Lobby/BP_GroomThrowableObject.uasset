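; BP_GroomThrowableObject is a lobby prop that gets knocked away when a BP_Groom overlaps it.
; On overlap, it makes its mesh movable, enables physics, ignores the Pawn channel and applies a velocity-change impulse.
; The impulse points away from the top of the groom's capsule, scaling the unnormalized offset by a random force.
; The Thrown guard never becomes true because its setter is disconnected, so repeat overlaps throw it again.
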(event `self.ReceiveActorBeginOverlap`
  (params (OtherActor :type "Actor Object Reference"))
  (bind _objectmesh (`self.ObjectMesh`))
  (bind _asbp_groom (cast `/Game/GameElements/Blueprints/Enemies/BP_Groom` OtherActor))
  (`/Engine/EditorBlueprintResources/StandardMacros.IsValid` _asbp_groom
    (:`Is Valid`
      (if (not (`self.Thrown?`))
        (`PrimitiveComponent.SetSimulatePhysics` _objectmesh true)
        (`SceneComponent.SetMobility` _objectmesh "Movable")
        (`PrimitiveComponent.SetCollisionResponseToChannel` (`self.ObjectMesh`) "ECC_Pawn" "ECR_Ignore")
        (`PrimitiveComponent.AddImpulse` _objectmesh (* (- (`self.K2_GetActorLocation`) (+ (`self.K2_GetActorLocation` _asbp_groom) (`KismetMathLibrary.MakeVector` 0.0 0.0 (`CapsuleComponent.GetScaledCapsuleHalfHeight` (`Character.CapsuleComponent` _asbp_groom))))) (`KismetMathLibrary.RandomFloatInRange` (`self.ThrowForceMin`) (`self.ThrowForceMax`))) "None" true)))))

(fn `UserConstructionScript`)