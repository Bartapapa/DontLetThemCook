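; BP_ElevatorDoors is a lobby elevator door actor that slides two doors open and closes them automatically.
; BeginPlay caches both pivots' relative locations, and the OpenDoor timeline offsets them in opposite directions along local X, scaled by DoorOpenValue.
; OpenDoors plays the timeline and sets a timer for OpenDoorDuration, which fires CloseDoors to reverse it from the end.
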(event `self.ReceiveBeginPlay`
  (set `self.Door1Pos` (`SceneComponent.RelativeLocation` (`self.Pivot1`)))
  (set `self.Door2Pos` (`SceneComponent.RelativeLocation` (`self.Pivot2`))))

(event `CloseDoors`
  (bind (_direction _openvalue) (`Timeline|OpenDoor` :!via `ReverseFromEnd` :!label _label)
    (:`Update`
      (`SceneComponent.K2_SetRelativeLocation` (`self.Pivot2`) (+ (`self.Door2Pos`) (`KismetMathLibrary.MakeVector` (* _openvalue (* (`self.DoorOpenValue`) -1.0)))) false false)
      (`SceneComponent.K2_SetRelativeLocation` (`self.Pivot1`) (+ (`self.Door1Pos`) (`KismetMathLibrary.MakeVector` (* _openvalue (`self.DoorOpenValue`)))) false false))))

(event `OpenDoors`
  (`KismetSystemLibrary.K2_SetTimerDelegate` (delegate `CloseDoors`) (`self.OpenDoorDuration`))
  (goto _label))

(fn `UserConstructionScript`)