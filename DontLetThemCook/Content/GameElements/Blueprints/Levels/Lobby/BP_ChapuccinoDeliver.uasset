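; Lobby interactible that delivers the Chappuccino and kicks off the groom chase sequence.
; Interaction locks the player, dismisses the desk groom, plays a montage that hides the mesh on completion, zooms the camera and shows the acquire widget.
; After a fixed delay it ends the interaction and toggles on follow-up level triggers.
; Ending pulls the camera back and hands the player to ChaseGroom's spawn sequence without unlocking them here.
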(event `self.ReceiveBeginPlay`
  (bind _ac_interactible (`self.AC_Interactible`))
  (add `/Game/GameElements/Blueprints/Levels/AC_Interactible.OnInteractionStarted` _ac_interactible (`|CreateDelegate` :!event `On Interaction Started`))
  (add `/Game/GameElements/Blueprints/Levels/AC_Interactible.OnInteractionEnded` _ac_interactible (`|CreateDelegate` :!event `On Interaction Ended`))
  (add `/Game/GameElements/Blueprints/Levels/AC_Interactible.OnTogglePromptRequest` _ac_interactible (`|CreateDelegate` :!event `On Toggle Prompt Request`)))

(event `InteractionEvent`
  (bind _skeletalmesh (`self.SkeletalMesh`))
  (`KismetSystemLibrary.PrintString` (`KismetStringLibrary.Concat_StrStr` (`KismetSystemLibrary.GetDisplayName` self) " was interacted with!"))
  (`|PlayMontage` _skeletalmesh "/Game/GA/Character_GA/Final/AnimFBX/Poichon/A_Poichon_SwitchOut_Montage.A_Poichon_SwitchOut_Montage"
    (:`then`
      (bind _asbp_game_mode (cast `/Game/GameElements/Blueprints/GameMode/BP_GameMode` (`GameplayStatics.GetGameMode`)))
      (`/Game/GameElements/Blueprints/Camera/BP_CameraManager.ChangeCameraParameters` (`/Game/GameElements/Blueprints/GameMode/BP_GameMode.CameraManager` _asbp_game_mode) (0.0 0.0 0.0) 500.0 3.0)
      (`GameplayStatics.SpawnSound2D` "/Game/Sound/SoundFiles/freed_chappuccino.freed_chappuccino" 1.0 1.0 0.0 null)
      (bind _returnvalue (`|CreateWidget` "/Game/GameElements/Blueprints/UI/WBP_ChappuccinoAcquire.WBP_ChappuccinoAcquire_C"))
      (`UserWidget.AddToViewport` _returnvalue 0)
      (`/Game/GameElements/Blueprints/UI/WBP_ChappuccinoAcquire.PlayIntro` _returnvalue)
      (`KismetSystemLibrary.Delay` 7.0)
      (`/Game/GameElements/Blueprints/Levels/AC_Interactible.EndInteract` (`self.AC_Interactible`))
      (`/Game/GameElements/Blueprints/Levels/TBX_TriggerBoxMaster.ToggleTrigger` (`self.GroomFallTrigger`) true)
      (`/Game/GameElements/Blueprints/Levels/TBX_TriggerBoxMaster.ToggleTrigger` (`self.ElevatorSecondPassTrigger`) true)
      (`/Game/GameElements/Blueprints/Levels/TBX_TriggerBoxMaster.ToggleTrigger` (`self.LaundryGroom`) true))
    (:`OnCompleted`
      (`SceneComponent.SetVisibility` _skeletalmesh false true))))

(fn `On Interaction Ended`
  (params (Interactible :type "/Game/GameElements/Blueprints/Levels/AC_Interactible Object Reference") (Interactor :type "/Game/GameElements/Blueprints/Characters/AC_Interactor Object Reference"))
  (bind _asbp_game_mode (cast `/Game/GameElements/Blueprints/GameMode/BP_GameMode` (`GameplayStatics.GetGameMode`)))
  (`/Game/GameElements/Blueprints/Camera/BP_CameraManager.ChangeCameraParameters` (`/Game/GameElements/Blueprints/GameMode/BP_GameMode.CameraManager` _asbp_game_mode) (0.0 0.0 300.0) 1500.0 1.0)
  (bind _asbp_player_character_master (cast `/Game/GameElements/Blueprints/Characters/BP_PlayerCharacter_Master` (`ActorComponent.GetOwner` Interactor)))
  (`/Game/GameElements/Blueprints/Enemies/Groom/BP_Groom.SpawnSequence` (`self.ChaseGroom`) _asbp_player_character_master))

(fn `On Interaction Started`
  (params (Interactible :type "/Game/GameElements/Blueprints/Levels/AC_Interactible Object Reference") (Interactor :type "/Game/GameElements/Blueprints/Characters/AC_Interactor Object Reference"))
  (bind _asbp_player_character_master (cast `/Game/GameElements/Blueprints/Characters/BP_PlayerCharacter_Master` (`ActorComponent.GetOwner` Interactor))
    (:`then`
      (set `/Game/GameElements/Blueprints/Characters/BP_PlayerCharacter_Master.Lock_Character` true _asbp_player_character_master)
      (`/Game/GameElements/Blueprints/Levels/Lobby/BP_GroomAtDesk.Despawn_SlideAway` (`self.GroomAtDesk`))
      (`self.InteractionEvent`))
    (:`CastFailed`
      (`/Game/GameElements/Blueprints/Levels/AC_Interactible.EndInteract` (`self.AC_Interactible`)))))

(fn `On Toggle Prompt Request`
  (params (`Show?` :type Boolean))
  (`SceneComponent.SetVisibility` (`self.InteractionPrompt`) `Show?` true))

(fn `UserConstructionScript`)