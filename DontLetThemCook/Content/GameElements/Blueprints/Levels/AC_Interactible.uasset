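; AC_Interactible is an interactable component that manages the start and end of an interaction with an interactor.
; StartInteract stores the current interactor, disables it and broadcasts OnInteractionStarted with both parties.
; EndInteract re-enables that interactor, broadcasts OnInteractionEnded and then clears the stored reference.
; The event graph is empty, so behavior specific to each interaction is left to the dispatcher listeners.
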(fn `EndInteract`
  (set `/Game/GameElements/Blueprints/Characters/AC_Interactor.Disabled?` false (`self.CurrentInteractor`))
  (`self.OnInteractionEnded` self (`self.CurrentInteractor`))
  (set `self.CurrentInteractor` null))

(fn `StartInteract`
  (params (Interactor :type "/Game/GameElements/Blueprints/Characters/AC_Interactor Object Reference"))
  (bind _output_get (set `self.CurrentInteractor` Interactor))
  (set `/Game/GameElements/Blueprints/Characters/AC_Interactor.Disabled?` true _output_get)
  (`self.OnInteractionStarted` self _output_get))