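; BP_Miwlk is an interactable dialogue actor in the HUB that talks to the player character.
; Delegates from its interactible component toggle the prompt and, on interaction, pass the player's CharacterID to the dialoguer component to start dialogue.
; Dialogue start switches BP_GameMode into dialogue mode and reads the first line.
; Dialogue end leaves that mode and ends the interaction, whose callback resets the stored character.
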(event `self.ReceiveBeginPlay`
  (bind _ac_dialoguer (`self.AC_Dialoguer`))
  (bind _ac_interactible (`self.AC_Interactible`))
  (add `/Game/GameElements/Blueprints/Levels/AC_Interactible.OnInteractionStarted` _ac_interactible (`|CreateDelegate` :!event `On Interaction Started`))
  (add `/Game/GameElements/Blueprints/Levels/AC_Interactible.OnInteractionEnded` _ac_interactible (`|CreateDelegate` :!event `On Interaction Ended`))
  (add `/Game/GameElements/Blueprints/Levels/AC_Interactible.OnTogglePromptRequest` _ac_interactible (`|CreateDelegate` :!event `On Toggle Prompt Request`))
  (add `/Game/GameElements/Blueprints/Dialogue/AC_Dialoguer.OnDialogueStart` _ac_dialoguer (`|CreateDelegate` :!event `On Dialogue Start`))
  (add `/Game/GameElements/Blueprints/Dialogue/AC_Dialoguer.OnDialogueEnd` _ac_dialoguer (`|CreateDelegate` :!event `On Dialogue End`)))

(event `InteractionEvent`
  (bind _ac_dialoguer (`self.AC_Dialoguer`))
  (`KismetSystemLibrary.PrintString` (`KismetStringLibrary.Concat_StrStr` (`KismetSystemLibrary.GetDisplayName` self) " was interacted with!"))
  (`/Game/GameElements/Blueprints/Dialogue/AC_Dialoguer.StartDialogue` _ac_dialoguer (`/Game/GameElements/Blueprints/Dialogue/AC_Dialoguer.PlayerCharacter` _ac_dialoguer)))

(fn `On Dialogue End`
  (bind _asbp_game_mode (cast `/Game/GameElements/Blueprints/GameMode/BP_GameMode` (`GameplayStatics.GetGameMode`)))
  (`/Game/GameElements/Blueprints/GameMode/BP_GameMode.SetDialogueMode` _asbp_game_mode false (`self.AC_Dialoguer`))
  (`/Game/GameElements/Blueprints/Levels/AC_Interactible.EndInteract` (`self.AC_Interactible`)))

(fn `On Dialogue Start`
  (params (NumberOfTimesDialogueStarted :type Integer) (PlayerCharacter :type "/Game/GameElements/Blueprints/Characters/E_CharacterID Enum" :default "NewEnumerator0"))
  (bind _asbp_game_mode (cast `/Game/GameElements/Blueprints/GameMode/BP_GameMode` (`GameplayStatics.GetGameMode`))
    (:`then`
      (`/Game/GameElements/Blueprints/GameMode/BP_GameMode.SetDialogueMode` _asbp_game_mode true (`self.AC_Dialoguer`))
      (`/Game/GameElements/Blueprints/Dialogue/AC_Dialoguer.ReadDialogue` (`self.AC_Dialoguer`) 0 0))
    (:`CastFailed`
      (`/Game/GameElements/Blueprints/Dialogue/AC_Dialoguer.EndDialogue` (`self.AC_Dialoguer`)))))

(fn `On Interaction Ended`
  (params (Interactible :type "/Game/GameElements/Blueprints/Levels/AC_Interactible Object Reference") (Interactor :type "/Game/GameElements/Blueprints/Characters/AC_Interactor Object Reference"))
  (set `/Game/GameElements/Blueprints/Dialogue/AC_Dialoguer.PlayerCharacter` "NewEnumerator0" (`self.AC_Dialoguer`)))

(fn `On Interaction Started`
  (params (Interactible :type "/Game/GameElements/Blueprints/Levels/AC_Interactible Object Reference") (Interactor :type "/Game/GameElements/Blueprints/Characters/AC_Interactor Object Reference"))
  (bind _asbp_player_character_master (cast `/Game/GameElements/Blueprints/Characters/BP_PlayerCharacter_Master` (`ActorComponent.GetOwner` Interactor))
    (:`then`
      (set `/Game/GameElements/Blueprints/Dialogue/AC_Dialoguer.PlayerCharacter` (`/Game/GameElements/Blueprints/Characters/BP_PlayerCharacter_Master.CharacterID` _asbp_player_character_master) (`self.AC_Dialoguer`))
      (`self.InteractionEvent`))
    (:`CastFailed`
      (`/Game/GameElements/Blueprints/Levels/AC_Interactible.EndInteract` (`self.AC_Interactible`)))))

(fn `On Toggle Prompt Request`
  (params (`Show?` :type Boolean))
  (`SceneComponent.SetVisibility` (`self.InteractionPrompt`) `Show?` true))

(fn `UserConstructionScript`)