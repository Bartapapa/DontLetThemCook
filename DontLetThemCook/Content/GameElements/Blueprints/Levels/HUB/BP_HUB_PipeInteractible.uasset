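; BP_HUB_PipeInteractible is a pipe in the hub that sends the player to another level when interacted with.
; Interaction stores the spawn name and saves active character, party and health to the GameInstance.
; It then plays the character's switch animation, stops music, closes the scene through the main widget, deactivates the character and opens the target level after a short delay.
; A toggle event controls whether it can be interacted with.
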(event `self.ReceiveBeginPlay`
  (`parent.ReceiveBeginPlay`))

(event `ToggleCanBeInteracted`
  (params (`CanBeInteractedWith?` :type Boolean))
  (set `/Game/GameElements/Blueprints/Levels/AC_Interactible.CanBeInteractedWith?` `CanBeInteractedWith?` (`self.AC_Interactible`)))

(event `self.InteractionEvent`
  (bind _asgi_game_instance (cast `/Game/GameElements/Blueprints/GameMode/GI_GameInstance` (`GameplayStatics.GetGameInstance`)))
  (bind _asbp_game_mode (cast `/Game/GameElements/Blueprints/GameMode/BP_GameMode` (`GameplayStatics.GetGameMode`)))
  (set `/Game/GameElements/Blueprints/GameMode/GI_GameInstance.ToSpawnName` (`self.ToSpawnName`) _asgi_game_instance)
  (bind _currentactivecharacter (`/Game/GameElements/Blueprints/GameMode/BP_GameMode.CurrentActiveCharacter` _asbp_game_mode))
  (`/Game/GameElements/Blueprints/GameMode/GI_GameInstance.Save Data` _asgi_game_instance _currentactivecharacter (`/Game/GameElements/Blueprints/GameMode/BP_GameMode.PartyMembers` _asbp_game_mode) (`/Game/GameElements/Blueprints/Characters/AC_Health.CurrentHealth` (`self.GetComponentByClass` _asbp_game_mode "/Game/GameElements/Blueprints/Characters/AC_Health.AC_Health_C")))
  (`/Game/GameElements/Blueprints/Characters/BP_PlayerCharacter_Master.Anim_PlaySwitch` _currentactivecharacter)
  (bind _asbp_game_mode_2 (cast `/Game/GameElements/Blueprints/GameMode/BP_GameMode` (`GameplayStatics.GetGameMode`)))
  (`/Game/GameElements/Blueprints/GameMode/BP_GameMode.StopMusic` _asbp_game_mode_2 false)
  (`/Game/UI/Widget/Ingame/WG_MainWidget.CloseNewScene` (`/Game/GameElements/Blueprints/GameMode/BP_GameMode.WG_Main` _asbp_game_mode_2))
  ;[1 0 0] Deactivate Character
  ;;[1 0 0] J'arrive Pas A le trouver
  (`/Game/GameElements/Blueprints/Characters/BP_PlayerCharacter_Master.DeactivateCharacter` (`/Game/GameElements/Blueprints/GameMode/BP_GameMode.CurrentActiveCharacter` _asbp_game_mode_2))
  (`KismetSystemLibrary.Delay` 0.4)
  (`GameplayStatics.OpenLevel` (`self.ToLevel`)))

(fn `UserConstructionScript`
  (`parent.UserConstructionScript`))