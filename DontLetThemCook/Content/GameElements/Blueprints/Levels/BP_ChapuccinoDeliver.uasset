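; BP_ChapuccinoDeliver is an interactible cappuccino delivery spot that plays a short locked-camera moment when used.
; It binds to its ACInteractible component's start, end and prompt-toggle events, the last controlling prompt visibility.
; On use by the player, it locks the character, slides GroomAtDesk away, hides the cappuccino and zooms the game mode's CameraManager.
; After a fixed delay it ends the interaction, resetting the camera and unlocking the player.
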(event `self.ReceiveBeginPlay`
  (bind _ac_interactible (`self.AC_Interactible`))
  (add `/Game/GameElements/Blueprints/Levels/AC_Interactible.OnInteractionStarted` _ac_interactible (`|CreateDelegate` :!event `On Interaction Started`))
  (add `/Game/GameElements/Blueprints/Levels/AC_Interactible.OnInteractionEnded` _ac_interactible (`|CreateDelegate` :!event `On Interaction Ended`))
  (add `/Game/GameElements/Blueprints/Levels/AC_Interactible.OnTogglePromptRequest` _ac_interactible (`|CreateDelegate` :!event `On Toggle Prompt Request`)))

(event `InteractionEvent`
  (`KismetSystemLibrary.PrintString` (`KismetStringLibrary.Concat_StrStr` (`KismetSystemLibrary.GetDisplayName` self) " was interacted with!"))
  ;[1 1 1] Play release animation
  (`SceneComponent.SetVisibility` (`self.Chappucino`) false true)
  (bind _asbp_game_mode (cast `/Game/GameElements/Blueprints/GameMode/BP_GameMode` (`GameplayStatics.GetGameMode`)))
  (`/Game/GameElements/Blueprints/Camera/BP_CameraManager.ChangeCameraParameters` (`/Game/GameElements/Blueprints/GameMode/BP_GameMode.CameraManager` _asbp_game_mode) (0.0 0.0 0.0) 500.0 3.0)
  (`KismetSystemLibrary.Delay` 5.0)
  (`/Game/GameElements/Blueprints/Levels/AC_Interactible.EndInteract` (`self.AC_Interactible`)))

(fn `On Interaction Ended`
  (params (Interactible :type "/Game/GameElements/Blueprints/Levels/AC_Interactible Object Reference") (Interactor :type "/Game/GameElements/Blueprints/Characters/AC_Interactor Object Reference"))
  (bind _asbp_game_mode (cast `/Game/GameElements/Blueprints/GameMode/BP_GameMode` (`GameplayStatics.GetGameMode`)))
  (`/Game/GameElements/Blueprints/Camera/BP_CameraManager.ResetCameraParameters` (`/Game/GameElements/Blueprints/GameMode/BP_GameMode.CameraManager` _asbp_game_mode))
  (bind _asbp_player_character_master (cast `/Game/GameElements/Blueprints/Characters/BP_PlayerCharacter_Master` (`ActorComponent.GetOwner` Interactor)))
  (set `/Game/GameElements/Blueprints/Characters/BP_PlayerCharacter_Master.Lock_Character` false _asbp_player_character_master))

(fn `On Interaction Started`
  (params (Interactible :type "/Game/GameElements/Blueprints/Levels/AC_Interactible Object Reference") (Interactor :type "/Game/GameElements/Blueprints/Characters/AC_Interactor Object Reference"))
  (bind _asbp_player_character_master (cast `/Game/GameElements/Blueprints/Characters/BP_PlayerCharacter_Master` (`ActorComponent.GetOwner` Interactor))
    (:`then`
      (set `/Game/GameElements/Blueprints/Characters/BP_PlayerCharacter_Master.Lock_Character` true _asbp_player_character_master)
      (`/Game/GameElements/Blueprints/Levels/Lobby/BP_GroomAtDesk.Despawn_SlideAway` (`self.GroomAtDesk`))
      (`self.InteractionEvent`))
    (:`CastFailed`
      (`/Game/GameElements/Blueprints/Levels/AC_Interactible.EndInteract` (`self.AC_Interactible`)))))

(fn `On Toggle Prompt Request`
  (params (`Show?` :type Boolean))
  (`SceneComponent.SetVisibility` (`self.InteractionPrompt`) `Show?` true))

(fn `UserConstructionScript`)