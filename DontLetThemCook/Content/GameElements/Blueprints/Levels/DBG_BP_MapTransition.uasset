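; Level transition trigger actor that sends the player to the map named by ToLevel when the player character overlaps it.
; On overlap it saves the active character, party members and party health from BP_GameMode (health via its AC_Health component) into GI_GameInstance.
; It then calls CloseNewScene on the game mode's main widget and waits briefly before opening the level by name.
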(event `self.ReceiveActorBeginOverlap`
  (params (OtherActor :type "Actor Object Reference"))
  (bind _asbp_player_character_master (cast `/Game/GameElements/Blueprints/Characters/BP_PlayerCharacter_Master` OtherActor))
  (`/Engine/EditorBlueprintResources/StandardMacros.IsValid` _asbp_player_character_master
    (:`Is Valid`
      (bind _asgi_game_instance (cast `/Game/GameElements/Blueprints/GameMode/GI_GameInstance` (`GameplayStatics.GetGameInstance`)))
      (bind _asbp_game_mode (cast `/Game/GameElements/Blueprints/GameMode/BP_GameMode` (`GameplayStatics.GetGameMode`)))
      (`/Game/GameElements/Blueprints/GameMode/GI_GameInstance.Save Data` _asgi_game_instance (`/Game/GameElements/Blueprints/GameMode/BP_GameMode.CurrentActiveCharacter` _asbp_game_mode) (`/Game/GameElements/Blueprints/GameMode/BP_GameMode.PartyMembers` _asbp_game_mode) (`/Game/GameElements/Blueprints/Characters/AC_Health.CurrentHealth` (`self.GetComponentByClass` _asbp_game_mode "/Game/GameElements/Blueprints/Characters/AC_Health.AC_Health_C")))
      (bind _asbp_game_mode_2 (cast `/Game/GameElements/Blueprints/GameMode/BP_GameMode` (`GameplayStatics.GetGameMode`)))
      (`/Game/UI/Widget/Ingame/WG_MainWidget.CloseNewScene` (`/Game/GameElements/Blueprints/GameMode/BP_GameMode.WG_Main` _asbp_game_mode_2))
      (`KismetSystemLibrary.Delay` 0.4)
      (`GameplayStatics.OpenLevel` (`self.ToLevel`)))))

(fn `UserConstructionScript`)