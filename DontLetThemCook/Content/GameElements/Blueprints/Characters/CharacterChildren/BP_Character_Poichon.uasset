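; Playable character Poichon, a child of the base character class, whose special ability is a water spit.
; Overrides animation events to play montages; the spit montage's notify spawns a projectile toward the facing direction.
; Dynamic materials per mesh slot drive the stealth hue blend, hit-flash emissive and facing-dependent mustache, updated each tick.
; The victory dance stops music, locks the character, shows the kitchen-cleared widget and opens the credits level.
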(event `self.ReceiveTick`
  (params (DeltaSeconds :type "Float (single-precision)"))
  (`parent.ReceiveTick` DeltaSeconds)
  (`self.HandleMustacheTransparency`))

(event `self.Anim_PlayDash`
  (`|PlayMontage` (`self.Mesh`) "/Game/GA/Character_GA/Final/AnimFBX/Poichon/A_Poichon_DashStart_Montage.A_Poichon_DashStart_Montage"))

(event `self.Anim_PlayDoubleJump`
  (`|PlayMontage` (`self.Mesh`) "/Game/GA/Character_GA/Final/AnimFBX/Poichon/Poichon_FBX_Anim_Armature_Poichon_Jump_Start_Montage.Poichon_FBX_Anim_Armature_Poichon_Jump_Start_Montage" :!label _label))

(event `self.Anim_PlayDeath`
  (`|PlayMontage` (`self.Mesh`) "/Game/GA/Character_GA/Final/AnimFBX/Poichon/Poichon_FBX_Anim_Armature_Poichon_Death_Montage.Poichon_FBX_Anim_Armature_Poichon_Death_Montage"))

(event `self.Anim_PlayWallJump`
  (goto _label))

(event `self.Anim_PlayJump`
  (goto _label))

(event `self.Anim_PlayHurt`
  (`|PlayMontage` (`self.Mesh`) "/Game/GA/Character_GA/Final/AnimFBX/Poichon/Poichon_FBX_Anim_Armature_Poichon_Hurt_Montage.Poichon_FBX_Anim_Armature_Poichon_Hurt_Montage"))

(event `Anim_Spit`
  (bind _notifyname (`|PlayMontage` (`self.Mesh`) "/Game/GA/Character_GA/Final/AnimFBX/Poichon/A_Poichon_Spit_Montage.A_Poichon_Spit_Montage")
    (:`OnNotifyBegin`
      (if (== _notifyname "SpitProjectile")
        (`self.SpawnProjectile`)
        (`GameplayStatics.SpawnSound2D` "/Game/Sound/SoundFiles/Water_Spit_Cue.Water_Spit_Cue" 1.0 1.0 0.0 null)))))

(event `self.Anim_PlayInteract`
  (`|PlayMontage` (`self.Mesh`) "/Game/GA/Character_GA/Final/AnimFBX/Poichon/A_Poichon_Interact_Montage.A_Poichon_Interact_Montage"))

(event `self.Anim_PlayStartWallSlide`
  (`|PlayMontage` (`self.Mesh`) "/Game/GA/Character_GA/Final/AnimFBX/Poichon/Poichon_FBX_Anim_Armature_Poichon_WallSlide_Start_Montage.Poichon_FBX_Anim_Armature_Poichon_WallSlide_Start_Montage"))

(event `self.Anim_PlaySwitch`
  (`|PlayMontage` (`self.Mesh`) "/Game/GA/Character_GA/Final/AnimFBX/Poichon/A_Poichon_SwitchOut_Montage.A_Poichon_SwitchOut_Montage"))

(event `self.Anim_PlaySwitchInto`
  (`|PlayMontage` (`self.Mesh`) "/Game/GA/Character_GA/Final/AnimFBX/Poichon/A_Poichon_SwitchIn_Montage.A_Poichon_SwitchIn_Montage"))

(event `self.Anim_PlayDance`
  (bind _asbp_game_mode (cast `/Game/GameElements/Blueprints/GameMode/BP_GameMode` (`GameplayStatics.GetGameMode`)))
  (`/Game/GameElements/Blueprints/GameMode/BP_GameMode.StopMusic` _asbp_game_mode false)
  (`GameplayStatics.SpawnSound2D` "/Game/Sound/SoundFiles/VictoryDancel.VictoryDancel" 1.0 1.0 0.0 null)
  (`|PlayMontage` (`self.Mesh`) "/Game/GA/Character_GA/Final/AnimFBX/Poichon/A_Poichon_Dance_Montage.A_Poichon_Dance_Montage"
    (:`then`
      (set `self.Lock_Character` true))
    (:`OnCompleted`
      (bind _returnvalue (`|CreateWidget` "/Game/GameElements/Blueprints/UI/WBP_KitchenCleared.WBP_KitchenCleared_C"))
      (`UserWidget.AddToViewport` _returnvalue 0)
      (`/Game/GameElements/Blueprints/UI/WBP_KitchenCleared.PlayIntro` _returnvalue)
      (`UserWidget.BindToAnimationEvent` _returnvalue (`/Game/GameElements/Blueprints/UI/WBP_KitchenCleared.KitchenClearedOutro` _returnvalue) (delegate `LaunchCredits`) "Started" "None"))))

(event `self.Sound_OnSwitchInto`
  (`GameplayStatics.SpawnSound2D` "/Game/Sound/SoundFiles/Splash_1_Cue.Splash_1_Cue" 1.0 1.0 0.0 null)
  (`KismetSystemLibrary.PrintString` "Hello"))

(event `LaunchCredits`
  (`KismetSystemLibrary.Delay` 1.95)
  (`GameplayStatics.OpenLevel` "B3_07_Credit"))

(fn `CanCharacterDash?`
  (returns (`CanDash?` :type Boolean))
  (return (`parent.CanCharacterDash?`)))

(fn `HandleHitFlash`
  (bind _returnvalue (`KismetMathLibrary.Lerp` (`self.HitFlashIntensity`) 0.02 (/ (`KismetSystemLibrary.K2_GetTimerElapsedTimeHandle` (`self.HitFlashTimer`)) (`self.HitFlashTime`))))
  (`parent.HandleHitFlash`)
  (if (`self.IsCharacterInHitFlash?`)
    (`MaterialInstanceDynamic.SetScalarParameterValue` (`self.BodyMat`) "Emissive_Intensity" _returnvalue)
    (`MaterialInstanceDynamic.SetScalarParameterValue` (`self.MustacheMat`) "Emissive_Intensity" _returnvalue)
    (`MaterialInstanceDynamic.SetScalarParameterValue` (`self.REyeMat`) "Emissive_Intensity" _returnvalue)
    (`MaterialInstanceDynamic.SetScalarParameterValue` (`self.LEyeMat`) "Emissive_Intensity" _returnvalue)
    (else
      (`MaterialInstanceDynamic.SetScalarParameterValue` (`self.BodyMat`) "Emissive_Intensity" 0.02)
      (`MaterialInstanceDynamic.SetScalarParameterValue` (`self.MustacheMat`) "Emissive_Intensity" 0.02)
      (`MaterialInstanceDynamic.SetScalarParameterValue` (`self.REyeMat`) "Emissive_Intensity" 0.02)
      (`MaterialInstanceDynamic.SetScalarParameterValue` (`self.LEyeMat`) "Emissive_Intensity" 0.02))))

(fn `HandleMustacheTransparency`
  (`MaterialInstanceDynamic.SetScalarParameterValue` (`self.MustacheMat`) "MustacheRight?" (`KismetMathLibrary.Conv_BoolToDouble` (not (`self.FacingRight`)))))

(fn `HandleStealthMaterials`
  (bind _bodymat (`self.BodyMat`))
  (bind _bodymat_2 (`self.BodyMat`))
  (`parent.HandleStealthMaterials`)
  (if (`self.IsHidden?`)
    (bind _returnvalue (`MaterialInstanceDynamic.K2_GetVectorParameterValue` _bodymat_2 "Hue"))
    (`MaterialInstanceDynamic.SetVectorParameterValue` _bodymat_2 "Hue" (`KismetMathLibrary.CInterpTo` _returnvalue (`self.StealthHue`) (`GameplayStatics.GetWorldDeltaSeconds`) 5.0))
    (else
      (bind _returnvalue_2 (`MaterialInstanceDynamic.K2_GetVectorParameterValue` _bodymat "Hue"))
      (`MaterialInstanceDynamic.SetVectorParameterValue` _bodymat "Hue" (`KismetMathLibrary.CInterpTo` _returnvalue_2 (`self.UnstealthHue`) (`GameplayStatics.GetWorldDeltaSeconds`) 5.0)))))

(fn `InitializeMaterials`
  (bind _mesh (`self.Mesh`))
  (bind _mesh_2 (`self.Mesh`))
  (bind _mesh_3 (`self.Mesh`))
  (bind _mesh_4 (`self.Mesh`))
  (`parent.InitializeMaterials`)
  (bind _returnvalue (`PrimitiveComponent.CreateDynamicMaterialInstance` _mesh 0 (`PrimitiveComponent.GetMaterial` _mesh 0) "None"))
  (bind _output_get (set `self.BodyMat` _returnvalue))
  (`PrimitiveComponent.SetMaterial` (`self.Mesh`) 0 _output_get)
  (bind _returnvalue_2 (`PrimitiveComponent.CreateDynamicMaterialInstance` _mesh_3 1 (`PrimitiveComponent.GetMaterial` _mesh_3 1) "None"))
  (bind _output_get_2 (set `self.MustacheMat` _returnvalue_2))
  (`PrimitiveComponent.SetMaterial` (`self.Mesh`) 1 _output_get_2)
  (bind _returnvalue_3 (`PrimitiveComponent.CreateDynamicMaterialInstance` _mesh_4 2 (`PrimitiveComponent.GetMaterial` _mesh_4 2) "None"))
  (bind _output_get_3 (set `self.REyeMat` _returnvalue_3))
  (`PrimitiveComponent.SetMaterial` (`self.Mesh`) 2 _output_get_3)
  (bind _returnvalue_4 (`PrimitiveComponent.CreateDynamicMaterialInstance` _mesh_2 3 (`PrimitiveComponent.GetMaterial` _mesh_2 3) "None"))
  (bind _output_get_4 (set `self.LEyeMat` _returnvalue_4))
  (`PrimitiveComponent.SetMaterial` (`self.Mesh`) 3 _output_get_4))

(fn `SpawnProjectile`
  (locals (LocalDir :type "Float (double-precision)"))
  (if (>= (`KismetMathLibrary.Conv_BoolToDouble` (`self.FacingRight`)) 0.5)
    (set `local.LocalDir` 1.0)
    (else
      (set `local.LocalDir` -1.0)))
  (`|SpawnActorFromClass` "/Game/GameElements/Blueprints/Characters/BP_PoichonProjectile.BP_PoichonProjectile_C" (`KismetMathLibrary.MakeTransform` (+ (`self.K2_GetActorLocation`) (`KismetMathLibrary.MakeVector` 0.0 (* (`local.LocalDir`) 100.0)))) "Undefined" "MultiplyWithRoot" null (* (`self.PoichonProjectileSpeed`) (`local.LocalDir`)) self null))

(fn `SpecialAbilityEffect`
  (`parent.SpecialAbilityEffect`)
  (`KismetSystemLibrary.PrintString` "Used Poichon special!")
  (`self.Anim_Spit`)
  ;[1 1 1] Affiche utilisation Comp UI
  (`/Game/UI/Widget/Ingame/WG_MainWidget.UseAbilityEvent` (`/Game/GameElements/Blueprints/GameMode/BP_GameMode.WG_Main` (`self.GameMode`))))

(fn `UserConstructionScript`
  (`parent.UserConstructionScript`))