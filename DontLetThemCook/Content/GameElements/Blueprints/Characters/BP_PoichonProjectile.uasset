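; BP_PoichonProjectile is a projectile that flies along the world Y axis and triggers objects it hits.
; Each tick it moves by ProjectileSpeed, yaws to match its direction, then sphere-checks slightly behind its center.
; WorldStatic overlaps destroy it; otherwise, WorldDynamic actors with an interactible AC_PoichonProjectileInteractible component receive PoichonProjectileInteract and destroy it.
; Destruction spawns the NS_ProjectileImpact effect.
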(event `self.ReceiveTick`
  (params (DeltaSeconds :type "Float (single-precision)"))
  (`self.HandleProjectileMovement`))

(event `DestroyProjectile`
  (`NiagaraFunctionLibrary.SpawnSystemAtLocation` "/Game/TechArt/VFX/Crachat/NS_ProjectileImpact.NS_ProjectileImpact" (`self.K2_GetActorLocation`))
  (`self.K2_DestroyActor`))

(fn `HandleProjectileMovement`
  (bind _returnvalue (* (`self.ProjectileSpeed`) (`GameplayStatics.GetWorldDeltaSeconds`)))
  (`self.K2_SetActorLocationAndRotation` (+ (`self.K2_GetActorLocation`) (`KismetMathLibrary.MakeVector` 0.0 _returnvalue)) (`KismetMathLibrary.MakeRotator` 0.0 0.0 (* (`KismetMathLibrary.SignOfFloat` _returnvalue) 90.0)))
  (bind (_outactors _returnvalue_2) (`KismetSystemLibrary.SphereOverlapActors` (+ (`self.K2_GetActorLocation`) (* (`self.GetActorForwardVector`) -20.0)) 25.0 (`|MakeArray` "ObjectTypeQuery1" :!type "EObjectTypeQuery Enum")))
  (if _returnvalue_2
    (`self.DestroyProjectile`)
    (else
      (bind (_outactors_2 _returnvalue_3) (`KismetSystemLibrary.SphereOverlapActors` (+ (`self.K2_GetActorLocation`) (* (`self.GetActorForwardVector`) -20.0)) 25.0 (`|MakeArray` "ObjectTypeQuery2" :!type "EObjectTypeQuery Enum")))
      (if _returnvalue_3
        (for _array_element _outactors_2
          (bind _returnvalue_4 (`self.GetComponentByClass` _array_element "/Game/GameElements/Blueprints/Characters/AC_PoichonProjectileInteractible.AC_PoichonProjectileInteractible_C"))
          (`/Engine/EditorBlueprintResources/StandardMacros.IsValid` _returnvalue_4
            (:`Is Valid`
              (if (`/Game/GameElements/Blueprints/Characters/AC_PoichonProjectileInteractible.CanBeInteractedWith?` _returnvalue_4)
                (`/Game/GameElements/Blueprints/Characters/AC_PoichonProjectileInteractible.PoichonProjectileInteract` _returnvalue_4)
                (`self.DestroyProjectile`)))))))))

(fn `UserConstructionScript`)