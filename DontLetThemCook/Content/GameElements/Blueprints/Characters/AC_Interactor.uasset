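; Actor component that lets its owning character find and use nearby AC_Interactible components.
; Each tick, unless disabled, it sphere-overlaps around the owner, keeps interactibles that can be interacted with, and selects the closest.
; Selection changes move the on-screen prompt from the previous interactible to the new one.
; Interact starts interaction on the selected one and clears the selection, printing a debug message when disabled or without a valid target.
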(event `self.ReceiveTick`
  (params (DeltaSeconds :type "Float (single-precision)"))
  (if (not (`self.Disabled?`))
    (`self.SetSelectedInteractible` (`self.GetSelectedInteractible` (`self.GetAllPotentialInteractibles`)))))

(fn `CanInteract?`
  (returns (`CanInteract?` :type Boolean))
  (return (not (`self.Disabled?`))))

(fn `GetAllPotentialInteractibles`
  (returns (PotentialInteractibles :type "Array of /Game/GameElements/Blueprints/Levels/AC_Interactible Object Reference"))
  (locals (ConfirmedInteractibles :type "Array of /Game/GameElements/Blueprints/Levels/AC_Interactible Object Reference"))
  (bind _outactors (`KismetSystemLibrary.SphereOverlapActors` (`Actor.K2_GetActorLocation` (`self.GetOwner`)) (`self.InteractionDistance`) (`|MakeArray` "ObjectTypeQuery1" "ObjectTypeQuery2" "ObjectTypeQuery3" :!type "EObjectTypeQuery Enum")))
  (for _array_element _outactors
    (bind _returnvalue (`Actor.GetComponentByClass` _array_element "/Game/GameElements/Blueprints/Levels/AC_Interactible.AC_Interactible_C"))
    (if (`KismetSystemLibrary.IsValid` _returnvalue)
      (`KismetArrayLibrary.Array_AddUnique` (`local.ConfirmedInteractibles`) _returnvalue)))
  (return (`local.ConfirmedInteractibles`)))

(fn `GetSelectedInteractible`
  (params (PotentialInteractibles :type "Array of /Game/GameElements/Blueprints/Levels/AC_Interactible Object Reference"))
  (returns (SelectedInteractible :type "/Game/GameElements/Blueprints/Levels/AC_Interactible Object Reference"))
  (locals (ShortestDistance :type "Float (double-precision)" :default 999999.0) (AcceptedInteractibles :type "Array of /Game/GameElements/Blueprints/Levels/AC_Interactible Object Reference") (LocalSelectedInteractible :type "/Game/GameElements/Blueprints/Levels/AC_Interactible Object Reference"))
  (for _array_element PotentialInteractibles
    (if (`/Game/GameElements/Blueprints/Levels/AC_Interactible.CanBeInteractedWith?` _array_element)
      (`KismetArrayLibrary.Array_AddUnique` (`local.AcceptedInteractibles`) _array_element)))
  (for _array_element_2 (`local.AcceptedInteractibles`)
    (bind _returnvalue (`KismetMathLibrary.Vector_Distance` (`Actor.K2_GetActorLocation` (`self.GetOwner`)) (`Actor.K2_GetActorLocation` (`self.GetOwner` _array_element_2))))
    (if (< _returnvalue (`local.ShortestDistance`))
      (set `local.ShortestDistance` _returnvalue)
      (set `local.LocalSelectedInteractible` _array_element_2)))
  (return (`local.LocalSelectedInteractible`)))

(fn `Interact`
  (bind _selectedinteractible (`self.SelectedInteractible`))
  (if (`self.CanInteract?`)
    (`/Engine/EditorBlueprintResources/StandardMacros.IsValid` _selectedinteractible
      (:`Is Valid`
        (`/Game/GameElements/Blueprints/Levels/AC_Interactible.StartInteract` _selectedinteractible self)
        (`self.SetSelectedInteractible` null))
      (:`Is Not Valid`
        (`KismetSystemLibrary.PrintString` "No valid interactible." true true (struct :`R` 1.0 :`B` 0.103908 :`A` 1.0) 5.0)))
    (else
      (`KismetSystemLibrary.PrintString` "Character can't interact right now." true true (struct :`R` 1.0 :`B` 0.103908 :`A` 1.0) 5.0))))

(fn `SetSelectedInteractible`
  (params (SelectedInteractible :type "/Game/GameElements/Blueprints/Levels/AC_Interactible Object Reference"))
  (bind _selectedinteractible (`self.SelectedInteractible`))
  (`/Engine/EditorBlueprintResources/StandardMacros.IsValid` _selectedinteractible
    (:`Is Valid`
      (if (!= SelectedInteractible _selectedinteractible)
        (`/Game/GameElements/Blueprints/Levels/AC_Interactible.TogglePrompt` (`self.SelectedInteractible`) false)
        (bind _output_get (set `self.SelectedInteractible` SelectedInteractible :!label _label))
        (`/Engine/EditorBlueprintResources/StandardMacros.IsValid` _output_get
          (:`Is Valid`
            (`/Game/GameElements/Blueprints/Levels/AC_Interactible.TogglePrompt` _output_get true)))))
    (:`Is Not Valid`
      (goto _label))))