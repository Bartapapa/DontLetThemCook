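; Health component for characters that tracks current and max health and handles damage, healing and instant kill.
; Damage is rejected when dead, invulnerable, immune to the damage type or from the same Player or Enemy faction, while healing rejects the opposing faction.
; Both feed clamped decrease and increase functions that fire events for damage, resistance, healing and limits reached.
; Increasing from zero health adds nothing but still fires its event.
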(fn `Damage`
  (params (Source :type "Actor Object Reference") (Instigator :type "Actor Object Reference") (SourceFaction :type "/Game/GameElements/Blueprints/Characters/E_CharacterFactions Enum" :default "NewEnumerator0") (`Damage value` :type Integer) (DamageType :type "/Game/GameElements/Blueprints/Characters/E_DamageTypes Enum" :default "NewEnumerator0") (`Hitstun?` :type Boolean) (KnockbackForceMultiplier :type "Float (double-precision)"))
  (returns (`HasDamaged?` :type Boolean))
  (if (or (`self.IsDead?`) (`self.IsInvulnerable?`))
    (return false)
    (elif (< (`KismetArrayLibrary.Array_Find` (`self.DamageImmunities`) DamageType) 0)
      (switch `/Game/GameElements/Blueprints/Characters/E_CharacterFactions` (`self.CharacterFaction`)
        (:`NewEnumerator0`
          _)
        (:`NewEnumerator1`
          (switch `/Game/GameElements/Blueprints/Characters/E_CharacterFactions` SourceFaction
            (:`NewEnumerator0`
              _)
            (:`NewEnumerator1`
              (return false))
            (:`NewEnumerator2`
              _)))
        (:`NewEnumerator2`
          (switch `/Game/GameElements/Blueprints/Characters/E_CharacterFactions` SourceFaction
            (:`NewEnumerator0`
              _)
            (:`NewEnumerator1`
              _)
            (:`NewEnumerator2`
              (return false)))))
      (`self.DecreaseHealth` `Damage value`)
      (`self.OnHealthDamaged` Source Instigator `Damage value` `Hitstun?` KnockbackForceMultiplier)
      (return true)
      (else
        (`self.OnDamageResisted` DamageType)
        (return false)))))

(fn `DecreaseHealth`
  (params (HealthDecrease :type Integer))
  (if (> HealthDecrease 0)
    (bind _output_get (set `self.CurrentHealth` (- (`self.CurrentHealth`) HealthDecrease)))
    (if (<= _output_get 0)
      (set `self.CurrentHealth` 0)
      (`self.OnHealthReachedZero`))))

(fn `Heal`
  (params (HealValue :type Integer) (HealFaction :type "/Game/GameElements/Blueprints/Characters/E_CharacterFactions Enum" :default "NewEnumerator0"))
  (if (`self.IsDamaged?`)
    (switch `/Game/GameElements/Blueprints/Characters/E_CharacterFactions` (`self.CharacterFaction`)
      (:`NewEnumerator0`
        _)
      (:`NewEnumerator1`
        (switch `/Game/GameElements/Blueprints/Characters/E_CharacterFactions` HealFaction
          (:`NewEnumerator0`
            _)
          (:`NewEnumerator1`
            _)))
      (:`NewEnumerator2`
        (switch `/Game/GameElements/Blueprints/Characters/E_CharacterFactions` HealFaction
          (:`NewEnumerator0`
            _)
          (:`NewEnumerator2`
            _))))
    (`self.IncreaseHealth` HealValue)
    (`self.OnHealthHealed` HealValue)))

(fn `HealToMax`
  (`self.Heal` (- (`self.MaxHealth`) (`self.CurrentHealth`))))

(fn `IncreaseHealth`
  (params (HealthIncrease :type Integer))
  (if (> HealthIncrease 0)
    (if (<= (`self.CurrentHealth`) 0)
      (bind _output_get (set `self.CurrentHealth` (+ (`self.CurrentHealth`) 0)))
      (if (> _output_get (`self.MaxHealth`))
        (set `self.CurrentHealth` (`self.MaxHealth`))
        (`self.OnHealthReachedMax`))
      (`self.OnHealthIncreasedFromZero`)
      (else
        (bind _output_get_2 (set `self.CurrentHealth` (+ (`self.CurrentHealth`) HealthIncrease)))
        (if (> _output_get_2 (`self.MaxHealth`))
          (set `self.CurrentHealth` (`self.MaxHealth`))
          (`self.OnHealthReachedMax`))))))

(fn `InitializeHealth`
  (params (MaxHealth :type Integer))
  (bind _output_get (set `self.MaxHealth` MaxHealth))
  (set `self.CurrentHealth` _output_get))

(fn `InstantKill`
  (`self.Damage` null null "NewEnumerator0" (`self.CurrentHealth`)))

(fn `IsDamaged?`
  (returns (`IsDamaged?` :type Boolean))
  (return (< (`self.CurrentHealth`) (`self.MaxHealth`))))

(fn `IsDead?`
  (returns (`IsDead?` :type Boolean))
  (return (<= (`self.CurrentHealth`) 0)))

(fn `IsInvulnerable?`
  (returns (`IsInvulnerable?` :type Boolean))
  (return (`self.Invulnerable`)))