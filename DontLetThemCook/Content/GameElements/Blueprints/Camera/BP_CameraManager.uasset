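; Player-controlled side-scroller camera rig that registers with BP_GameMode and routes Enhanced Input to its active character, or Jump to the current dialoguer during dialogue.
; Each tick it follows the averaged position of that character and registered focus objects, unless an override object is set.
; Zoom-scaled facing look-ahead and grounded up/down look shift the unoverridden view.
; Other actors can change zoom and focus offset, which interpolate smoothly.
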(event `self.ReceiveBeginPlay`
  (bind _asplayer_controller (cast `PlayerController` (`self.GetController`)))
  (bind _returnvalue (pcsubsystem `EnhancedInputLocalPlayerSubsystem` _asplayer_controller))
  (`/Engine/EditorBlueprintResources/StandardMacros.IsValid` _returnvalue
    (:`Is Valid`
      (`EnhancedInputSubsystemInterface.AddMappingContext` _returnvalue "/Game/GameElements/Input/IMC_Default.IMC_Default" 0 (struct))
      (bind _asbp_game_mode (cast `/Game/GameElements/Blueprints/GameMode/BP_GameMode` (`GameplayStatics.GetGameMode`)))
      (bind _output_get (set `self.GameMode` _asbp_game_mode))
      (set `/Game/GameElements/Blueprints/GameMode/BP_GameMode.CameraManager` self _output_get)
      (`self.InitializeCamera`))))

(event `self.ReceiveTick`
  (params (DeltaSeconds :type "Float (single-precision)"))
  (`self.HandleCameraFocus`)
  (`self.HandleCameraZoom`)
  (`self.HandleCameraFocusOffset`))

(event `EnhancedInput|/Game/GameElements/Input/Actions/IA_Move`
  (params (ActionValue :type "Vector2D Structure") (ElapsedSeconds :type "Float (double-precision)") (TriggeredSeconds :type "Float (double-precision)") (InputAction :type "InputAction Object Reference" :default "/Game/GameElements/Input/Actions/IA_Move.IA_Move"))
  (bind _returnvalue (`KismetMathLibrary.SignOfFloat` ActionValue_Y))
  (bind _returnvalue_2 (`SceneComponent.GetRightVector` (`self.FollowCamera`)))
  (bind _currentactivecharacter (`/Game/GameElements/Blueprints/GameMode/BP_GameMode.CurrentActiveCharacter` (`self.GameMode`)))
  (bind _currentactivecharacter_2 (`/Game/GameElements/Blueprints/GameMode/BP_GameMode.CurrentActiveCharacter` (`self.GameMode`)))
  (:`Triggered`
    (if (and (>= (`KismetMathLibrary.Abs` ActionValue_Y) 0.75) (not (`/Game/GameElements/Blueprints/Characters/BP_PlayerCharacter_Master.Lock_Character` (`/Game/GameElements/Blueprints/GameMode/BP_GameMode.CurrentActiveCharacter` (`self.GameMode`)))))
      (if (`KismetSystemLibrary.IsValid` _currentactivecharacter_2)
        (if (`/Game/GameElements/Blueprints/Characters/BP_PlayerCharacter_Master.IsCharacterInAir?` _currentactivecharacter_2)
          (if (`KismetSystemLibrary.IsValid` _currentactivecharacter) :!label _label
            (if (> (`KismetMathLibrary.SignOfFloat` ActionValue_X) 0.0)
              (`/Game/GameElements/Blueprints/Characters/BP_PlayerCharacter_Master.Move` _currentactivecharacter ActionValue_X _returnvalue_2 true)
              (else
                (`/Game/GameElements/Blueprints/Characters/BP_PlayerCharacter_Master.Move` _currentactivecharacter ActionValue_X _returnvalue_2 false))))
          (else
            (set `self.LookUpDownValue` (* (`KismetMathLibrary.MapRangeClamped` ActionValue_Y (* 0.75 _returnvalue) (* 1.0 _returnvalue) 0.0 (* 1.0 _returnvalue)) (`self.LookUpDownStrength`)))))
        (else
          (goto _label)))
      (else
        (set `self.LookUpDownValue` 0.0)
        (goto _label))))
  (:`Completed`
    (set `self.LookUpDownValue` 0.0)))

(event `EnhancedInput|/Game/GameElements/Input/Actions/IA_Jump`
  (params (ActionValue :type Boolean) (ElapsedSeconds :type "Float (double-precision)") (TriggeredSeconds :type "Float (double-precision)") (InputAction :type "InputAction Object Reference" :default "/Game/GameElements/Input/Actions/IA_Jump.IA_Jump"))
  (bind _currentactivecharacter (`/Game/GameElements/Blueprints/GameMode/BP_GameMode.CurrentActiveCharacter` (`self.GameMode`)))
  (:`Started`
    (if (`self.InDialogue?`)
      (`/Game/GameElements/Blueprints/Dialogue/AC_Dialoguer.GoNext` (`self.CurrentDialoguer`))
      (else
        (`/Game/GameElements/Blueprints/Characters/BP_PlayerCharacter_Master.JumpRequest` _currentactivecharacter))))
  (:`Completed`
    (`/Game/GameElements/Blueprints/Characters/BP_PlayerCharacter_Master.JumpComplete` _currentactivecharacter)))

(event `SetDialogueMode`
  (params (DialogueMode :type Boolean) (Dialoguer :type "/Game/GameElements/Blueprints/Dialogue/AC_Dialoguer Object Reference"))
  (set `self.CurrentDialoguer` Dialoguer)
  (set `self.InDialogue?` DialogueMode)
  (set `/Game/GameElements/Blueprints/Characters/BP_PlayerCharacter_Master.Lock_Character` DialogueMode (`/Game/GameElements/Blueprints/GameMode/BP_GameMode.CurrentActiveCharacter` (`self.GameMode`))))

(event `EnhancedInput|/Game/GameElements/Input/Actions/IA_Dash`
  (params (ActionValue :type "Float (double-precision)") (ElapsedSeconds :type "Float (double-precision)") (TriggeredSeconds :type "Float (double-precision)") (InputAction :type "InputAction Object Reference" :default "/Game/GameElements/Input/Actions/IA_Dash.IA_Dash"))
  (bind _currentactivecharacter (`/Game/GameElements/Blueprints/GameMode/BP_GameMode.CurrentActiveCharacter` (`self.GameMode`)))
  (:`Triggered`
    (`/Game/GameElements/Blueprints/Characters/BP_PlayerCharacter_Master.DashRequest` _currentactivecharacter ActionValue))
  (:`Completed`
    (`/Game/GameElements/Blueprints/Characters/BP_PlayerCharacter_Master.DashComplete` _currentactivecharacter)))

(event `EnhancedInput|/Game/GameElements/Input/Actions/IA_Switch`
  (params (ActionValue :type "Float (double-precision)") (ElapsedSeconds :type "Float (double-precision)") (TriggeredSeconds :type "Float (double-precision)") (InputAction :type "InputAction Object Reference" :default "/Game/GameElements/Input/Actions/IA_Switch.IA_Switch"))
  (:`Started`
    (`/Game/GameElements/Blueprints/Characters/BP_PlayerCharacter_Master.SwitchRequest` (`/Game/GameElements/Blueprints/GameMode/BP_GameMode.CurrentActiveCharacter` (`self.GameMode`)) ActionValue)))

(event `EnhancedInput|/Game/GameElements/Input/Actions/IA_Interact`
  (params (ActionValue :type Boolean) (ElapsedSeconds :type "Float (double-precision)") (TriggeredSeconds :type "Float (double-precision)") (InputAction :type "InputAction Object Reference" :default "/Game/GameElements/Input/Actions/IA_Interact.IA_Interact"))
  (:`Started`
    (`/Game/GameElements/Blueprints/Characters/BP_PlayerCharacter_Master.InteractRequest` (`/Game/GameElements/Blueprints/GameMode/BP_GameMode.CurrentActiveCharacter` (`self.GameMode`)))))

(fn `AddCameraFocusObject`
  (params (FocusObject :type "Actor Object Reference"))
  (`KismetArrayLibrary.Array_AddUnique` (`self.FocusObjects`) FocusObject)
  (add `self.OnDestroyed` FocusObject (`|CreateDelegate` :!event `On Focus Object Destroyed`)))

(fn `ChangeCameraParameters`
  (params (FocusOffset :type "Vector Structure") (ToZoom :type "Float (double-precision)") (`Zoom Interpolation` :type "Float (double-precision)"))
  (`self.ZoomCamera` ToZoom `Zoom Interpolation`)
  (set `self.SecondaryFocusOffset` FocusOffset))

(fn `GetCameraLookForward`
  (returns (LookForwardValue :type "Float (double-precision)"))
  (bind _gamemode (`self.GameMode`))
  (bind _currentactivecharacter (`/Game/GameElements/Blueprints/GameMode/BP_GameMode.CurrentActiveCharacter` _gamemode))
  (if (`KismetSystemLibrary.IsValid` _gamemode)
    (if (`KismetSystemLibrary.IsValid` _currentactivecharacter)
      (if (`/Game/GameElements/Blueprints/Characters/BP_PlayerCharacter_Master.FacingRight` _currentactivecharacter)
        (return (* (`self.BaseCameraLookForward`) (`self.GetForwardValueMultiplier`)))
        (else
          (return (* (`self.BaseCameraLookForward`) -1.0 (`self.GetForwardValueMultiplier`)))))
      (else
        _)))
  (return 0.0))

(fn `GetFocusObjectsAveragePosition`
  (returns (AveragePosition :type "Vector Structure"))
  (locals (LocalAveragePosition :type "Vector Structure"))
  (bind _gamemode (`self.GameMode`))
  (bind _focusobjects (`self.FocusObjects`))
  (bind _currentactivecharacter (`/Game/GameElements/Blueprints/GameMode/BP_GameMode.CurrentActiveCharacter` _gamemode))
  (if (`KismetSystemLibrary.IsValid` _gamemode)
    (if (`KismetSystemLibrary.IsValid` _currentactivecharacter)
      (set `local.LocalAveragePosition` (`self.K2_GetActorLocation` _currentactivecharacter))
      (for _array_element _focusobjects
        (bind (_returnvalue_x _returnvalue_y _returnvalue_z) (`KismetMathLibrary.BreakVector` (`self.K2_GetActorLocation` _array_element)))
        (set `local.LocalAveragePosition` (+ (`local.LocalAveragePosition`) (`KismetMathLibrary.MakeVector` 0.0 _returnvalue_y _returnvalue_z))))
      (bind _output_get (set `local.LocalAveragePosition` (/ (`local.LocalAveragePosition`) (+ (`KismetArrayLibrary.Array_Length` _focusobjects) 1))))
      (return _output_get)
      (else
        _)))
  (return (0.0 0.0 0.0)))

(fn `GetForwardValueMultiplier`
  (returns (Multiplier :type "Float (double-precision)"))
  (return (/ (`self.ToZoom`) (`self.DefaultZoom`))))

(fn `HandleCameraFocus`
  (locals (LocalFocusPoint :type "Vector Structure") (TotalFocusOffset :type "Vector Structure") (CameraPosition :type "Vector Structure"))
  (bind (_returnvalue_x _returnvalue_y _returnvalue_z) (`KismetMathLibrary.BreakVector` (`self.K2_GetActorLocation` (`self.OverrideFocusObject`))))
  (set `local.CameraPosition` (`self.CurrentFocusOffset`))
  (if (`KismetSystemLibrary.IsValid` (`self.OverrideFocusObject`))
    (bind _output_get (set `local.CameraPosition` (+ (`local.CameraPosition`) (`KismetMathLibrary.MakeVector` 0.0 _returnvalue_y _returnvalue_z) (`self.OverrideFocusOffset`))))
    (`self.K2_SetActorLocation` _output_get)
    (else
      (bind _output_get_2 (set `self.CameraLookForwardValue` (`KismetMathLibrary.FInterpTo_Constant` (`self.CameraLookForwardValue`) (`self.GetCameraLookForward`) (`GameplayStatics.GetWorldDeltaSeconds`) 250.0)))
      (bind _output_get_3 (set `local.CameraPosition` (+ (`local.CameraPosition`) (+ (`self.GetFocusObjectsAveragePosition`) (`KismetMathLibrary.MakeVector` 0.0 _output_get_2 (`self.LookUpDownValue`))))))
      (`self.K2_SetActorLocation` _output_get_3))))

(fn `HandleCameraFocusOffset`
  (bind _output_get (set `self.ToFocusOffset` (+ (`self.BaseFocusOffset`) (`self.SecondaryFocusOffset`))))
  (set `self.CurrentFocusOffset` (`KismetMathLibrary.VInterpTo` (`self.CurrentFocusOffset`) _output_get (`GameplayStatics.GetWorldDeltaSeconds`) (`self.ZoomInterpolationSpeed`))))

(fn `HandleCameraZoom`
  (bind _cameraboom (`self.CameraBoom`))
  (set `SpringArmComponent.TargetArmLength` (`KismetMathLibrary.FInterpTo` (`SpringArmComponent.TargetArmLength` _cameraboom) (`self.ToZoom`) (`GameplayStatics.GetWorldDeltaSeconds`) (`self.ZoomInterpolationSpeed`)) _cameraboom))

(fn `InitializeCamera`
  (bind _output_get (set `self.ToZoom` (`self.DefaultZoom`)))
  (set `SpringArmComponent.TargetArmLength` _output_get (`self.CameraBoom`))
  (set `self.CurrentFocusOffset` (+ (`self.BaseFocusOffset`) (`self.SecondaryFocusOffset`))))

(fn `On Focus Object Destroyed`
  (params (DestroyedActor :type "Actor Object Reference"))
  (`self.RemoveCameraFocusObject` DestroyedActor))

(fn `RemoveCameraFocusObject`
  (params (ItemToRemove :type "Actor Object Reference"))
  (`KismetArrayLibrary.Array_RemoveItem` (`self.FocusObjects`) ItemToRemove)
  (remove `self.OnDestroyed` ItemToRemove (`|CreateDelegate` :!event `On Focus Object Destroyed`)))

(fn `ResetCameraParameters`
  (`self.ChangeCameraParameters` (0.0 0.0 0.0) (`self.DefaultZoom`) 5.0))

(fn `ReturnToDefaultZoom`
  (`self.ZoomCamera` (`self.DefaultZoom`)))

(fn `UserConstructionScript`)

(fn `ZoomCamera`
  (params (ToZoom :type "Float (double-precision)") (ZoomInterpolationSpeed :type "Float (double-precision)" :default 5.0))
  (set `self.ToZoom` ToZoom)
  (set `self.ZoomInterpolationSpeed` ZoomInterpolationSpeed))