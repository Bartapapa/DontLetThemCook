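; DBG_BP_CameraChange is an overlap-driven actor that changes the camera parameters of a player character entering it.
; On begin overlap it casts to BP_PlayerCharacter_Master and passes its focus offset, zoom and zoom interpolation speed to that character's current camera.
; On end overlap it resets that camera's parameters unless KeepParameters is set, which lets the change persist after leaving.
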(event `self.ReceiveActorBeginOverlap`
  (params (OtherActor :type "Actor Object Reference"))
  (bind _asbp_player_character_master (cast `/Game/GameElements/Blueprints/Characters/BP_PlayerCharacter_Master` OtherActor))
  (`/Engine/EditorBlueprintResources/StandardMacros.IsValid` _asbp_player_character_master
    (:`Is Valid`
      (`/Game/GameElements/Blueprints/Camera/BP_CameraManager.ChangeCameraParameters` (`/Game/GameElements/Blueprints/Characters/BP_PlayerCharacter_Master.CurrentCamera` _asbp_player_character_master) (`self.FocusOffset`) (`self.ToZoom`) (`self.ZoomInterpolationSpeed`)))))

(event `self.ReceiveActorEndOverlap`
  (params (OtherActor :type "Actor Object Reference"))
  (bind _asbp_player_character_master (cast `/Game/GameElements/Blueprints/Characters/BP_PlayerCharacter_Master` OtherActor))
  (`/Engine/EditorBlueprintResources/StandardMacros.IsValid` _asbp_player_character_master
    (:`Is Valid`
      (if (not (`self.KeepParameters`))
        (`/Game/GameElements/Blueprints/Camera/BP_CameraManager.ResetCameraParameters` (`/Game/GameElements/Blueprints/Characters/BP_PlayerCharacter_Master.CurrentCamera` _asbp_player_character_master))))))

(fn `UserConstructionScript`)