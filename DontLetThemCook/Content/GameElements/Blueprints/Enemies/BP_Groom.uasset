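; BP_Groom is a chaser enemy character that instantly kills the player on first contact.
; SpawnSequence stores the target, disables gravity and uses a timeline to animate its height at the spawn point, then restores gravity and starts the chase.
; While the target lives, Tick pushes it along fixed world +Y rather than steering toward the target.
; Walk speed is remapped from target distance, clamped between minimum and maximum.
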(event `self.ReceiveTick`
  (params (DeltaSeconds :type "Float (single-precision)"))
  (bind _target (`self.Target`))
  (if (`self.Chase?`)
    (if (`KismetSystemLibrary.IsValid` _target)
      (if (not (`/Game/GameElements/Blueprints/Characters/AC_Health.IsDead?` (`/Game/GameElements/Blueprints/Characters/BP_PlayerCharacter_Master.AC_Health` _target)))
        (`self.HandleChaseMovespeed`)
        (`PawnMovementComponent.AddInputVector` (`self.CharacterMovement`) (`KismetMathLibrary.GetRightVector` (struct)) false)))))

(event `self.ReceiveHit`
  (params (MyComp :type "PrimitiveComponent Object Reference") (Other :type "Actor Object Reference") (OtherComp :type "PrimitiveComponent Object Reference") (bSelfMoved :type Boolean) (HitLocation :type "Vector Structure") (HitNormal :type "Vector Structure") (NormalImpulse :type "Vector Structure") (Hit :type "HitResult Structure (by ref)"))
  (bind _asbp_player_character_master (cast `/Game/GameElements/Blueprints/Characters/BP_PlayerCharacter_Master` Other))
  (if (`KismetSystemLibrary.IsValid` _asbp_player_character_master)
    (`/Engine/EditorBlueprintResources/StandardMacros.DoOnce` false
      (:`Completed`
        (`/Game/GameElements/Blueprints/Characters/AC_Health.InstantKill` (`/Game/GameElements/Blueprints/Characters/BP_PlayerCharacter_Master.AC_Health` _asbp_player_character_master))))))

(event `SpawnSequence`
  (params (Target :type "/Game/GameElements/Blueprints/Characters/BP_PlayerCharacter_Master Object Reference"))
  (bind (_returnvalue_x _returnvalue_y) (`KismetMathLibrary.BreakVector` (`self.K2_GetActorLocation`)))
  (bind _spawnpoint (`self.SpawnPoint`))
  (bind (_returnvalue_x_2 _returnvalue_y_2 _returnvalue_z) (`KismetMathLibrary.BreakVector` (`self.K2_GetActorLocation` (`self.SpawnPoint`))))
  (set `self.Target` Target)
  (set `CharacterMovementComponent.GravityScale` 0.0 (`self.CharacterMovement`))
  (`self.K2_SetActorLocationAndRotation` (+ (`self.K2_GetActorLocation` _spawnpoint) (`KismetMathLibrary.MakeVector` 0.0 0.0 (`CapsuleComponent.CapsuleHalfHeight` (`self.CapsuleComponent`)))) (`self.K2_GetActorRotation` _spawnpoint) false true)
  (bind (_direction _height) (`Timeline|Spawn`)
    (:`Update`
      (`self.K2_SetActorLocation` (`KismetMathLibrary.MakeVector` _returnvalue_x _returnvalue_y (+ (+ _returnvalue_z (* _height (`self.UnderHeight`))) (`CapsuleComponent.CapsuleHalfHeight` (`self.CapsuleComponent`)))) false true))
    (:`Finished`
      (set `self.Chase?` true)
      (set `CharacterMovementComponent.GravityScale` 1.0 (`self.CharacterMovement`)))))

(fn `GetCurrentTargetDistance`
  (returns (CurrentDistance :type "Float (double-precision)"))
  (return (`KismetMathLibrary.Vector_Distance` (`self.K2_GetActorLocation`) (`self.K2_GetActorLocation` (`self.Target`)))))

(fn `HandleChaseMovespeed`
  (set `CharacterMovementComponent.MaxWalkSpeed` (`KismetMathLibrary.MapRangeClamped` (`self.GetCurrentTargetDistance`) (`self.MinChaseDistance`) (`self.MaxChaseDistance`) (`self.MinMoveSpeed`) (`self.MaxMoveSpeed`)) (`self.CharacterMovement`)))

(fn `UserConstructionScript`)