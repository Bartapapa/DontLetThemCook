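; Physics-driven pot holder (mitten) prop among the BossCat enemy assets that gets flung away and then removed.
; Yeet picks the left or right mesh, enables physics, and ignores Pawn and one custom collision channel.
; It applies randomized linear and angular impulses as velocity changes, both drawn from the same min/max vector range.
; A one-shot timer then destroys the actor after its configured lifetime.
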(event `Yeet`
  (params (`Right?` :type Boolean))
  (bind _impulsedir (`self.GetRandomImpulse`))
  (bind _potholdermesh (`self.PotHolderMesh`))
  (bind _potholdermesh_2 (`self.PotHolderMesh`))
  (if `Right?`
    (`StaticMeshComponent.SetStaticMesh` _potholdermesh_2 "/Game/GA/Character_GA/Final/Enemy_Boss_body_elements/SM_PotHolderR_01.SM_PotHolderR_01")
    (else
      (`StaticMeshComponent.SetStaticMesh` _potholdermesh_2 "/Game/GA/Character_GA/Final/Enemy_Boss_body_elements/SM_PotHolderL_01.SM_PotHolderL_01")))
  (`PrimitiveComponent.SetSimulatePhysics` _potholdermesh true)
  (`SceneComponent.SetMobility` _potholdermesh "Movable")
  (`PrimitiveComponent.SetCollisionResponseToChannel` _potholdermesh "ECC_Pawn" "ECR_Ignore")
  (`PrimitiveComponent.SetCollisionResponseToChannel` _potholdermesh "ECC_GameTraceChannel1" "ECR_Ignore")
  (`PrimitiveComponent.AddImpulse` _potholdermesh _impulsedir "None" true)
  (`PrimitiveComponent.AddAngularImpulseInDegrees` _potholdermesh _impulsedir "None" true)
  (`self.StartLifeTime`))

(event `StartLifeTime`
  (`KismetSystemLibrary.K2_SetTimerDelegate` (delegate `DestroyMitten`) (`self.LifeTime`)))

(event `DestroyMitten`
  (`self.K2_DestroyActor`))

(fn `GetRandomImpulse`
  (returns (ImpulseDir :type "Vector Structure"))
  (return (`KismetMathLibrary.MakeVector` (`KismetMathLibrary.RandomFloatInRange` (.x (`self.MinImpulse`)) (.x (`self.MaxImpulse`))) (`KismetMathLibrary.RandomFloatInRange` (.y (`self.MinImpulse`)) (.y (`self.MaxImpulse`))) (`KismetMathLibrary.RandomFloatInRange` (.z (`self.MinImpulse`)) (.z (`self.MaxImpulse`))))))

(fn `UserConstructionScript`)