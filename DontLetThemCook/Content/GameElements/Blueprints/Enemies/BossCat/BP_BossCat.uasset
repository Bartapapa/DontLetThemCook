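; Cat boss enemy that tracks the active player character and attacks through two separately spawned BP_BossCatArm actors.
; BeginPlay spawns both arms and makes them appear after a short delay.
; In phases 1 and 2, Tick slides the body along Y toward the player, turns the eyes and serves queued attack requests once both arms are idle.
; Attacks are random smack down, swipe, two-arm clap or ladle, also bound to debug keys.
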(event `self.ReceiveBeginPlay`
  (bind _returnvalue (`SceneComponent.K2_GetComponentLocation` (`self.BossRoot`)))
  (bind _returnvalue_2 (`SceneComponent.K2_GetComponentRotation` (`self.DefaultSceneRoot`)))
  (bind _asbp_game_mode (cast `/Game/GameElements/Blueprints/GameMode/BP_GameMode` (`GameplayStatics.GetGameMode`)))
  (set `self.GameMode` _asbp_game_mode)
  (bind _returnvalue_3 (`|SpawnActorFromClass` "/Game/GameElements/Blueprints/Enemies/BossCat/BP_BossCatArm.BP_BossCatArm_C" (`KismetMathLibrary.MakeTransform` (0.0 0.0 -2000.0) _returnvalue_2) "AlwaysSpawn" "MultiplyWithRoot" null null))
  (`/Game/GameElements/Blueprints/Enemies/BossCat/BP_BossCatArm.InitializeArm` _returnvalue_3 true self)
  (set `self.RightArm` _returnvalue_3)
  (bind _returnvalue_4 (`|SpawnActorFromClass` "/Game/GameElements/Blueprints/Enemies/BossCat/BP_BossCatArm.BP_BossCatArm_C" (`KismetMathLibrary.MakeTransform` (0.0 0.0 -2000.0) _returnvalue_2) "AlwaysSpawn" "MultiplyWithRoot" null null))
  (`/Game/GameElements/Blueprints/Enemies/BossCat/BP_BossCatArm.InitializeArm` _returnvalue_4 false self)
  (set `self.LeftArm` _returnvalue_4)
  (`KismetSystemLibrary.Delay` 3.0)
  (`/Game/GameElements/Blueprints/Enemies/BossCat/BP_BossCatArm.Appear` (`self.RightArm`) _returnvalue)
  (`/Game/GameElements/Blueprints/Enemies/BossCat/BP_BossCatArm.Appear` (`self.LeftArm`) _returnvalue))

(event `self.ReceiveTick`
  (params (DeltaSeconds :type "Float (single-precision)"))
  (if (or (== (`self.Phase`) 1) (== (`self.Phase`) 2))
    (`self.HandleBodyMovement`)
    (`self.Handle Follow Player Eye Movement`)
    (`self.HandleAttackRequest`)))

(event `Key|N`
  (params (Key :type "Key Structure")))

(event `Key|B`
  (params (Key :type "Key Structure"))
  (:`Pressed`
    (`/Game/GameElements/Blueprints/Enemies/BossCat/BP_BossCatArm.PrepareSmackDown` (`self.RightArm`))))

(event `Key|V`
  (params (Key :type "Key Structure"))
  (:`Pressed`
    (`/Game/GameElements/Blueprints/Enemies/BossCat/BP_BossCatArm.PrepareSwipe` (`self.LeftArm`))))

(event `Key|C`
  (params (Key :type "Key Structure"))
  (:`Pressed`
    (`/Game/GameElements/Blueprints/Enemies/BossCat/BP_BossCatArm.PrepareClap` (`self.RightArm`))
    (`/Game/GameElements/Blueprints/Enemies/BossCat/BP_BossCatArm.PrepareClap` (`self.LeftArm`))))

(event `Key|L`
  (params (Key :type "Key Structure"))
  (:`Pressed`
    (`/Game/GameElements/Blueprints/Enemies/BossCat/BP_BossCatArm.PrepareLadle` (`self.RightArm`))))

(fn `AreBothArmsIdle?`
  (returns (`Both arms idle?` :type Boolean))
  (return (and (== (`/Game/GameElements/Blueprints/Enemies/BossCat/BP_BossCatArm.State` (`self.RightArm`)) 0) (== (`/Game/GameElements/Blueprints/Enemies/BossCat/BP_BossCatArm.State` (`self.LeftArm`)) 0))))

(fn `Call Random Attack`
  (bind _arm (`self.GetRandomAvailableArm`))
  (bind _arm_2 (`self.GetRandomAvailableArm`))
  (bind _arm_3 (`self.GetRandomAvailableArm`))
  (switch `int` (`KismetMathLibrary.RandomIntegerInRange` 0 3)
    (:`0`
      (if (`KismetSystemLibrary.IsValid` _arm_2)
        (`/Game/GameElements/Blueprints/Enemies/BossCat/BP_BossCatArm.PrepareSmackDown` _arm_2)))
    (:`1`
      (if (`KismetSystemLibrary.IsValid` _arm)
        (`/Game/GameElements/Blueprints/Enemies/BossCat/BP_BossCatArm.PrepareSwipe` _arm)))
    (:`2`
      (`/Game/GameElements/Blueprints/Enemies/BossCat/BP_BossCatArm.PrepareClap` (`self.RightArm`))
      (`/Game/GameElements/Blueprints/Enemies/BossCat/BP_BossCatArm.PrepareClap` (`self.LeftArm`)))
    (:`3`
      (if (`KismetSystemLibrary.IsValid` _arm_3)
        (`/Game/GameElements/Blueprints/Enemies/BossCat/BP_BossCatArm.PrepareLadle` _arm_3)))))

(fn `GetRandomAvailableArm`
  (returns (Arm :type "/Game/GameElements/Blueprints/Enemies/BossCat/BP_BossCatArm Object Reference"))
  (bind _leftarm (`self.LeftArm`))
  (bind _rightarm (`self.RightArm`))
  (bind _leftarm_2 (`self.LeftArm`))
  (bind _rightarm_2 (`self.RightArm`))
  (if (== (`KismetMathLibrary.RandomIntegerInRange` 0 1) 0)
    (if (`/Game/GameElements/Blueprints/Enemies/BossCat/BP_BossCatArm.IsAttacking?` _rightarm_2)
      (if (`/Game/GameElements/Blueprints/Enemies/BossCat/BP_BossCatArm.IsAttacking?` _leftarm)
        (return null)
        (else
          (return _leftarm)))
      (else
        (return _rightarm_2)))
    (elif (`/Game/GameElements/Blueprints/Enemies/BossCat/BP_BossCatArm.IsAttacking?` _leftarm_2)
      (if (`/Game/GameElements/Blueprints/Enemies/BossCat/BP_BossCatArm.IsAttacking?` _rightarm)
        (return null)
        (else
          (return _rightarm)))
      (else
        (return _leftarm_2)))))

(fn `Handle Follow Player Eye Movement`
  (bind _eyer (`self.EyeR`))
  (bind _eyel (`self.EyeL`))
  (bind _currentactivecharacter (`/Game/GameElements/Blueprints/GameMode/BP_GameMode.CurrentActiveCharacter` (`self.GameMode`)))
  (bind _returnvalue (`SceneComponent.K2_GetComponentLocation` (`Character.CapsuleComponent` _currentactivecharacter)))
  (if (and (`self.IsInitialized?`) (`self.EyeFollowPlayer`))
    (if (`KismetSystemLibrary.IsValid` _currentactivecharacter)
      (`SceneComponent.K2_SetWorldRotation` _eyer (`KismetMathLibrary.RInterpTo` (`SceneComponent.K2_GetComponentRotation` _eyer) (`KismetMathLibrary.FindLookAtRotation` (`SceneComponent.K2_GetComponentLocation` _eyer) _returnvalue) (`GameplayStatics.GetWorldDeltaSeconds`) (`self.EyeFollowSpeed`)) false false)
      (`SceneComponent.K2_SetWorldRotation` _eyel (`KismetMathLibrary.RInterpTo` (`SceneComponent.K2_GetComponentRotation` _eyel) (`KismetMathLibrary.FindLookAtRotation` (`SceneComponent.K2_GetComponentLocation` _eyel) _returnvalue) (`GameplayStatics.GetWorldDeltaSeconds`) (`self.EyeFollowSpeed`)) false false))))

(fn `HandleArmMovement`)

(fn `HandleAttackRequest`
  (if (`self.AttackRequested`)
    (if (`self.AreBothArmsIdle?`)
      (`self.Call Random Attack`)
      (set `self.AttackRequested` false))))

(fn `HandleBodyMovement`
  (bind _bossroot (`self.BossRoot`))
  (bind (_returnvalue_x _returnvalue_y _returnvalue_z) (`KismetMathLibrary.BreakVector` (`SceneComponent.K2_GetComponentLocation` _bossroot)))
  (bind (_returnvalue_x_2 _returnvalue_y_2) (`KismetMathLibrary.BreakVector` (`SceneComponent.K2_GetComponentLocation` (`self.BossRoot`))))
  (bind _currentactivecharacter (`/Game/GameElements/Blueprints/GameMode/BP_GameMode.CurrentActiveCharacter` (`self.GameMode`)))
  (bind (_returnvalue_x_3 _returnvalue_y_3) (`KismetMathLibrary.BreakVector` (`SceneComponent.K2_GetComponentLocation` (`Character.CapsuleComponent` _currentactivecharacter))))
  (bind _returnvalue (- _returnvalue_y_2 _returnvalue_y_3))
  (if (`self.IsInitialized?`)
    (if (`KismetSystemLibrary.IsValid` _currentactivecharacter)
      (if (> (`KismetMathLibrary.Abs` _returnvalue) (`self.BodyApproachToProximity`))
        (`SceneComponent.K2_SetWorldLocation` _bossroot (`KismetMathLibrary.MakeVector` _returnvalue_x (`KismetMathLibrary.FInterpTo` _returnvalue_y (+ _returnvalue_y_3 (* (`self.BodyApproachToProximity`) (`KismetMathLibrary.SignOfFloat` _returnvalue))) (`GameplayStatics.GetWorldDeltaSeconds`) (`self.BodyMoveSpeed`)) _returnvalue_z) false false)))))

(fn `IsInitialized?`
  (returns (`Initialized?` :type Boolean))
  (return (`KismetSystemLibrary.IsValid` (`self.GameMode`))))

(fn `Request Attack`
  (set `self.AttackRequested` true))

(fn `UserConstructionScript`)