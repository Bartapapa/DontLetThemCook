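; Hot soup projectile for the Boss Cat enemy that falls and damages actors it overlaps.
; Each tick moves it down by lifetime times gravity, a per-frame step not scaled by delta time, and destroys it at a minimum Z.
; InitializeProjectile randomizes gravity within a range.
; Overlapping an actor with AC_Health deals damage with hitstun and knockback, then destroys the projectile.
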(event `self.ReceiveActorBeginOverlap`
  (params (OtherActor :type "Actor Object Reference"))
  (bind _returnvalue (`self.GetComponentByClass` OtherActor "/Game/GameElements/Blueprints/Characters/AC_Health.AC_Health_C"))
  (`/Engine/EditorBlueprintResources/StandardMacros.IsValid` _returnvalue
    (:`Is Valid`
      (`/Game/GameElements/Blueprints/Characters/AC_Health.Damage` _returnvalue self (`self.ProjectileOwner`) "NewEnumerator2" 1 true 1.0)
      (`self.DestroyProjectile`))))

(event `self.ReceiveTick`
  (params (DeltaSeconds :type "Float (single-precision)"))
  (`self.HandleAcceleration`))

(event `DestroyProjectile`
  (`self.K2_DestroyActor`))

(fn `HandleAcceleration`
  (bind (_returnvalue_x _returnvalue_y _returnvalue_z) (`KismetMathLibrary.BreakVector` (`self.K2_GetActorLocation`)))
  (set `self.CurrentLifetimeTimer` (+ (`self.CurrentLifetimeTimer`) (`GameplayStatics.GetWorldDeltaSeconds`)))
  (`self.K2_SetActorLocation` (+ (`self.K2_GetActorLocation`) (`KismetMathLibrary.MakeVector` 0.0 0.0 (* (* (`self.CurrentLifetimeTimer`) (`self.GravityAcceleration`)) -1.0))) false true)
  (if (<= _returnvalue_z (`self.MinimumZPos`))
    (`self.DestroyProjectile`)))

(fn `InitializeProjectile`
  (set `self.GravityAcceleration` (`KismetMathLibrary.RandomFloatInRange` (`self.MinGravityAcceleration`) (`self.MaxGravityAcceleration`))))

(fn `UserConstructionScript`)