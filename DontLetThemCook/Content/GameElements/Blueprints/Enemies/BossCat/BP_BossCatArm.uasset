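; Left or right arm of the cat boss, which appears and disappears along Z via timelines and attacks the player.
; Tick runs a state machine: idle eases it alongside the boss at a Y offset.
; Smack-down uses timed phases: tracking the active character with narrowing sine sway, locking with growing shake, then sphere-tracing to damage AC_Health actors.
; Swipe only sets its state; its handlers are empty stubs.
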(event `self.ReceiveTick`
  (params (DeltaSeconds :type "Float (single-precision)"))
  (switch `int` (`self.State`)
    (:`0`
      (`self.HandleIdleArmPositioning`)
      (if (`self.Right?`)
        (`KismetSystemLibrary.PrintString` "!!!")))
    (:`1`
      (switch `int` (`self.SmackDownState`)
        (:`1`
          (`self.HandleSmackDownArmPositioning`))
        (:`2`
          (`self.HandleSmackDownLockShake`))))
    (:`2`
      (switch `int` (`self.SwipeState`)))))

(event `InitializeArm`
  (params (`Right?` :type Boolean) (BossCat :type "/Game/GameElements/Blueprints/Enemies/BossCat/BP_BossCat Object Reference"))
  (`SceneComponent.SetVisibility` (`self.BossArmR`) `Right?` true)
  (`SceneComponent.SetVisibility` (`self.BossArmL`) (not `Right?`) true)
  (set `self.BossCat` BossCat)
  (set `self.Right?` `Right?`))

(event `Appear`
  (params (Location :type "Vector Structure"))
  (bind (_returnvalue_x _returnvalue_y _returnvalue_z) (`KismetMathLibrary.BreakVector` (`self.K2_GetActorLocation`)))
  (bind _returnvalue (+ Location (`self.BaseBodyOffset`)))
  (if (`self.Right?`)
    (`self.K2_SetActorLocation` (+ _returnvalue (`KismetMathLibrary.MakeVector` 0.0 (* (`self.ArmYPositioningOffset`) -1.0))) false true)
    (bind (_direction _appearcurve) (`Timeline|ArmAppear` :!via `PlayFromStart` :!label _label)
      (:`Update`
        (set `self.Spawning?` true)
        (`SceneComponent.K2_SetWorldLocation` (`self.ArmRoot`) (`KismetMathLibrary.MakeVector` _returnvalue_x _returnvalue_y (+ _returnvalue_z (* (`self.SpawnZPosition`) _appearcurve))) false false))
      (:`Finished`
        (set `self.Spawning?` false)
        (set `self.Active?` true)))
    (else
      (`self.K2_SetActorLocation` (+ _returnvalue (`KismetMathLibrary.MakeVector` 0.0 (`self.ArmYPositioningOffset`))) false true)
      (goto _label :!via `PlayFromStart`))))

(event `Disappear`
  (bind (_returnvalue_x _returnvalue_y _returnvalue_z) (`KismetMathLibrary.BreakVector` (`self.K2_GetActorLocation`)))
  (bind (_direction _disappearcurve) (`Timeline|ArmDisappear` :!via `PlayFromStart`)
    (:`Update`
      (set `self.Spawning?` true)
      (set `self.Active?` false)
      (`SceneComponent.K2_SetWorldLocation` (`self.ArmRoot`) (`KismetMathLibrary.MakeVector` _returnvalue_x _returnvalue_y (+ _returnvalue_z (* (`self.SpawnZPosition`) _disappearcurve))) false false))
    (:`Finished`
      (set `self.Spawning?` false))))

(fn `HandleIdleArmPositioning`
  (bind _armroot (`self.ArmRoot`))
  (bind _bosscat (`self.BossCat`))
  (bind _armroot_2 (`self.ArmRoot`))
  (bind (_returnvalue_x _returnvalue_y _returnvalue_z) (`KismetMathLibrary.BreakVector` (`SceneComponent.K2_GetComponentLocation` _armroot)))
  (bind (_returnvalue_x_2 _returnvalue_y_2 _returnvalue_z_2) (`KismetMathLibrary.BreakVector` (`SceneComponent.K2_GetComponentLocation` _armroot_2)))
  (bind _bossroot (`/Game/GameElements/Blueprints/Enemies/BossCat/BP_BossCat.BossRoot` _bosscat))
  (bind (_returnvalue_x_3 _returnvalue_y_3) (`KismetMathLibrary.BreakVector` (`SceneComponent.K2_GetComponentLocation` _bossroot)))
  (bind (_returnvalue_x_4 _returnvalue_y_4) (`KismetMathLibrary.BreakVector` (`SceneComponent.K2_GetComponentLocation` _bossroot)))
  (bind _returnvalue (- _returnvalue_y_2 _returnvalue_y_4))
  (bind _returnvalue_2 (- _returnvalue_y _returnvalue_y_3))
  (if (and (`self.Active?`) (not (`self.Spawning?`)))
    (if (`KismetSystemLibrary.IsValid` _bosscat)
      (if (`self.Right?`)
        (if (< _returnvalue_2 (`self.ArmYPositioningOffset`))
          (`SceneComponent.K2_SetWorldLocation` _armroot (`KismetMathLibrary.VInterpTo` (`KismetMathLibrary.MakeVector` _returnvalue_x _returnvalue_y _returnvalue_z) (`KismetMathLibrary.MakeVector` _returnvalue_x_3 (+ _returnvalue_y_3 (* (`self.ArmYPositioningOffset`) (`KismetMathLibrary.SignOfFloat` _returnvalue_2))) _returnvalue_z) (`GameplayStatics.GetWorldDeltaSeconds`) (`self.IdleArmMovementSpeed`)) false false))
        (elif (> _returnvalue (* (`self.ArmYPositioningOffset`) -1.0))
          (`SceneComponent.K2_SetWorldLocation` _armroot_2 (`KismetMathLibrary.VInterpTo` (`KismetMathLibrary.MakeVector` _returnvalue_x_2 _returnvalue_y_2 _returnvalue_z_2) (`KismetMathLibrary.MakeVector` _returnvalue_x_4 (+ _returnvalue_y_4 (* (`self.ArmYPositioningOffset`) (`KismetMathLibrary.SignOfFloat` _returnvalue))) _returnvalue_z_2) (`GameplayStatics.GetWorldDeltaSeconds`) (`self.IdleArmMovementSpeed`)) false false))))))

(fn `HandleSmackDownArmPositioning`
  (bind _smackdownpreptimer (`self.SmackDownPrepTimer`))
  (bind _bosscat (`self.BossCat`))
  (bind _armroot (`self.ArmRoot`))
  (bind _returnvalue (`KismetSystemLibrary.K2_GetTimerElapsedTimeHandle` _smackdownpreptimer))
  (bind _currentactivecharacter (`/Game/GameElements/Blueprints/GameMode/BP_GameMode.CurrentActiveCharacter` (`/Game/GameElements/Blueprints/Enemies/BossCat/BP_BossCat.GameMode` _bosscat)))
  (bind (_returnvalue_x _returnvalue_y) (`KismetMathLibrary.BreakVector` (+ (`SceneComponent.K2_GetComponentLocation` (`Character.CapsuleComponent` _currentactivecharacter)) (`KismetMathLibrary.MakeVector` (`self.ForegroundCharacterXOffset`)))))
  (if (and (`self.Active?`) (not (`self.Spawning?`)) (== (`self.SmackDownState`) 1))
    (if (`KismetSystemLibrary.IsValid` _bosscat)
      (if (`KismetSystemLibrary.IsValid` _currentactivecharacter)
        (if (`KismetSystemLibrary.K2_IsValidTimerHandle` _smackdownpreptimer)
          (`SceneComponent.K2_SetWorldLocation` _armroot (`KismetMathLibrary.VInterpTo` (`SceneComponent.K2_GetComponentLocation` _armroot) (`KismetMathLibrary.MakeVector` _returnvalue_x (+ (* (* (- 1.3 (/ _returnvalue (`self.SmackDownPrepTime`))) (`self.SmackDownArmMaxYVariance`)) (`KismetMathLibrary.DegSin` (* (+ _returnvalue (`self.RandomFloat`)) 200.0))) _returnvalue_y)) (`GameplayStatics.GetWorldDeltaSeconds`) (`self.TargetingArmMovementSpeed`)) false false))))))

(fn `HandleSmackDownLockShake`
  (bind _smackdownlocktimer (`self.SmackDownLockTimer`))
  (bind _returnvalue (/ (`KismetSystemLibrary.K2_GetTimerElapsedTimeHandle` _smackdownlocktimer) (`self.SmackDownLockTime`)))
  (bind _returnvalue_2 (* _returnvalue (* (`KismetMathLibrary.RandomFloatInRange` 0.0 1.0) (`self.SmackDownLockShakeIntensity`))))
  (bind _returnvalue_3 (* _returnvalue (* (`KismetMathLibrary.RandomFloatInRange` 0.0 1.0) (`self.SmackDownLockShakeIntensity`))))
  (if (`KismetSystemLibrary.K2_IsValidTimerHandle` _smackdownlocktimer)
    (if (`self.Right?`)
      (`SceneComponent.K2_SetRelativeLocation` (`self.BossArmR`) (`KismetMathLibrary.MakeVector` _returnvalue_2 0.0 _returnvalue_3) false false)
      (else
        (`SceneComponent.K2_SetRelativeLocation` (`self.BossArmL`) (`KismetMathLibrary.MakeVector` _returnvalue_2 0.0 _returnvalue_3) false false)))))

(fn `HandleSwipeArmPositioning`)

(fn `HandleSwipeLockShake`)

(fn `IsReady?`
  (returns (`Ready?` :type Boolean))
  (return (not (`self.Spawning?`))))

(fn `Post Smack Down Return to Idle`
  (set `self.SmackDownState` 0)
  (set `self.State` 0)
  (`KismetSystemLibrary.PrintString` "RETURN TO IDLE"))

(fn `PostSwipeReturnToIdle`)

(fn `PrepareSmackDown`
  (if (== (`self.State`) 0)
    (set `self.State` 1)
    (set `self.SmackDownState` 1)
    (bind _returnvalue (`KismetSystemLibrary.K2_SetTimerDelegate` (`|CreateDelegate` :!event `Smack Down Lock`) (`self.SmackDownPrepTime`)))
    (set `self.SmackDownPrepTimer` _returnvalue)
    (set `self.RandomFloat` (`KismetMathLibrary.RandomFloatInRange` 0.0 100.0))))

(fn `PrepareSwipe`
  (if (== (`self.State`) 0)
    (set `self.State` 2)
    (set `self.SwipeState` 1)))

(fn `Smack Down`
  (bind _armroot (`self.ArmRoot`))
  (bind _returnvalue (+ (`SceneComponent.K2_GetComponentLocation` _armroot) (* (`SceneComponent.GetRightVector` _armroot) 200.0)))
  (set `self.SmackDownState` 3)
  (`SceneComponent.K2_SetRelativeLocation` (`self.BossArmR`) (0.0 0.0 0.0) false false)
  (`SceneComponent.K2_SetRelativeLocation` (`self.BossArmL`) (0.0 0.0 0.0) false false)
  (bind _outhits (`KismetSystemLibrary.SphereTraceMultiForObjects` :`Start` _returnvalue :`End` _returnvalue :`Radius` 200.0 :`ObjectTypes` (`|MakeArray` "ObjectTypeQuery1" "ObjectTypeQuery2" "ObjectTypeQuery3" :!type "EObjectTypeQuery Enum") :`DrawDebugType` "ForOneFrame" :`DrawTime` 0.0))
  (for _array_element _outhits
    (bind _returnvalue_2 (`self.GetComponentByClass` (`.HitActor` (`GameplayStatics.BreakHitResult` _array_element)) "/Game/GameElements/Blueprints/Characters/AC_Health.AC_Health_C"))
    (if (`KismetSystemLibrary.IsValid` _returnvalue_2)
      (`/Game/GameElements/Blueprints/Characters/AC_Health.Damage` _returnvalue_2 self (`self.BossCat`) "NewEnumerator2" 1 true 2.0)))
  (set `self.SmackDownState` 4)
  (bind _returnvalue_3 (`KismetSystemLibrary.K2_SetTimerDelegate` (`|CreateDelegate` :!event `Post Smack Down Return to Idle`) (`self.SmackAfterHitIdleTime`)))
  (set `self.SmackAfterHitIdleTimer` _returnvalue_3))

(fn `Smack Down Lock`
  (set `self.SmackDownState` 2)
  (bind _returnvalue (`KismetSystemLibrary.K2_SetTimerDelegate` (`|CreateDelegate` :!event `Smack Down`) (`self.SmackDownLockTime`)))
  (set `self.SmackDownLockTimer` _returnvalue))

(fn `SwipeLock`)

(fn `SwipeMovement`)

(fn `UserConstructionScript`)