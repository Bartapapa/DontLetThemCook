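; BP_CommyCat is a boss enemy that trails the active player along Y, eyes tracking them, and attacks through two spawned BP_CommyArm actors.
; Spawn starts phase 1, reveals only the right arm and starts a looping attack timer.
; Tick passes attack requests to idle arms; random selection currently allows only SmackDown.
; Hurt clears the timer, then montage completion triggers a one-time low-health enrage or restarts attacks; death destroys boss and arms.
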(event `self.ReceiveBeginPlay`
  (bind _returnvalue (`SceneComponent.K2_GetComponentRotation` (`self.DefaultSceneRoot`)))
  (bind _asbp_game_mode (cast `/Game/GameElements/Blueprints/GameMode/BP_GameMode` (`GameplayStatics.GetGameMode`)))
  (set `self.GameMode` _asbp_game_mode)
  (bind _returnvalue_2 (`|SpawnActorFromClass` "/Game/GameElements/Blueprints/Enemies/CommyBastard/BP_CommyArm.BP_CommyArm_C" (`KismetMathLibrary.MakeTransform` (0.0 0.0 -2000.0) _returnvalue) "AlwaysSpawn" "MultiplyWithRoot" null null))
  (`/Game/GameElements/Blueprints/Enemies/CommyBastard/BP_CommyArm.InitializeArm` _returnvalue_2 true self (`self.MinY`) (`self.MaxY`))
  (set `self.RightArm` _returnvalue_2)
  (bind _returnvalue_3 (`|SpawnActorFromClass` "/Game/GameElements/Blueprints/Enemies/CommyBastard/BP_CommyArm.BP_CommyArm_C" (`KismetMathLibrary.MakeTransform` (0.0 0.0 -2000.0) _returnvalue) "AlwaysSpawn" "MultiplyWithRoot" null null))
  (`/Game/GameElements/Blueprints/Enemies/CommyBastard/BP_CommyArm.InitializeArm` _returnvalue_3 false self (`self.MinY`) (`self.MaxY`))
  (set `self.LeftArm` _returnvalue_3)
  (`self.InitializeStats`))

(event `self.ReceiveTick`
  (params (DeltaSeconds :type "Float (single-precision)"))
  (if (or (== (`self.Phase`) 1) (== (`self.Phase`) 2))
    (`self.HandleBodyMovement`)
    (`self.Handle Follow Player Eye Movement`)
    (`self.HandleAttackRequest`)))

(event `Spawn`
  (`self.Anim_Spawn`)
  (set `self.HasSpawned?` true)
  (set `self.Phase` 1)
  (`KismetSystemLibrary.Delay` 5.0)
  (`/Game/GameElements/Blueprints/Enemies/CommyBastard/BP_CommyArm.Appear` (`self.RightArm`) (`SceneComponent.K2_GetComponentLocation` (`self.BossRoot`)))
  (bind _returnvalue (`KismetSystemLibrary.K2_SetTimerDelegate` (`|CreateDelegate` :!event `Request Attack`) (`self.TimeBetweenAttacks`) true))
  (set `self.TimeBetweenAttacksTimer` _returnvalue))

(event `Anim_Spawn`
  (`|PlayMontage` (`self.BossSMesh`) "/Game/GA/Character_GA/Final/AnimFBX/BossEnemy/A_Enemy_Spawn_Montage.A_Enemy_Spawn_Montage"))

(event `Anim_PrepareLock`
  (`|PlayMontage` (`self.BossSMesh`) "/Game/GA/Character_GA/Final/AnimFBX/BossEnemy/Boss_FBX_Anim_Armature_Enemy_FG_PrepLock_Montage.Boss_FBX_Anim_Armature_Enemy_FG_PrepLock_Montage"))

(event `Anim_Attack`
  (`|PlayMontage` (`self.BossSMesh`) "/Game/GA/Character_GA/Final/AnimFBX/BossEnemy/Boss_FBX_Anim_Armature_Enemy_FG_Attack_Montage.Boss_FBX_Anim_Armature_Enemy_FG_Attack_Montage"))

(event `Anim_Death`
  (`|PlayMontage` (`self.BossSMesh`) "/Game/GA/Character_GA/Final/AnimFBX/BossEnemy/Boss_FBX_Anim_Armature_Enemy_FG_Boss_Death_Montage.Boss_FBX_Anim_Armature_Enemy_FG_Boss_Death_Montage" 0.5
    (:`OnCompleted`
      (`self.K2_DestroyActor` (`self.RightArm`))
      (`self.K2_DestroyActor` (`self.LeftArm`))
      (`self.K2_DestroyActor`))))

(event `Anim_IntoEnrage`
  (`|PlayMontage` (`self.BossSMesh`) "/Game/GA/Character_GA/Final/AnimFBX/BossEnemy/Boss_FBX_Anim_Armature_Enemy_FG_BossIntoEnrage_REWORK_Montage.Boss_FBX_Anim_Armature_Enemy_FG_BossIntoEnrage_REWORK_Montage"
    (:`OnCompleted`
      (bind _returnvalue (`KismetSystemLibrary.K2_SetTimerDelegate` (`|CreateDelegate` :!event `Request Attack`) (`self.TimeBetweenAttacks`) true :!label _label))
      (set `self.TimeBetweenAttacksTimer` _returnvalue))))

(event `Anim_Hurt`
  (`|PlayMontage` (`self.BossSMesh`) "/Game/GA/Character_GA/Final/AnimFBX/BossEnemy/Boss_FBX_Anim_Armature_Enemy_FG_Hurt_Montage.Boss_FBX_Anim_Armature_Enemy_FG_Hurt_Montage"
    (:`OnCompleted`
      (bind _enrage_ (`self.CheckTransitionToEnrage`))
      (if _enrage_
        (`self.Enrage`)
        (else
          (goto _label))))))

(fn `AreBothArmsIdle?`
  (returns (`Both arms idle?` :type Boolean))
  (return (and (== (`/Game/GameElements/Blueprints/Enemies/CommyBastard/BP_CommyArm.State` (`self.RightArm`)) 0) (== (`/Game/GameElements/Blueprints/Enemies/CommyBastard/BP_CommyArm.State` (`self.LeftArm`)) 0))))

(fn `AreBothArmsSpawned?`
  (returns (`BothSpawned?` :type Boolean))
  (return (and (`/Game/GameElements/Blueprints/Enemies/CommyBastard/BP_CommyArm.Spawned?` (`self.RightArm`)) (`/Game/GameElements/Blueprints/Enemies/CommyBastard/BP_CommyArm.Spawned?` (`self.LeftArm`)))))

(fn `Call Random Attack`
  (bind _arm (`self.GetRandomAvailableArm`))
  (bind _arm_2 (`self.GetRandomAvailableArm`))
  (bind _arm_3 (`self.GetRandomAvailableArm`))
  (switch `int` (`KismetMathLibrary.RandomIntegerInRange` 0)
    (:`0`
      (if (`KismetSystemLibrary.IsValid` _arm_2)
        (`/Game/GameElements/Blueprints/Enemies/CommyBastard/BP_CommyArm.PrepareSmackDown` _arm_2)))
    (:`1`
      (if (`KismetSystemLibrary.IsValid` _arm)
        (`/Game/GameElements/Blueprints/Enemies/CommyBastard/BP_CommyArm.PrepareSwipe` _arm)))
    (:`2`
      (`/Game/GameElements/Blueprints/Enemies/CommyBastard/BP_CommyArm.PrepareClap` (`self.RightArm`))
      (`/Game/GameElements/Blueprints/Enemies/CommyBastard/BP_CommyArm.PrepareClap` (`self.LeftArm`)))
    (:`3`
      (if (`KismetSystemLibrary.IsValid` _arm_3)
        (`/Game/GameElements/Blueprints/Enemies/CommyBastard/BP_CommyArm.PrepareLadle` _arm_3)))))

(fn `CallRandomAttackOnArm`
  (params (Arm :type "/Game/GameElements/Blueprints/Enemies/CommyBastard/BP_CommyArm Object Reference"))
  (switch `int` (`KismetMathLibrary.RandomIntegerInRange` 0)
    (:`0`
      (`/Game/GameElements/Blueprints/Enemies/CommyBastard/BP_CommyArm.PrepareSmackDown` Arm))
    (:`1`
      (`/Game/GameElements/Blueprints/Enemies/CommyBastard/BP_CommyArm.PrepareSwipe` Arm))
    (:`2`
      (`/Game/GameElements/Blueprints/Enemies/CommyBastard/BP_CommyArm.PrepareLadle` Arm))))

(fn `CheckTransitionToEnrage`
  (returns (`Enrage?` :type Boolean))
  (return (and (<= (`/Game/GameElements/Blueprints/Characters/AC_Health.CurrentHealth` (`self.AC_Health`)) 3) (not (`self.Enraged?`)))))

(fn `Die`
  (`self.Anim_Death`)
  (`/Game/GameElements/Blueprints/Enemies/CommyBastard/BP_CommyArm.Die` (`self.RightArm`))
  (`/Game/GameElements/Blueprints/Enemies/CommyBastard/BP_CommyArm.Die` (`self.LeftArm`)))

(fn `Enrage`
  (set `self.Enraged?` true)
  (`self.Anim_IntoEnrage`))

(fn `GetRandomAvailableArm`
  (returns (Arm :type "/Game/GameElements/Blueprints/Enemies/CommyBastard/BP_CommyArm Object Reference"))
  (bind _leftarm (`self.LeftArm`))
  (bind _leftarm_2 (`self.LeftArm`))
  (bind _rightarm (`self.RightArm`))
  (bind _rightarm_2 (`self.RightArm`))
  (if (== (`KismetMathLibrary.RandomIntegerInRange` 0 1) 0)
    (if (and (`/Game/GameElements/Blueprints/Enemies/CommyBastard/BP_CommyArm.IsAttacking?` _rightarm) (not (`/Game/GameElements/Blueprints/Enemies/CommyBastard/BP_CommyArm.Spawned?` _rightarm)))
      (if (and (`/Game/GameElements/Blueprints/Enemies/CommyBastard/BP_CommyArm.IsAttacking?` _leftarm) (not (`/Game/GameElements/Blueprints/Enemies/CommyBastard/BP_CommyArm.Spawned?` _leftarm)))
        (return null)
        (else
          (return _leftarm)))
      (else
        (return null)))
    (elif (and (`/Game/GameElements/Blueprints/Enemies/CommyBastard/BP_CommyArm.IsAttacking?` _leftarm_2) (not (`/Game/GameElements/Blueprints/Enemies/CommyBastard/BP_CommyArm.Spawned?` _leftarm_2)))
      (if (and (`/Game/GameElements/Blueprints/Enemies/CommyBastard/BP_CommyArm.IsAttacking?` _rightarm_2) (not (`/Game/GameElements/Blueprints/Enemies/CommyBastard/BP_CommyArm.Spawned?` _rightarm_2)))
        (return null)
        (else
          (return _rightarm_2)))
      (else
        (return null)))))

(fn `Handle Follow Player Eye Movement`
  (bind _eyer (`self.EyeR`))
  (bind _eyel (`self.EyeL`))
  (bind _currentactivecharacter (`/Game/GameElements/Blueprints/GameMode/BP_GameMode.CurrentActiveCharacter` (`self.GameMode`)))
  (bind _returnvalue (`SceneComponent.K2_GetComponentLocation` (`Character.CapsuleComponent` _currentactivecharacter)))
  (if (and (`self.IsInitialized?`) (`self.EyeFollowPlayer`))
    (if (`KismetSystemLibrary.IsValid` _currentactivecharacter)
      (`SceneComponent.K2_SetWorldRotation` _eyer (`KismetMathLibrary.RInterpTo` (`SceneComponent.K2_GetComponentRotation` _eyer) (`KismetMathLibrary.FindLookAtRotation` (`SceneComponent.K2_GetComponentLocation` _eyer) _returnvalue) (`GameplayStatics.GetWorldDeltaSeconds`) (`self.EyeFollowSpeed`)) false false)
      (`SceneComponent.K2_SetWorldRotation` _eyel (`KismetMathLibrary.RInterpTo` (`SceneComponent.K2_GetComponentRotation` _eyel) (`KismetMathLibrary.FindLookAtRotation` (`SceneComponent.K2_GetComponentLocation` _eyel) _returnvalue) (`GameplayStatics.GetWorldDeltaSeconds`) (`self.EyeFollowSpeed`)) false false))))

(fn `HandleArmMovement`)

(fn `HandleAttackRequest`
  (bind _rightarm (`self.RightArm`))
  (bind _leftarm (`self.LeftArm`))
  (if (`self.AttackRequested`)
    (if (`self.AreBothArmsSpawned?`)
      (if (`self.AreBothArmsIdle?`)
        (`self.Call Random Attack`))
      (set `self.AttackRequested` false)
      (else
        (if (`self.IsArmIdle?` _rightarm)
          (if (`self.IsArmIdle?` _leftarm)
            (`self.Call Random Attack`)
            (else
              (`self.CallRandomAttackOnArm` _rightarm)))
          (elif (`self.IsArmIdle?` _leftarm)
            (`self.CallRandomAttackOnArm` _leftarm)))
        (set `self.AttackRequested` false)))))

(fn `HandleBodyMovement`
  (bind _bossroot (`self.BossRoot`))
  (bind (_returnvalue_x _returnvalue_y _returnvalue_z) (`KismetMathLibrary.BreakVector` (`SceneComponent.K2_GetComponentLocation` _bossroot)))
  (bind (_returnvalue_x_2 _returnvalue_y_2) (`KismetMathLibrary.BreakVector` (`SceneComponent.K2_GetComponentLocation` (`self.BossRoot`))))
  (bind _currentactivecharacter (`/Game/GameElements/Blueprints/GameMode/BP_GameMode.CurrentActiveCharacter` (`self.GameMode`)))
  (bind (_returnvalue_x_3 _returnvalue_y_3) (`KismetMathLibrary.BreakVector` (`SceneComponent.K2_GetComponentLocation` (`Character.CapsuleComponent` _currentactivecharacter))))
  (bind _returnvalue (- _returnvalue_y_2 _returnvalue_y_3))
  (if (`self.IsInitialized?`)
    (if (`KismetSystemLibrary.IsValid` _currentactivecharacter)
      (if (> (`KismetMathLibrary.Abs` _returnvalue) (`self.BodyApproachToProximity`))
        (`SceneComponent.K2_SetWorldLocation` _bossroot (`KismetMathLibrary.MakeVector` _returnvalue_x (`KismetMathLibrary.FInterpTo` _returnvalue_y (+ _returnvalue_y_3 (* (`self.BodyApproachToProximity`) (`KismetMathLibrary.SignOfFloat` _returnvalue))) (`GameplayStatics.GetWorldDeltaSeconds`) (`self.BodyMoveSpeed`)) _returnvalue_z) false false)))))

(fn `Hurt`
  (bind _timebetweenattackstimer (`self.TimeBetweenAttacksTimer`))
  (if (> (`/Game/GameElements/Blueprints/Characters/AC_Health.CurrentHealth` (`self.AC_Health`)) 0)
    (`self.Anim_Hurt`)
    (else
      (`self.Die`)))
  (if (`KismetSystemLibrary.K2_IsValidTimerHandle` _timebetweenattackstimer)
    (`KismetSystemLibrary.K2_ClearAndInvalidateTimerHandle` _timebetweenattackstimer))
  (set `self.AttackRequested` false))

(fn `InitializeStats`
  (bind _ac_health (`self.AC_Health`))
  (`/Game/GameElements/Blueprints/Characters/AC_Health.InitializeHealth` _ac_health 2)
  (add `/Game/GameElements/Blueprints/Characters/AC_Health.OnHealthDamaged` _ac_health (`|CreateDelegate` :!event `On Health Damaged`))
  (add `/Game/GameElements/Blueprints/Characters/AC_Health.OnHealthHealed` _ac_health (`|CreateDelegate` :!event `On Health Healed`)))

(fn `IsArmIdle?`
  (params (Arm :type "/Game/GameElements/Blueprints/Enemies/CommyBastard/BP_CommyArm Object Reference"))
  (returns (`IsIdle?` :type Boolean))
  (return (and (== (`/Game/GameElements/Blueprints/Enemies/CommyBastard/BP_CommyArm.State` Arm) 0) (`/Game/GameElements/Blueprints/Enemies/CommyBastard/BP_CommyArm.Spawned?` Arm))))

(fn `IsInitialized?`
  (returns (`Initialized?` :type Boolean))
  (return (`KismetSystemLibrary.IsValid` (`self.GameMode`))))

(fn `On Health Damaged`
  (params (Source :type "Actor Object Reference") (Instigator :type "Actor Object Reference") (`Damage value` :type Integer) (`Hitstun?` :type Boolean) (KnockbackForceMultiplier :type "Float (double-precision)")))

(fn `On Health Healed`
  (params (HealValue :type Integer)))

(fn `Request Attack`
  (set `self.AttackRequested` true))

(fn `UserConstructionScript`)