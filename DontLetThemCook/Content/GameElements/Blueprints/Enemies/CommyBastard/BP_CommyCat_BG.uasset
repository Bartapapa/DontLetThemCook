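; BP_CommyCat_BG is a background CommyCat enemy that switches into an active state after a random delay.
; BeginPlay clears the Activity flag and starts a random timer; the timeout handler sets it and starts a second random timer.
; Pressing N triggers Surprise, which plays the surprise montage.
; Montage completion only prints a placeholder message for spawning a foreground enemy, and DestroyActor is left unwired.
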(event `self.ReceiveBeginPlay`
  (`self.InitializeActivity`)
  (`self.EnableInput` (`GameplayStatics.GetPlayerController` 0)))

(event `Key|N`
  (params (Key :type "Key Structure"))
  (:`Pressed`
    (`self.Surprise`)))

(event `Anim_Surprise`
  (`|PlayMontage` (`self.CommyCat`) "/Game/GA/Character_GA/Final/AnimFBX/BossEnemy/Boss_FBX_Anim_Armature_Enemy_BG_Surprise_Montage.Boss_FBX_Anim_Armature_Enemy_BG_Surprise_Montage"
    (:`OnCompleted`
      (`KismetSystemLibrary.PrintString` "Sapwn foreground enemy!"))))

(fn `InitializeActivity`
  (set `self.Activity?` false)
  (`KismetSystemLibrary.K2_SetTimerDelegate` (`|CreateDelegate` :!event `On Time Before Activity End`) (`KismetMathLibrary.RandomFloatInRange` (`self.MinTimeBeforeActivity`) (`self.MaxTimeBeforeActivity`))))

(fn `On Time Before Activity End`
  (set `self.Activity?` true)
  (`KismetSystemLibrary.K2_SetTimerDelegate` (`|CreateDelegate` :!event `InitializeActivity`) (`KismetMathLibrary.RandomFloatInRange` (`self.MinTimeEndActivity`) (`self.MaxTimeEndActivity`))))

(fn `Surprise`
  (`self.Anim_Surprise`))

(fn `UserConstructionScript`)