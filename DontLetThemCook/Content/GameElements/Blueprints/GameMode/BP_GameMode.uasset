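; Game mode that runs a switchable character party with shared health, plus music playback and a spectator camera for the zoo and credits levels.
; On BeginPlay in other non-menu levels it creates the HUD, initializes camera and health, and activates the first member.
; Switching teleports the new character into place and parks the old one at a prison position, gated by cooldown and air-switch limit.
; LoadData respawns the party from saved data; SaveData is stubbed.
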(event `self.ReceiveBeginPlay`
  (bind _ac_health (`self.AC_Health`))
  ;[1 1 1] C'est pas beau mais je sais pas comment faire autrement ^^'
  (bind _returnvalue (`GameplayStatics.GetCurrentLevelName` true))
  (if (`KismetStringLibrary.EqualEqual_StrStr` _returnvalue "Level_Menu")
    _
    (elif (or false (`KismetStringLibrary.EqualEqual_StrStr` _returnvalue "B3_07_Credit") (`KismetStringLibrary.EqualEqual_StrStr` _returnvalue "Level_Zoo"))
      (`self.SetToSpectatorMod`)
      (else
        (bind _returnvalue_2 (`|CreateWidget` "/Game/UI/Widget/Ingame/WG_MainWidget.WG_MainWidget_C" (`GameplayStatics.GetPlayerController` 0)))
        (bind _output_get (set `self.WG_Main` _returnvalue_2))
        (`UserWidget.AddToViewport` _output_get 0)
        (`KismetSystemLibrary.Delay` 0.5)
        (`self.InitializeCamera`)
        (`self.SwitchToCharacter` (`|GetArrayItem` (`self.PartyMembers`)) true)
        (`/Game/GameElements/Blueprints/Characters/AC_Health.InitializeHealth` _ac_health (`/Game/GameElements/Blueprints/Characters/AC_Health.MaxHealth` _ac_health))
        (add `/Game/GameElements/Blueprints/Characters/AC_Health.OnHealthDamaged` _ac_health (`|CreateDelegate` :!event `On Party Health Damaged`))
        (add `/Game/GameElements/Blueprints/Characters/AC_Health.OnHealthHealed` _ac_health (`|CreateDelegate` :!event `On Party Health Healed`))
        (add `/Game/GameElements/Blueprints/Characters/AC_Health.OnHealthReachedZero` _ac_health (`|CreateDelegate` :!event `On Party Health Reached Zero`))))))

(event `PlayMusic`
  (params (MusicToPlay :type "SoundBase Object Reference"))
  (bind _returnvalue (`GameplayStatics.SpawnSound2D` MusicToPlay 1.0 1.0 0.0 null))
  (set `self.PlayingMusic` _returnvalue)
  (`self.StartMusic`))

(event `StartMusic`
  (bind _playingmusic (`self.PlayingMusic`))
  (`/Engine/EditorBlueprintResources/StandardMacros.IsValid` (`self.PlayingMusic`)
    (:`Is Valid`
      (`AudioComponent.Stop` _playingmusic)
      (`AudioComponent.Play` _playingmusic 0.0)
      (`AudioComponent.FadeIn` _playingmusic 1.0 1.0 0.0 "Linear"))))

(event `StopMusic`
  (params (`Immediate?` :type Boolean))
  (bind _playingmusic (`self.PlayingMusic`))
  (`/Engine/EditorBlueprintResources/StandardMacros.IsValid` (`self.PlayingMusic`)
    (:`Is Valid`
      (if `Immediate?`
        (`AudioComponent.Stop` _playingmusic)
        (else
          (`AudioComponent.FadeOut` _playingmusic 1.0 0.0 "Linear")
          (`AudioComponent.StopDelayed` _playingmusic 1.0))))))

(fn `AddPartyMember`
  (params (`New Member` :type "/Game/GameElements/Blueprints/Characters/BP_PlayerCharacter_Master Object Reference"))
  (bind _wg_main (`self.WG_Main`))
  (if (< (`KismetArrayLibrary.Array_Find` (`self.PartyMembers`) `New Member`) 0)
    (`KismetArrayLibrary.Array_AddUnique` (`self.PartyMembers`) `New Member`)
    (`KismetSystemLibrary.PrintString` (`KismetStringLibrary.Concat_StrStr` "Added party member: " (`KismetSystemLibrary.GetDisplayName` `New Member`)))
    (`/Engine/EditorBlueprintResources/StandardMacros.IsValid` _wg_main
      (:`Is Valid`
        (`/Game/UI/Widget/Ingame/WG_MainWidget.StartDisplayChar` _wg_main "NewEnumerator1" (> (`KismetArrayLibrary.Array_Length` (`self.PartyMembers`)) 1))))
    (else
      (`KismetSystemLibrary.PrintString` "Character already within PartyMembers. Not adding." true true (struct :`R` 1.0 :`B` 0.085798 :`A` 1.0) 5.0))))

(fn `CanSwitch?`
  (returns (`CanSwitch?` :type Boolean))
  (return (and (not (or (`KismetSystemLibrary.K2_IsValidTimerHandle` (`self.SwitchCooldownTimer`)) (>= (`self.CurrentAirSwitches`) (`self.MaxAirSwitches`)))) (> (`KismetArrayLibrary.Array_Length` (`self.PartyMembers`)) 1))))

(fn `ClearSpawnPoints`
  (`KismetArrayLibrary.Array_Clear` (`self.SpawnPoints`))
  (set `self.DefaultSpawnPoint` null))

(fn `InitializeCamera`
  (if (`KismetSystemLibrary.IsValid` (`self.CameraManager`))
    (for _array_element (`self.PartyMembers`)
      (set `/Game/GameElements/Blueprints/Characters/BP_PlayerCharacter_Master.CurrentCamera` (`self.CameraManager`) _array_element))
    (else
      (`KismetSystemLibrary.PrintString` "No camera manager." true true (struct :`R` 1.0 :`B` 0.058244 :`A` 1.0) 5.0))))

(fn `LoadData`
  (params (PartyData :type "/Game/GameElements/Blueprints/DataSaving/F_PartyData Structure"))
  (bind (_partymembers _currentactivemember _partycharm _partyhealth) (break `/Game/GameElements/Blueprints/DataSaving/F_PartyData` PartyData))
  (bind _ac_health (`self.AC_Health`))
  (`KismetArrayLibrary.Array_Clear` (`self.PartyMembers`))
  (`|ExecutionSequence`
    (:`then_0`
      (for _array_element _partymembers
        (switch `/Game/GameElements/Blueprints/Characters/E_CharacterID` (`.CharacterID_6_BAC3B6564D162039221FD6BDD66E7322` (break `/Game/GameElements/Blueprints/DataSaving/F_CharacterData` _array_element))
          (:`NewEnumerator0`
            (bind _returnvalue (`|SpawnActorFromClass` "/Game/GameElements/Blueprints/Characters/BP_PlayerCharacter_Master.BP_PlayerCharacter_Master_C" (`KismetMathLibrary.MakeTransform` (`self.PartyPrisonPos`)) "AlwaysSpawn" "MultiplyWithRoot" null null))
            (`Pawn.SpawnDefaultController` _returnvalue)
            (`/Game/GameElements/Blueprints/Characters/BP_PlayerCharacter_Master.DeactivateCharacter` _returnvalue)
            (`self.AddPartyMember` _returnvalue))
          (:`NewEnumerator1`
            (bind _returnvalue_2 (`|SpawnActorFromClass` "/Game/GameElements/Blueprints/Characters/CharacterChildren/BP_Character_Poichon.BP_Character_Poichon_C" (`KismetMathLibrary.MakeTransform` (`self.PartyPrisonPos`)) "AlwaysSpawn" "MultiplyWithRoot" null null))
            (`Pawn.SpawnDefaultController` _returnvalue_2)
            (`/Game/GameElements/Blueprints/Characters/BP_PlayerCharacter_Master.DeactivateCharacter` _returnvalue_2)
            (`self.AddPartyMember` _returnvalue_2))
          (:`NewEnumerator2`
            (bind _returnvalue_3 (`|SpawnActorFromClass` "/Game/GameElements/Blueprints/Characters/CharacterChildren/BP_Character_Chappucino.BP_Character_Chappucino_C" (`KismetMathLibrary.MakeTransform` (`self.PartyPrisonPos`)) "AlwaysSpawn" "MultiplyWithRoot" null null))
            (`Pawn.SpawnDefaultController` _returnvalue_3)
            (`/Game/GameElements/Blueprints/Characters/BP_PlayerCharacter_Master.DeactivateCharacter` _returnvalue_3)
            (`self.AddPartyMember` _returnvalue_3)))))
    (:`then_1`
      (for _array_element_2 (`self.PartyMembers`)
        (if (`|EnumEquality` (`/Game/GameElements/Blueprints/Characters/BP_PlayerCharacter_Master.CharacterID` _array_element_2) _currentactivemember)
          (`self.InitializeCamera`)
          (`self.SwitchToCharacter` _array_element_2 true)
          (`KismetSystemLibrary.PrintString` "DATA LOADED!" true true (struct :`R` 0.136643 :`G` 1.0 :`A` 1.0) 5.0)
          (break))))
    (:`then_2`
      (`/Game/GameElements/Blueprints/Characters/AC_Health.DecreaseHealth` _ac_health (- (`/Game/GameElements/Blueprints/Characters/AC_Health.MaxHealth` _ac_health) _partyhealth)))))

(fn `LoadLevel`
  (params (`LoadData?` :type Boolean))
  (if `LoadData?`
    (`self.LoadData` (struct))))

(fn `On Party Health Damaged`
  (params (Source :type "Actor Object Reference") (Instigator :type "Actor Object Reference") (`Damage value` :type Integer) (`Hitstun?` :type Boolean) (KnockbackForceMultiplier :type "Float (double-precision)")))

(fn `On Party Health Healed`
  (params (HealValue :type Integer)))

(fn `On Party Health Reached Zero`
  (bind _currentactivecharacter (`self.CurrentActiveCharacter`))
  (for _array_element (`self.PartyMembers`)
    (`/Game/GameElements/Blueprints/Characters/BP_PlayerCharacter_Master.Die` _array_element))
  (`/Game/UI/Widget/Ingame/WG_MainWidget.LaunchDead` (`self.WG_Main`) (`self.K2_GetActorLocation` _currentactivecharacter) (`/Game/GameElements/Blueprints/Characters/BP_PlayerCharacter_Master.FacingRight` _currentactivecharacter))
  (`self.StopMusic` true)
  (`GameplayStatics.SpawnSound2D` "/Game/Sound/SoundFiles/death_01.death_01" 1.0 1.0 0.0 null))

(fn `On Switch Cooldown Ended`
  (bind _switchcooldowntimer (`self.SwitchCooldownTimer`))
  (if (`KismetSystemLibrary.K2_IsValidTimerHandle` _switchcooldowntimer)
    (`KismetSystemLibrary.K2_ClearAndInvalidateTimerHandle` _switchcooldowntimer)))

(fn `OnCharacterLanded`
  (params (LandedCharacter :type "/Game/GameElements/Blueprints/Characters/BP_PlayerCharacter_Master Object Reference"))
  (if (== LandedCharacter (`self.CurrentActiveCharacter`))
    (`KismetSystemLibrary.PrintString` "Character landed!")
    (set `self.CurrentAirDashes` 0)
    (set `self.CurrentAirSwitches` 0)
    (set `self.CurrentJumps` 0)))

(fn `RegisterSpawnPoint`
  (params (SpawnPoint :type "/Game/GameElements/Blueprints/Levels/BP_LevelSpawnPoint Object Reference"))
  (if (`/Game/GameElements/Blueprints/Levels/BP_LevelSpawnPoint.DefaultSpawnPoint` SpawnPoint)
    (set `self.DefaultSpawnPoint` SpawnPoint)
    (else
      (`KismetArrayLibrary.Array_AddUnique` (`self.SpawnPoints`) SpawnPoint))))

(fn `RemovePartyMember`
  (params (PartyMember :type "/Game/GameElements/Blueprints/Characters/BP_PlayerCharacter_Master Object Reference"))
  (bind _returnvalue (`KismetArrayLibrary.Array_RemoveItem` (`self.PartyMembers`) PartyMember))
  (if _returnvalue
    (`KismetSystemLibrary.PrintString` (`KismetStringLibrary.Concat_StrStr` "Removed " (`KismetSystemLibrary.GetDisplayName` PartyMember) " from the party!") true true (struct :`R` 1.0 :`G` 0.360092 :`A` 1.0) 5.0)
    (else
      (`KismetSystemLibrary.PrintString` "Nothing was removed from the party." true true (struct :`R` 1.0 :`G` 0.051568 :`A` 1.0) 5.0))))

(fn `SaveData`
  (returns (SaveData :type "/Game/GameElements/Blueprints/DataSaving/F_PartyData Structure"))
  (locals (LocalPartyMembers :type "Array of /Game/GameElements/Blueprints/DataSaving/F_CharacterData Structure") (LocalCurrentActiveCharacterID :type "/Game/GameElements/Blueprints/Characters/E_CharacterID Enum") (LocalPartyCharm :type Integer)))

(fn `SendCachedCharacterToPrison`
  (bind _cachedcharactertosend (`self.CachedCharacterToSend`))
  (`/Engine/EditorBlueprintResources/StandardMacros.IsValid` _cachedcharactertosend
    (:`Is Valid`
      (`self.K2_SetActorLocation` _cachedcharactertosend (`self.PartyPrisonPos`) false true))))

(fn `SetCurrentActiveCharacter`
  (params (CurrentActiveCharacter :type "/Game/GameElements/Blueprints/Characters/BP_PlayerCharacter_Master Object Reference"))
  (bind _output_get (set `self.CurrentActiveCharacter` CurrentActiveCharacter)))

(fn `SetDialogueMode`
  (params (`InDialogue?` :type Boolean) (Dialoguer :type "/Game/GameElements/Blueprints/Dialogue/AC_Dialoguer Object Reference"))
  (`/Game/GameElements/Blueprints/Camera/BP_CameraManager.SetDialogueMode` (`self.CameraManager`) `InDialogue?` Dialoguer))

(fn `SetToSpectatorMod`
  (bind _returnvalue (`|SpawnActorFromClass` "/Game/GameElements/Blueprints/Camera/SpectatorCam/BP_SpectatorCamera.BP_SpectatorCamera_C" (`KismetMathLibrary.MakeTransform` (0.0 -200.0 200.0)) "AdjustIfPossibleButAlwaysSpawn" "MultiplyWithRoot" null null))
  (`Controller.Possess` (`GameplayStatics.GetPlayerController` 0) _returnvalue))

(fn `SwitchCharacterBackward`
  (bind _partymembers (`self.PartyMembers`))
  (bind _returnvalue (`KismetArrayLibrary.Array_Find` _partymembers (`self.CurrentActiveCharacter`)))
  (if (> (`KismetArrayLibrary.Array_Length` (`self.PartyMembers`)) 1)
    (if (> _returnvalue 0)
      (`self.SwitchToCharacter` (`|GetArrayItem` _partymembers (- _returnvalue 1)))
      (else
        (`self.SwitchToCharacter` (`|GetArrayItem` _partymembers (- (`KismetArrayLibrary.Array_Length` _partymembers) 1)))))
    (else
      (`KismetSystemLibrary.PrintString` "PartyMembers length is 0 or 1. Not switching." true true (struct :`R` 1.0 :`B` 0.061241 :`A` 1.0) 5.0))))

(fn `SwitchCharacterForward`
  (bind _partymembers (`self.PartyMembers`))
  (bind _returnvalue (+ (`KismetArrayLibrary.Array_Find` _partymembers (`self.CurrentActiveCharacter`)) 1))
  (if (> (`KismetArrayLibrary.Array_Length` (`self.PartyMembers`)) 1)
    (if (< _returnvalue (`KismetArrayLibrary.Array_Length` _partymembers))
      (`self.SwitchToCharacter` (`|GetArrayItem` _partymembers _returnvalue))
      (else
        (`self.SwitchToCharacter` (`|GetArrayItem` _partymembers))))
    (else
      (`KismetSystemLibrary.PrintString` "PartyMembers length is 0 or 1. Not switching." true true (struct :`R` 1.0 :`B` 0.061241 :`A` 1.0) 5.0))))

(fn `SwitchToCharacter`
  (params (ToCharacter :type "/Game/GameElements/Blueprints/Characters/BP_PlayerCharacter_Master Object Reference") (ForceSwitch :type Boolean))
  (locals (ActiveCharacterPosition :type "Vector Structure") (PreviousCharacterInAir :type Boolean))
  (bind _currentactivecharacter (`self.CurrentActiveCharacter`))
  (bind _currentactivecharacter_2 (`self.CurrentActiveCharacter`))
  (if ForceSwitch
    (if (>= (`KismetArrayLibrary.Array_Find` (`self.PartyMembers`) ToCharacter) 0) :!label _label
      (if (== ToCharacter (`self.CurrentActiveCharacter`))
        (`KismetSystemLibrary.PrintString` "Selected character is currently active one. Not switching." true true (struct :`R` 1.0 :`B` 0.03671 :`A` 1.0) 5.0)
        (else
          (if (`KismetSystemLibrary.IsValid` _currentactivecharacter)
            (set `local.ActiveCharacterPosition` (`self.K2_GetActorLocation` _currentactivecharacter))
            (set `local.PreviousCharacterInAir` (`/Game/GameElements/Blueprints/Characters/BP_PlayerCharacter_Master.IsCharacterInAir?` _currentactivecharacter))
            (`/Game/GameElements/Blueprints/Characters/BP_PlayerCharacter_Master.DeactivateCharacter` _currentactivecharacter)
            (set `self.CachedCharacterToSend` _currentactivecharacter)
            (`KismetSystemLibrary.K2_SetTimerDelegate` (`|CreateDelegate` :!event `SendCachedCharacterToPrison`) (`self.SwitchTime`))
            (else
              ;[1 0.05177 0] Default placement. Replace by SpawnPoint.
              (set `local.ActiveCharacterPosition` (`self.K2_GetActorLocation` (`self.DefaultSpawnPoint`)))
              (`KismetSystemLibrary.PrintString` "No ActiveCharacterPosition, placed at SpawnPoint!" true true (struct :`R` 1.0 :`B` 0.066903 :`A` 1.0) 5.0)))
          (`self.K2_SetActorLocation` ToCharacter (`local.ActiveCharacterPosition`) false true)
          (`/Game/GameElements/Blueprints/Characters/BP_PlayerCharacter_Master.ActivateCharacter` ToCharacter)
          (`self.SetCurrentActiveCharacter` ToCharacter)
          (bind _returnvalue (`KismetSystemLibrary.K2_SetTimerDelegate` (`|CreateDelegate` :!event `On Switch Cooldown Ended`) (`self.SwitchCooldownDuration`)))
          (set `self.SwitchCooldownTimer` _returnvalue)
          (`/Game/GameElements/Blueprints/Characters/BP_PlayerCharacter_Master.OnCharacterSwitch` _currentactivecharacter_2 (`local.PreviousCharacterInAir`))
          (`KismetSystemLibrary.PrintString` (`KismetStringLibrary.Concat_StrStr` "Switched to " (`KismetSystemLibrary.GetDisplayName` _currentactivecharacter_2)))
          (`/Game/UI/Widget/Ingame/WG_MainWidget.ChangeCharacter` (`self.WG_Main`) (`/Game/GameElements/Blueprints/Characters/BP_PlayerCharacter_Master.CharacterID` _currentactivecharacter_2))))
      (else
        (`KismetSystemLibrary.PrintString` "Selected character isn't in party members. Not switching." true true (struct :`R` 1.0 :`G` 0.044237 :`A` 1.0) 5.0)))
    (elif (`self.CanSwitch?`)
      (goto _label)
      (else
        (`KismetSystemLibrary.PrintString` "Can't switch right now. Not switching." true true (struct :`R` 1.0 :`G` 0.044237 :`A` 1.0) 5.0)))))

(fn `UserConstructionScript`)