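; Game instance that holds party data and passes it back to the game mode on load.
; SaveData builds a party struct from each member's ID and AC_Health current health, plus the active character's ID and a zeroed charm value, then prints debug confirmation.
; LoadData hands the stored struct to BP_GameMode and has it initialize the camera.
; The data lives in memory, with no SaveGame write shown.
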(fn `Load Data`
  (bind _asbp_game_mode (cast `/Game/GameElements/Blueprints/GameMode/BP_GameMode` (`GameplayStatics.GetGameMode`)))
  (`/Game/GameElements/Blueprints/GameMode/BP_GameMode.LoadData` _asbp_game_mode (`self.PartyData`))
  (`/Game/GameElements/Blueprints/GameMode/BP_GameMode.InitializeCamera` _asbp_game_mode))

(fn `Save Data`
  (params (CurrentActiveCharacter :type "/Game/GameElements/Blueprints/Characters/BP_PlayerCharacter_Master Object Reference") (PartyMembers :type "Array of /Game/GameElements/Blueprints/Characters/BP_PlayerCharacter_Master Object Reference"))
  (returns (SaveData :type "/Game/GameElements/Blueprints/DataSaving/F_PartyData Structure"))
  (locals (LocalPartyMembers :type "Array of /Game/GameElements/Blueprints/DataSaving/F_CharacterData Structure") (LocalPartyCharm :type Integer) (LocalCurrentActiveCharacterID :type "/Game/GameElements/Blueprints/Characters/E_CharacterID Enum"))
  (set `self.PartyData` (struct))
  (`|ExecutionSequence`
    (:`then_0`
      (for _array_element PartyMembers
        (`KismetArrayLibrary.Array_AddUnique` (`local.LocalPartyMembers`) (make `/Game/GameElements/Blueprints/DataSaving/F_CharacterData` (`/Game/GameElements/Blueprints/Characters/BP_PlayerCharacter_Master.CharacterID` _array_element) (`/Game/GameElements/Blueprints/Characters/AC_Health.CurrentHealth` (`Actor.GetComponentByClass` _array_element "/Game/GameElements/Blueprints/Characters/AC_Health.AC_Health_C"))))))
    (:`then_1`
      (set `local.LocalCurrentActiveCharacterID` (`/Game/GameElements/Blueprints/Characters/BP_PlayerCharacter_Master.CharacterID` CurrentActiveCharacter)))
    (:`then_2`
      (set `local.LocalPartyCharm` 0))
    (:`then_3`
      (bind _output_get (set `self.PartyData` (make `/Game/GameElements/Blueprints/DataSaving/F_PartyData` (`local.LocalPartyMembers`) (`local.LocalCurrentActiveCharacterID`) (`local.LocalPartyCharm`))))
      (`KismetSystemLibrary.PrintString` "DATA SAVED!" true true (struct :`R` 0.02247 :`G` 1.0 :`A` 1.0) 5.0)
      (`KismetSystemLibrary.PrintString` (`KismetStringLibrary.Conv_IntToString` (`KismetArrayLibrary.Array_Length` (`.PartyMembers_4_C80301B047991FC07E3244BBF3FDFE40` (break `/Game/GameElements/Blueprints/DataSaving/F_PartyData` _output_get)))))
      (return _output_get))))