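; BP_Ventilo is a fan level element that can be switched on and off, controlling the wind of its linked vents.
; On BeginPlay it applies its IsActive state, and while active Tick spins the actor around local yaw by Rotation scaled by delta time.
; ActiveVentilo and DesactiveVentilo set that state and toggle wind on every BPVent entry; only activation also plays a Timeline.
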(event `self.ReceiveBeginPlay`
  (if (`self.is_Active`)
    (`self.ActiveVentilo`)
    (else
      (`self.DesactiveVentilo`))))

(event `self.ReceiveTick`
  (params (DeltaSeconds :type "Float (single-precision)"))
  (if (`self.is_Active`)
    (`self.K2_AddActorLocalRotation` (`KismetMathLibrary.MakeRotator` 0.0 0.0 (* DeltaSeconds (`self.Rotation`))))))

(event `ActiveVentilo`
  (set `self.is_Active` true)
  (for _array_element (`self.BP_Vent`)
    (`/Game/GameElements/Blueprints/LevelElement/BP_WindVentilo.Active_Wind` _array_element))
  (`Timeline|Timeline`))

(event `DesactiveVentilo`
  (set `self.is_Active` false)
  (for _array_element (`self.BP_Vent`)
    (`/Game/GameElements/Blueprints/LevelElement/BP_WindVentilo.Desactive_Wind` _array_element)))

(fn `UserConstructionScript`)