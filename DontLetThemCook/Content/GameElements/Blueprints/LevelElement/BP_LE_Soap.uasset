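; A soap level element that falls from its placed spot to a destination when a Character touches it.
; BeginPlay caches the location of DestinationActor as the target, printing a warning if none is set.
; The first Character overlap on Box_Interaction fires SoapFailing, where a timeline lerps location and rotation on separate alphas toward DestVec and DestRot.
; A second Box overlap only casts to Character and does nothing further.
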(event `self.ReceiveBeginPlay`
  (bind _destinationactor (`self.DestinationActor`))
  (`/Engine/EditorBlueprintResources/StandardMacros.IsValid` _destinationactor
    (:`Is Valid`
      (set `self.Dest_Vec` (`self.K2_GetActorLocation` _destinationactor)))
    (:`Is Not Valid`
      (`KismetSystemLibrary.PrintString` "NOT SET DESTINATION SOAP"))))

(event `SoapFailing`
  (set `self.Orig_Rot` (`self.K2_GetActorRotation`))
  (set `self.Orig_Vec` (`self.K2_GetActorLocation`))
  (bind (_direction _alphafall _alpharot) (`Timeline|Timeline` :!via `PlayFromStart`)
    (:`Update`
      (`self.K2_SetActorLocation` (`KismetMathLibrary.VLerp` (`self.Orig_Vec`) (`self.Dest_Vec`) _alphafall))
      (`self.K2_SetActorRotation` (`KismetMathLibrary.RLerp` (`self.Orig_Rot`) (`self.Dest_Rot`) _alpharot)))))

(event `self.Box_Interaction.OnComponentBeginOverlap`
  (params (OverlappedComponent :type "PrimitiveComponent Object Reference") (OtherActor :type "Actor Object Reference") (OtherComp :type "PrimitiveComponent Object Reference") (OtherBodyIndex :type Integer) (bFromSweep :type Boolean) (SweepResult :type "HitResult Structure (by ref)"))
  (cast `Character` OtherActor)
  (`KismetSystemLibrary.PrintString` "Soap_isPush")
  (`/Engine/EditorBlueprintResources/StandardMacros.DoOnce` false
    (:`Completed`
      (`self.SoapFailing`))))

(event `self.Box.OnComponentBeginOverlap`
  (params (OverlappedComponent :type "PrimitiveComponent Object Reference") (OtherActor :type "Actor Object Reference") (OtherComp :type "PrimitiveComponent Object Reference") (OtherBodyIndex :type Integer) (bFromSweep :type Boolean) (SweepResult :type "HitResult Structure (by ref)"))
  (cast `Character` OtherActor))

(fn `UserConstructionScript`)