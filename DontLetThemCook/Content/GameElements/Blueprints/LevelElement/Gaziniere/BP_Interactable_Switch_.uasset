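; Interactable switch that toggles between left and right groups of gas stoves (gazinière) when flagged for stove use.
; Each accepted interaction flips the side, activates that side's stoves, deactivates the other side's and plays a button sound.
; A Timeline rotates the button mesh between its initial rotation and a 90-degree yaw offset.
; IsPush blocks retriggering until the Timeline finishes, or permanently when StayPush is set.
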(event `self.ReceiveBeginPlay`
  (bind _output_get (set `self.RelativeLeft` (`SceneComponent.RelativeRotation` (`self.SM_Bouton`))))
  (set `self.RelativeRight` (`KismetMathLibrary.MakeRotator` (.roll _output_get) (.pitch _output_get) (- (.yaw _output_get) 90.0)))
  (`parent.ReceiveBeginPlay`))

(event `ActiveButton`
  (if (`self.is_Left`)
    (bind (_direction _newtrack_0) (`Timeline|Timeline` :!via `Reverse` :!label _label)
      (:`Update`
        (`SceneComponent.K2_SetRelativeRotation` (`self.SM_Bouton`) (`KismetMathLibrary.RLerp` (`self.RelativeLeft`) (`self.RelativeRight`) _newtrack_0) false false))
      (:`Finished`
        (if (not (`self.StayPush`))
          (set `self.Is_Push` false)
          (`/Game/GameElements/Blueprints/Levels/AC_Interactible.EndInteract` (`self.AC_Interactible`))
          (`KismetSystemLibrary.PrintString` "END" true true (struct :`R` 1.0 :`G` 0.008232 :`A` 1.0)))))
    (else
      (goto _label))))

(event `self.InteractionEvent`
  ;[1 1 1] Activation Button
  ;;[1 1 1] En attendant la compétence
  (if (not (`self.Is_Push`))
    (`self.ClickOnBut`)))

(event `ClickOnBut`
  ;[1 1 1] Activation Button
  (set `self.Is_Push` true)
  (set `self.is_Left` (not (`self.is_Left`)))
  ;;[1 1 1] Active Gaziniere
  (if (`self.Is_ForGaziniere`)
    (if (`self.is_Left`)
      (for _array_element (`self.Gaziniere_Left`)
        (`/Game/GameElements/Blueprints/LevelElement/Gaziniere/BP_Gaziniere.ActiveGaziniere` _array_element))
      (for _array_element_2 (`self.Gaziniere_Right`)
        (`/Game/GameElements/Blueprints/LevelElement/Gaziniere/BP_Gaziniere.DesactiveGaziniere` _array_element_2))
      (else
        (for _array_element_3 (`self.Gaziniere_Left`)
          (`/Game/GameElements/Blueprints/LevelElement/Gaziniere/BP_Gaziniere.DesactiveGaziniere` _array_element_3))
        (for _array_element_4 (`self.Gaziniere_Right`)
          (`/Game/GameElements/Blueprints/LevelElement/Gaziniere/BP_Gaziniere.ActiveGaziniere` _array_element_4))))
    (else
      (`KismetSystemLibrary.PrintString` "Is NOT FOR HOTTE")))
  (`self.ActiveButton`)
  (`GameplayStatics.SpawnSoundAtLocation` "/Game/Sound/SoundFiles/Button_1.Button_1" (`self.K2_GetActorLocation`) (struct) 1.0 1.0 0.0 null null))

(fn `UserConstructionScript`
  (`parent.UserConstructionScript`))