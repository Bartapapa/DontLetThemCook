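; BP_Gaziniere is a gas burner hazard that can be switched on or off, starting in the state set by IsOn.
; Activation turns on Niagara fire, burst and crackle sounds and the damage collider, then shuts off after Duration unless time is infinite.
; Overlapping actors with AC_Health take damage with hitstun and knockback.
; When it has a saucepan, both state changes also toggle that saucepan's hot state.
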(event `self.ReceiveBeginPlay`
  (if (`self.is_On`)
    (`self.ActiveGaziniere`)
    (else
      (`self.DesactiveGaziniere`))))

(event `ActiveGaziniere`
  (set `self.is_On` true)
  (`ActorComponent.Activate` (`self.NiagaraFire`) false)
  (`ActorComponent.Activate` (`self.NiagaraBurst`) false)
  (`PrimitiveComponent.SetCollisionEnabled` (`self.DamageCollider`) "QueryAndPhysics")
  (`GameplayStatics.SpawnSoundAtLocation` "/Game/Sound/SoundFiles/Fire_Burst_Cue.Fire_Burst_Cue" (`self.K2_GetActorLocation`) (struct) 1.0 1.0 0.0 null null)
  (bind _returnvalue (`GameplayStatics.SpawnSoundAtLocation` "/Game/Sound/SoundFiles/Fire_Crackle_Cue.Fire_Crackle_Cue" (`self.K2_GetActorLocation`) (struct) 1.0 1.0 0.0 null null))
  (set `self.FlameLoop` _returnvalue)
  (if (`self.HasSaucePan`)
    (`/Game/GameElements/Blueprints/LevelElement/BP_Saucepan.ActiveHot` (`self.Saucepan_Ref`)))
  (if (not (`self.Have_InfiniteTime`))
    (`KismetSystemLibrary.Delay` (`self.Duration`))
    (if (`self.is_On`)
      (`self.DesactiveGaziniere`))))

(event `DesactiveGaziniere`
  (bind _flameloop (`self.FlameLoop`))
  (set `self.is_On` false)
  (`ActorComponent.Deactivate` (`self.NiagaraFire`))
  (`ActorComponent.Deactivate` (`self.NiagaraBurst`))
  (`PrimitiveComponent.SetCollisionEnabled` (`self.DamageCollider`) "NoCollision")
  (if (`KismetSystemLibrary.IsValid` _flameloop)
    (`AudioComponent.Stop` _flameloop)
    (set `self.FlameLoop` null))
  (if (`self.HasSaucePan`)
    (`/Game/GameElements/Blueprints/LevelElement/BP_Saucepan.DesactiveHot` (`self.Saucepan_Ref`))))

(event `self.ReceiveActorBeginOverlap`
  (params (OtherActor :type "Actor Object Reference"))
  (bind _returnvalue (`self.GetComponentByClass` OtherActor "/Game/GameElements/Blueprints/Characters/AC_Health.AC_Health_C"))
  (`/Engine/EditorBlueprintResources/StandardMacros.IsValid` _returnvalue
    (:`Is Valid`
      (`/Game/GameElements/Blueprints/Characters/AC_Health.Damage` _returnvalue self self "NewEnumerator0" 1 "NewEnumerator2" true 0.5))))

(event `self.DamageCollider.OnComponentEndOverlap`
  (params (OverlappedComponent :type "PrimitiveComponent Object Reference") (OtherActor :type "Actor Object Reference") (OtherComp :type "PrimitiveComponent Object Reference") (OtherBodyIndex :type Integer)))

(fn `UserConstructionScript`)