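; BP_SmokeWind is a level element: a Niagara smoke wind, activated when both its pan-hot and hood (hotte) flags are set and deactivated when either clears.
; While active, its box tracks the overlapping player and toggles Chapuccino's cloud ability on entry and exit.
; Tick interpolates Chapuccino's velocity, or Poichon's if Y force is nonzero, toward LaunchForce, adding a small hop when grounded with upward force.
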(event `self.ReceiveBeginPlay`
  (if (`self.is_Active`)
    (`self.Active_SmokeWind` false)
    (`self.Active_SmokeWind` true)
    (else
      (`self.Desactive_SmokeWind` false))))

(event `Desactive_SmokeWind`
  (params (is_From_Sauce_Pan :type Boolean))
  ;[1 1 1] Gestion de si actif
  (if is_From_Sauce_Pan
    (set `self.is_PanHot` false)
    (else
      (set `self.is_HotteActive` false)))
  (set `self.is_Active` false)
  (`ActorComponent.Deactivate` (`self.Niagara`)))

(event `Active_SmokeWind`
  (params (is_From_SaucePan :type Boolean))
  ;[1 1 1] Gestion de si actif
  (if is_From_SaucePan
    (set `self.is_PanHot` true)
    (else
      (set `self.is_HotteActive` true)))
  (if (and (`self.is_HotteActive`) (`self.is_PanHot`))
    (set `self.is_Active` true)
    (`ActorComponent.Activate` (`self.Niagara`) false)))

(event `self.Box.OnComponentBeginOverlap`
  (params (OverlappedComponent :type "PrimitiveComponent Object Reference") (OtherActor :type "Actor Object Reference") (OtherComp :type "PrimitiveComponent Object Reference") (OtherBodyIndex :type Integer) (bFromSweep :type Boolean) (SweepResult :type "HitResult Structure (by ref)"))
  (bind _player_ref (`self.Player_Ref`))
  (if (`self.Is_Active`)
    (bind _asbp_player_character_master (cast `/Game/GameElements/Blueprints/Characters/BP_PlayerCharacter_Master` OtherActor))
    (`/Engine/EditorBlueprintResources/StandardMacros.IsValid` _asbp_player_character_master
      (:`Is Valid`
        (set `self.Player_Ref` _asbp_player_character_master)
        (switch `/Game/GameElements/Blueprints/Characters/E_CharacterID` (`/Game/GameElements/Blueprints/Characters/BP_PlayerCharacter_Master.CharacterID` _player_ref)
          (:`NewEnumerator2`
            (bind _asbp_character_chappucino (cast `/Game/GameElements/Blueprints/Characters/CharacterChildren/BP_Character_Chappucino` _player_ref))
            (if (not (`/Game/GameElements/Blueprints/Characters/CharacterChildren/BP_Character_Chappucino.IsCloud?` _asbp_character_chappucino))
              (`/Game/GameElements/Blueprints/Characters/BP_PlayerCharacter_Master.Call Special Ability` _asbp_character_chappucino))))))))

(event `self.Box.OnComponentEndOverlap`
  (params (OverlappedComponent :type "PrimitiveComponent Object Reference") (OtherActor :type "Actor Object Reference") (OtherComp :type "PrimitiveComponent Object Reference") (OtherBodyIndex :type Integer))
  (if (`self.Is_Active`)
    (bind _asbp_player_character_master (cast `/Game/GameElements/Blueprints/Characters/BP_PlayerCharacter_Master` OtherActor))
    (`/Engine/EditorBlueprintResources/StandardMacros.IsValid` _asbp_player_character_master
      (:`Is Valid`
        (set `self.Player_Ref` null)
        (switch `/Game/GameElements/Blueprints/Characters/E_CharacterID` (`/Game/GameElements/Blueprints/Characters/BP_PlayerCharacter_Master.CharacterID` _asbp_player_character_master)
          (:`NewEnumerator2`
            (bind _asbp_character_chappucino (cast `/Game/GameElements/Blueprints/Characters/CharacterChildren/BP_Character_Chappucino` _asbp_player_character_master))
            (if (`/Game/GameElements/Blueprints/Characters/CharacterChildren/BP_Character_Chappucino.IsCloud?` _asbp_character_chappucino)
              (`/Game/GameElements/Blueprints/Characters/BP_PlayerCharacter_Master.Call Special Ability` _asbp_character_chappucino))))))))

(event `self.ReceiveTick`
  (params (DeltaSeconds :type "Float (single-precision)"))
  (bind (_launchforce_x _launchforce_y) (`KismetMathLibrary.BreakVector` (`self.LaunchForce`)))
  (if (`self.is_Active`)
    (`/Engine/EditorBlueprintResources/StandardMacros.IsValid` (`self.Player_Ref`)
      (:`Is Valid`
        (switch `/Game/GameElements/Blueprints/Characters/E_CharacterID` (`/Game/GameElements/Blueprints/Characters/BP_PlayerCharacter_Master.CharacterID` (`self.Player_Ref`))
          (:`NewEnumerator1`
            (if (!= _launchforce_y 0.0)
              (`self.HandlePlayerRefApplyForce` :!label _label)))
          (:`NewEnumerator2`
            (goto _label)))))))

(fn `HandlePlayerRefApplyForce`
  (locals (ToYLaunchForce :type "Float (double-precision)") (ToZLaunchForce :type "Float (double-precision)"))
  (bind (_launchforce_x _launchforce_y _launchforce_z) (`KismetMathLibrary.BreakVector` (`self.LaunchForce`)))
  (bind _y (.y (`self.LaunchForce`)))
  (if (!= _y 0.0)
    (set `local.ToYLaunchForce` _y)
    (else
      (set `local.ToYLaunchForce` (.y (`MovementComponent.Velocity` (`Character.CharacterMovement` (`self.Player_Ref`)))))))
  (if true
    (set `local.ToZLaunchForce` (.z (`self.LaunchForce`)))
    (else
      (set `local.ToZLaunchForce` (.z (`MovementComponent.Velocity` (`Character.CharacterMovement` (`self.Player_Ref`)))))))
  (if (and (not (`NavMovementComponent.IsFalling` (`Character.CharacterMovement` (`self.Player_Ref`)))) (> _launchforce_z 0.0))
    ;[1 1 1] Make a little jump if Force Z
    (`Character.LaunchCharacter` (`self.Player_Ref`) (0.0 0.0 50.0) false false))
  (set `MovementComponent.Velocity` (`KismetMathLibrary.VInterpTo` (`MovementComponent.Velocity` (`Character.CharacterMovement` (`self.Player_Ref`))) (`KismetMathLibrary.MakeVector` 0.0 (`local.ToYLaunchForce`) (`local.ToZLaunchForce`)) (`GameplayStatics.GetWorldDeltaSeconds`) (`self.InterpolationSpeed`)) (`Character.CharacterMovement` (`self.Player_Ref`))))

(fn `UserConstructionScript`)