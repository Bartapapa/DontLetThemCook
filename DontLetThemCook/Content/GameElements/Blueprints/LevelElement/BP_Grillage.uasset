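; BP_Grillage is a level element actor, a grillage that moves vertically between its placed position and an offset position.
; BeginPlay stores the start location and computes the destination by adding NumberOfOfset on Z.
; ActiveGrillage plays a timeline that lerps the actor's location toward the destination without sweep, and DesactiveGrillage reverses that timeline to bring it back.
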(event `self.ReceiveBeginPlay`
  (bind _output_get (set `self.Orig` (`self.K2_GetActorLocation`)))
  (set `self.Dest` (`KismetMathLibrary.MakeVector` (.x _output_get) (.y _output_get) (+ (.z _output_get) (`self.NumberOfOfset`)))))

(event `ActiveGrillage`
  (bind (_direction _newtrack_0) (`Timeline|Timeline` :!label _label)
    (:`Update`
      (`self.K2_SetActorLocation` (`KismetMathLibrary.VLerp` (`self.Orig`) (`self.Dest`) _newtrack_0)))))

(event `DesactiveGrillage`
  (goto _label :!via `Reverse`))

(fn `UserConstructionScript`)