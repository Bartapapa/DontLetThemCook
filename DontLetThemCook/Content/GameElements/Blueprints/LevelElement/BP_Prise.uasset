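; Electric socket switch (prise) that toggles linked fans or a grid actor (grillage) when hit by a Poichon projectile.
; Each trigger flips an on/off state, calls the targets, then applies an electrified material and Niagara effect.
; IsPush blocks retriggering until a Character leaves the box, unless StayPush keeps it pressed.
; The grid branch requires DebugGrillage, and the button-press timeline is unconnected.
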(event `ActiveButton`
  (bind _niagara (`self.Niagara`))
  (if (`self.StayPush`)
    (`/Engine/EditorBlueprintResources/StandardMacros.DoOnce` false
      (:`Completed`
        (`ActorComponent.Activate` _niagara false :!label _label)))
    (else
      (`/Engine/EditorBlueprintResources/StandardMacros.FlipFlop`
        (:`A`
          (goto _label))
        (:`B`
          (`ActorComponent.Deactivate` _niagara)))))
  (`PrimitiveComponent.SetMaterial` (`self.SM_Bouton`) 0 (`self.Material_Elec`))
  (`ActorComponent.Activate` (`self.Niagara`) false))

(event `InverseButton`)

(event `self.ReceiveBeginPlay`
  (add `/Game/GameElements/Blueprints/Characters/AC_PoichonProjectileInteractible.OnPoichonProjectileInteracted` (`self.AC_PoichonProjectileInteractible`) (delegate `TriggerTheEffect`)))

(event `self.Box.OnComponentBeginOverlap`
  (params (OverlappedComponent :type "PrimitiveComponent Object Reference") (OtherActor :type "Actor Object Reference") (OtherComp :type "PrimitiveComponent Object Reference") (OtherBodyIndex :type Integer) (bFromSweep :type Boolean) (SweepResult :type "HitResult Structure (by ref)"))
  (cast `Character` OtherActor))

(event `TriggerTheEffect`
  ;[1 1 1] Activation Button
  (if (`self.StayPush`)
    (`/Engine/EditorBlueprintResources/StandardMacros.DoOnce` false
      (:`Completed`
        _)))
  (if (not (`self.Is_Push`))
    (set `self.Is_Push` true)
    (`self.ClickOnBut`)))

(event `ClickOnBut`
  (bind _bp_ventilo_ref (`self.BP_Ventilo_Ref`))
  (bind _actorgrillage (`self.ActorGrillage`))
  ;[1 1 1] Activation Button
  (set `self.Is_Ventilo_Grillage_On` (not (`self.Is_Ventilo_Grillage_On`)))
  ;;[1 1 1] Active Ventilo
  (if (`self.Is_PourVentilo`)
    (if (`self.Is_Ventilo_Grillage_On`)
      (for _array_element _bp_ventilo_ref
        (`/Engine/EditorBlueprintResources/StandardMacros.IsValid` _array_element
          (:`Is Valid`
            (`/Game/GameElements/Blueprints/LevelElement/BP_Ventilo.ActiveVentilo` _array_element)
            (`self.ActiveButton` :!label _label_2))))
      (else
        (for _array_element_2 _bp_ventilo_ref
          (`/Engine/EditorBlueprintResources/StandardMacros.IsValid` _array_element_2
            (:`Is Valid`
              (`/Game/GameElements/Blueprints/LevelElement/BP_Ventilo.DesactiveVentilo` _array_element_2)
              (goto _label_2))))))
    (elif (`self.DebugGrillage`)
      (if (`self.Is_Ventilo_Grillage_On`)
        (`/Game/GameElements/Blueprints/LevelElement/BP_Grillage.ActiveGrillage` _actorgrillage)
        (else
          (`/Game/GameElements/Blueprints/LevelElement/BP_Grillage.DesactiveGrillage` _actorgrillage)))
      (else
        (`KismetSystemLibrary.PrintString` "Is NOT FOR GRILLAGE \nIs NOT FOR VENTILO"))))
  (goto _label_2))

(event `self.Box.OnComponentEndOverlap`
  (params (OverlappedComponent :type "PrimitiveComponent Object Reference") (OtherActor :type "Actor Object Reference") (OtherComp :type "PrimitiveComponent Object Reference") (OtherBodyIndex :type Integer))
  ;[1 1 1] Activation Button
  (cast `Character` OtherActor)
  (if (not (`self.StayPush`))
    (set `self.Is_Push` false)))

(fn `UserConstructionScript`)