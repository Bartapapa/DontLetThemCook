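; Bottle level element (apparently soap) that topples toward a destination actor the first time a character overlaps its interaction box.
; BeginPlay caches the target location, then a timeline moves the bottle along separate Y and Z curves, keeping X, while rotating it to DestRot.
; When the fall finishes, it optionally activates a linked bumper actor and starts a second timeline that animates the cylinder's height and roll as a floating motion.
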(event `self.ReceiveBeginPlay`
  (bind _destinationactor (`self.DestinationActor`))
  (`/Engine/EditorBlueprintResources/StandardMacros.IsValid` _destinationactor
    (:`Is Valid`
      (set `self.Dest_Vec` (`self.K2_GetActorLocation` _destinationactor)))
    (:`Is Not Valid`
      (`KismetSystemLibrary.PrintString` "NOT SET DESTINATION SOAP"))))

(event `SoapFailing`
  (bind (_dest_vec_x _dest_vec_y _dest_vec_z) (`KismetMathLibrary.BreakVector` (`self.Dest_Vec`)))
  (bind (_dest_vec_x_2 _dest_vec_y_2) (`KismetMathLibrary.BreakVector` (`self.Dest_Vec`)))
  (bind (_orig_vec_x _orig_vec_y) (`KismetMathLibrary.BreakVector` (`self.Orig_Vec`)))
  (bind (_orig_vec_x_2 _orig_vec_y_2 _orig_vec_z) (`KismetMathLibrary.BreakVector` (`self.Orig_Vec`)))
  (set `self.Orig_Rot` (`self.K2_GetActorRotation`))
  (set `self.Orig_Vec` (`self.K2_GetActorLocation`))
  (bind (_direction _newtrack_0 _newtrack_1) (`Timeline|Timeline` :!via `PlayFromStart`)
    (:`Update`
      (`self.K2_SetActorLocation` (`KismetMathLibrary.MakeVector` _orig_vec_x_2 (`KismetMathLibrary.Lerp` _orig_vec_y _dest_vec_y_2 (.x _newtrack_1)) (`KismetMathLibrary.Lerp` _orig_vec_z _dest_vec_z (.z _newtrack_1))))
      (`self.K2_SetActorRotation` (`KismetMathLibrary.RLerp` (`self.Orig_Rot`) (`self.Dest_Rot`) _newtrack_0)))
    (:`Finished`
      (if (`self.CanActiveBumper`)
        (set `/Game/GameElements/Blueprints/LevelElement/Bouteille/BP_PusherBouteille.Is_Active` true (`self.Actor_Bumper`)))
      (`self.FloatActivation`))))

(event `self.Box_Interaction.OnComponentBeginOverlap`
  (params (OverlappedComponent :type "PrimitiveComponent Object Reference") (OtherActor :type "Actor Object Reference") (OtherComp :type "PrimitiveComponent Object Reference") (OtherBodyIndex :type Integer) (bFromSweep :type Boolean) (SweepResult :type "HitResult Structure (by ref)"))
  (cast `Character` OtherActor)
  (`/Engine/EditorBlueprintResources/StandardMacros.DoOnce` false
    (:`Completed`
      (`self.SoapFailing`))))

(event `FloatActivation`
  (bind _cylinder (`self.Cylinder`))
  (bind _cylinder_2 (`self.Cylinder`))
  (bind _output_get (set `self.Orig` (`SceneComponent.K2_GetComponentRotation` _cylinder_2)))
  (set `self.Destination` (`KismetMathLibrary.MakeRotator` (+ (.roll _output_get) 10.0) (.pitch _output_get) (.yaw _output_get)))
  (bind _output_get_2 (set `self.Orig_Vec` (`SceneComponent.K2_GetComponentLocation` _cylinder_2)))
  (set `self.Dest_Vec` (`KismetMathLibrary.MakeVector` (.x _output_get_2) (.y _output_get_2) (+ (.z _output_get_2) 10.0)))
  (bind (_direction _newtrack_1) (`Timeline|Timeline_0` :!via `PlayFromStart`)
    (:`Update`
      (`SceneComponent.K2_SetWorldRotation` _cylinder (`KismetMathLibrary.RLerp` (`self.Orig`) (`self.Destination`) (.z _newtrack_1)) false false)
      (`SceneComponent.K2_SetWorldLocation` _cylinder (`KismetMathLibrary.VLerp` (`self.Orig_Vec`) (`self.Dest_Vec`) (.y _newtrack_1)) false false)
      (`SceneComponent.K2_SetWorldLocation` (`self.Cylinder`) (`KismetMathLibrary.VLerp` (`self.Orig_Vec`) (`self.Dest_Vec`) (.y _newtrack_1)) false false))))

(fn `UserConstructionScript`)