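; BP_PusherBouteille is a bottle pusher level element that propels player characters entering its Box while IsActive is set.
; By default it calls LaunchCharacter with LaunchForce, overriding velocity, behind a DoOnce that resets when the player leaves.
; With DebugUseDestinationActor on, a Timeline instead lerps the player from the pusher's location to the DestinationBump actor without sweep.
; A leftover debug PrintString fires on each player overlap.
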(event `self.Box.OnComponentBeginOverlap`
  (params (OverlappedComponent :type "PrimitiveComponent Object Reference") (OtherActor :type "Actor Object Reference") (OtherComp :type "PrimitiveComponent Object Reference") (OtherBodyIndex :type Integer) (bFromSweep :type Boolean) (SweepResult :type "HitResult Structure (by ref)"))
  (if (`self.Is_Active`)
    (bind _asbp_player_character_master (cast `/Game/GameElements/Blueprints/Characters/BP_PlayerCharacter_Master` OtherActor))
    (`KismetSystemLibrary.PrintString` "ZERTYUIOIUYTREZAZERTYUIO")
    (if (`self.Debug_Use_DestinationActor`)
      (set `self.Vec_Dest` (`self.K2_GetActorLocation` (`self.Destination_Bump`)))
      (set `self.Vec_Orig` (`self.K2_GetActorLocation`))
      (bind (_direction _newtrack_0) (`Timeline|Timeline` :!via `PlayFromStart`)
        (:`Update`
          (`self.K2_SetActorLocation` _asbp_player_character_master (`KismetMathLibrary.VLerp` (`self.Vec_Orig`) (`self.Vec_Dest`) _newtrack_0) false false)))
      (else
        (`/Engine/EditorBlueprintResources/StandardMacros.IsValid` _asbp_player_character_master
          (:`Is Valid`
            (`/Engine/EditorBlueprintResources/StandardMacros.DoOnce` false :!label _label
              (:`Completed`
                (`Character.LaunchCharacter` _asbp_player_character_master (`self.LaunchForce`) true true)))))))))

(event `self.Box.OnComponentEndOverlap`
  (params (OverlappedComponent :type "PrimitiveComponent Object Reference") (OtherActor :type "Actor Object Reference") (OtherComp :type "PrimitiveComponent Object Reference") (OtherBodyIndex :type Integer))
  (if (`self.Is_Active`)
    (bind _asbp_player_character_master (cast `/Game/GameElements/Blueprints/Characters/BP_PlayerCharacter_Master` OtherActor))
    (if (not (`self.Debug_Use_DestinationActor`))
      (`/Engine/EditorBlueprintResources/StandardMacros.IsValid` _asbp_player_character_master
        (:`Is Valid`
          (goto _label :!via `Reset`))))))

(fn `UserConstructionScript`)