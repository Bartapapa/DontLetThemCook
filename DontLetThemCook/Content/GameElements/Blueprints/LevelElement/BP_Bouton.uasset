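; BP_Bouton is a level button that toggles on and off when a Character overlaps its box, switching either a referenced hood (Hotte) or grating (Grillage) actor.
; ClickOnBut flips the state, drives the target selected by flags, then calls ActiveButton to swap the material.
; A timeline lerps the mesh down along Z and reverses it unless StayPush is set, which also keeps the button from being pressed again.
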(event `ActiveButton`
  (if (`self.is_On`)
    (`PrimitiveComponent.SetMaterial` (`self.SM_Bouton`) 0 (`self.Material_Appuyer`))
    (bind (_direction _newtrack_0) (`Timeline|Timeline` :!label _label)
      (:`Update`
        (`SceneComponent.K2_SetRelativeLocation` (`self.SM_Bouton`) (`KismetMathLibrary.VLerp` (`self.Relative Location`) (`self.Location_Appuyer`) _newtrack_0) false false))
      (:`Finished`
        (if (not (`self.StayPush`))
          (`self.InverseButton`)
          (set `self.Is_Push` false))))
    (else
      (`PrimitiveComponent.SetMaterial` (`self.SM_Bouton`) 0 (`self.MaterialNone_Appuyer`))
      (goto _label))))

(event `InverseButton`
  (goto _label :!via `Reverse`))

(event `self.ReceiveBeginPlay`
  (bind _output_get (set `self.Relative Location` (`SceneComponent.RelativeLocation` (`self.SM_Bouton`))))
  (set `self.Location_Appuyer` (`KismetMathLibrary.MakeVector` (.x _output_get) (.y _output_get) (- (.z _output_get) 50.0))))

(event `self.Box.OnComponentBeginOverlap`
  (params (OverlappedComponent :type "PrimitiveComponent Object Reference") (OtherActor :type "Actor Object Reference") (OtherComp :type "PrimitiveComponent Object Reference") (OtherBodyIndex :type Integer) (bFromSweep :type Boolean) (SweepResult :type "HitResult Structure (by ref)"))
  ;[1 1 1] Activation Button
  ;;[1 1 1] En attendant la compétence
  (cast `Character` OtherActor)
  (if (not (`self.Is_Push`))
    (`self.ClickOnBut`)))

(event `ClickOnBut`
  (bind _bp_hotte_ref (`self.BP_Hotte_Ref`))
  (bind _actorgrillage (`self.ActorGrillage`))
  ;[1 1 1] Activation Button
  (set `self.Is_Push` true)
  (set `self.is_On` (not (`self.is_On`)))
  ;;[1 1 1] Active Hotte
  (if (`self.Is_PourHotte`)
    (if (`self.is_On`)
      (`/Game/GameElements/Blueprints/LevelElement/BP_Hotte.Active_Hotte` _bp_hotte_ref)
      (else
        (`/Game/GameElements/Blueprints/LevelElement/BP_Hotte.Desactive_Hotte` _bp_hotte_ref)))
    (elif (`self.DebugGrillage`)
      (if (`self.is_On`)
        (`/Game/GameElements/Blueprints/LevelElement/BP_Grillage.ActiveGrillage` _actorgrillage)
        (else
          (`/Game/GameElements/Blueprints/LevelElement/BP_Grillage.DesactiveGrillage` _actorgrillage)))
      (else
        (`KismetSystemLibrary.PrintString` "Is NOT FOR HOTTE"))))
  (`self.ActiveButton`))

(event `self.Box.OnComponentEndOverlap`
  (params (OverlappedComponent :type "PrimitiveComponent Object Reference") (OtherActor :type "Actor Object Reference") (OtherComp :type "PrimitiveComponent Object Reference") (OtherBodyIndex :type Integer))
  ;[1 1 1] Activation Button
  (cast `Character` OtherActor)
  (if (not (`self.StayPush`))
    (set `self.Is_Push` false)))

(fn `UserConstructionScript`)