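; Interactive switch that flips between two sides when a Character overlaps its box, alternately activating a left or right gazinière (stove) when set up for one.
; Each press toggles IsLeft, activates one stove and deactivates the other, then plays or reverses a Timeline rotating the button mesh 90 degrees in yaw.
; IsPush blocks re-triggering until overlap ends or the Timeline finishes, unless StayPush keeps it locked after one press.
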(event `ActiveButton`
  (if (`self.is_Left`)
    (bind (_direction _newtrack_0) (`Timeline|Timeline` :!label _label)
      (:`Update`
        (`SceneComponent.K2_SetRelativeRotation` (`self.SM_Bouton`) (`KismetMathLibrary.RLerp` (`self.Relative Location`) (`self.Location_Appuyer`) _newtrack_0) false false))
      (:`Finished`
        (if (not (`self.StayPush`))
          (set `self.Is_Push` false))))
    (else
      (goto _label :!via `Reverse`))))

(event `self.ReceiveBeginPlay`
  (bind _output_get (set `self.Relative Location` (`SceneComponent.RelativeRotation` (`self.SM_Bouton`))))
  (set `self.Location_Appuyer` (`KismetMathLibrary.MakeRotator` (.roll _output_get) (.pitch _output_get) (- (.yaw _output_get) 90.0))))

(event `self.Box.OnComponentBeginOverlap`
  (params (OverlappedComponent :type "PrimitiveComponent Object Reference") (OtherActor :type "Actor Object Reference") (OtherComp :type "PrimitiveComponent Object Reference") (OtherBodyIndex :type Integer) (bFromSweep :type Boolean) (SweepResult :type "HitResult Structure (by ref)"))
  ;[1 1 1] Activation Button
  ;;[1 1 1] En attendant la compétence
  (cast `Character` OtherActor)
  (if (not (`self.Is_Push`))
    (`self.ClickOnBut`)))

(event `ClickOnBut`
  ;[1 1 1] Activation Button
  (set `self.Is_Push` true)
  (set `self.is_Left` (not (`self.is_Left`)))
  ;;[1 1 1] Active Gaziniere
  (if (`self.Is_ForGaziniere`)
    (if (`self.is_Left`)
      (`/Game/GameElements/Blueprints/LevelElement/BP_Gaziniere.ActiveGaziniere` (`self.Gaziniere_Left`))
      (`/Game/GameElements/Blueprints/LevelElement/BP_Gaziniere.DesactiveGaziniere` (`self.Gaziniere_Right`))
      (else
        (`/Game/GameElements/Blueprints/LevelElement/BP_Gaziniere.DesactiveGaziniere` (`self.Gaziniere_Left`))
        (`/Game/GameElements/Blueprints/LevelElement/BP_Gaziniere.ActiveGaziniere` (`self.Gaziniere_Right`))))
    (else
      (`KismetSystemLibrary.PrintString` "Is NOT FOR HOTTE")))
  (`self.ActiveButton`))

(event `self.Box.OnComponentEndOverlap`
  (params (OverlappedComponent :type "PrimitiveComponent Object Reference") (OtherActor :type "Actor Object Reference") (OtherComp :type "PrimitiveComponent Object Reference") (OtherBodyIndex :type Integer))
  ;[1 1 1] Activation Button
  (cast `Character` OtherActor)
  (if (not (`self.StayPush`))
    (set `self.Is_Push` false)))

(fn `UserConstructionScript`
  (`parent.UserConstructionScript`))