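; BP_Interactible is an interactible level actor, apparently a template for object-specific interactions.
; On BeginPlay it binds handlers to the ACInteractible component's interaction started, ended and prompt toggle events.
; Starting an interaction runs InteractionEvent, a placeholder that prints a message, waits briefly, then calls EndInteract.
; Prompt requests show or hide InteractionPrompt with a debug print, while the ended handler is empty.
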(event `self.ReceiveBeginPlay`
  (bind _ac_interactible (`self.AC_Interactible`))
  (add `/Game/GameElements/Blueprints/Levels/AC_Interactible.OnInteractionStarted` _ac_interactible (`|CreateDelegate` :!event `On Interaction Started`))
  (add `/Game/GameElements/Blueprints/Levels/AC_Interactible.OnInteractionEnded` _ac_interactible (`|CreateDelegate` :!event `On Interaction Ended`))
  (add `/Game/GameElements/Blueprints/Levels/AC_Interactible.OnTogglePromptRequest` _ac_interactible (`|CreateDelegate` :!event `On Toggle Prompt Request`)))

(event `InteractionEvent`
  (`KismetSystemLibrary.PrintString` (`KismetStringLibrary.Concat_StrStr` (`KismetSystemLibrary.GetDisplayName` self) " was interacted with!"))
  ;[1 0.2963 0] Change to object-specific event on interact. Remember to use "End Interact" at the end of the interaction code.
  (`KismetSystemLibrary.Delay` 1.0)
  (`/Game/GameElements/Blueprints/Levels/AC_Interactible.EndInteract` (`self.AC_Interactible`)))

(event `self.ReceiveActorBeginOverlap`
  (params (OtherActor :type "Actor Object Reference")))

(event `self.ReceiveActorEndOverlap`
  (params (OtherActor :type "Actor Object Reference")))

(fn `On Interaction Ended`
  (params (Interactible :type "/Game/GameElements/Blueprints/Levels/AC_Interactible Object Reference") (Interactor :type "/Game/GameElements/Blueprints/Characters/AC_Interactor Object Reference")))

(fn `On Interaction Started`
  (params (Interactible :type "/Game/GameElements/Blueprints/Levels/AC_Interactible Object Reference") (Interactor :type "/Game/GameElements/Blueprints/Characters/AC_Interactor Object Reference"))
  (`self.InteractionEvent`))

(fn `On Toggle Prompt Request`
  (params (`Show?` :type Boolean))
  (`SceneComponent.SetVisibility` (`self.InteractionPrompt`) `Show?` true)
  (`KismetSystemLibrary.PrintString` "APPARAIT" true true (struct :`R` 1.0 :`B` 0.78409 :`A` 1.0)))

(fn `UserConstructionScript`)