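; BP_Pot is a level element pot that can be filled with liquid.
; Fill plays a timeline that lerps FillCurrent from zero to FillMax and applies it as the Z scale of the Liquid component.
; When the timeline finishes, the pot is flagged as filled and ignores further Fill and StopFill calls.
; StopFill halts the timeline while filling is incomplete, leaving the liquid at its current level.
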(event `Fill`
  (if (not (`self.isFilled`))
    (bind (_direction _alpha) (`Timeline|Timeline` :!label _label)
      (:`Update`
        (bind _output_get (set `self.FillCurrent` (`KismetMathLibrary.Lerp` 0.0 (`self.FillMax`) _alpha)))
        (`SceneComponent.SetWorldScale3D` (`self.Liquid`) (`KismetMathLibrary.MakeVector` 1.0 1.0 _output_get)))
      (:`Finished`
        (set `self.isFilled` true)))))

(event `StopFill`
  (if (not (`self.isFilled`))
    (goto _label :!via `Stop`)))

(fn `UserConstructionScript`)