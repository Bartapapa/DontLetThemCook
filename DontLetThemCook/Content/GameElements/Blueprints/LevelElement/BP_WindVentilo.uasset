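; BP_WindVentilo is a wind fan level element that can be switched on or off with its Niagara effect and moves player characters entering its box.
; A looping timer repeatedly launches Chapuccino with LaunchForce and Poichon with zero velocity until overlap ends.
; Chapuccino's special is requested to toggle its cloud state on entry and exit.
; A debug mode instead lerps the player to DestinationBump with a timeline.
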(event `self.ReceiveBeginPlay`
  (if (`self.is_Active`)
    (`self.Active_Wind`)
    (else
      (`self.Desactive_Wind`))))

(event `Active_Wind`
  (set `self.is_Active` true)
  (`ActorComponent.Activate` (`self.Niagara`) false))

(event `Desactive_Wind`
  (set `self.is_Active` false)
  (`ActorComponent.Deactivate` (`self.Niagara`)))

(event `self.Box.OnComponentBeginOverlap`
  (params (OverlappedComponent :type "PrimitiveComponent Object Reference") (OtherActor :type "Actor Object Reference") (OtherComp :type "PrimitiveComponent Object Reference") (OtherBodyIndex :type Integer) (bFromSweep :type Boolean) (SweepResult :type "HitResult Structure (by ref)"))
  (bind _player_ref (`self.Player_Ref`))
  (if (`self.Is_Active`)
    ;[1 0 0] REGARDER ETAT PERSONNAGE
    (bind _asbp_player_character_master (cast `/Game/GameElements/Blueprints/Characters/BP_PlayerCharacter_Master` OtherActor))
    (set `self.Player_Ref` _asbp_player_character_master)
    (`self.TriggerWind`)
    (switch `/Game/GameElements/Blueprints/Characters/E_CharacterID` (`/Game/GameElements/Blueprints/Characters/BP_PlayerCharacter_Master.CharacterID` _player_ref)
      (:`NewEnumerator2`
        (bind _asbp_character_chappucino (cast `/Game/GameElements/Blueprints/Characters/CharacterChildren/BP_Character_Chappucino` _player_ref))
        (if (not (`/Game/GameElements/Blueprints/Characters/CharacterChildren/BP_Character_Chappucino.IsCloud?` _asbp_character_chappucino))
          (`/Game/GameElements/Blueprints/Characters/BP_PlayerCharacter_Master.SpecialRequest` _asbp_character_chappucino 1.0)
          (`/Game/GameElements/Blueprints/Characters/BP_PlayerCharacter_Master.SpecialRequestComplete` _asbp_character_chappucino)
          (`KismetSystemLibrary.PrintString` "ENTER" true true (struct :`R` 1.0 :`B` 0.047369 :`A` 1.0)))))))

(event `self.Box.OnComponentEndOverlap`
  (params (OverlappedComponent :type "PrimitiveComponent Object Reference") (OtherActor :type "Actor Object Reference") (OtherComp :type "PrimitiveComponent Object Reference") (OtherBodyIndex :type Integer))
  (bind _player_ref (`self.Player_Ref`))
  (if (`self.Is_Active`)
    (cast `/Game/GameElements/Blueprints/Characters/BP_PlayerCharacter_Master` OtherActor)
    (if (not (`self.Debug_Use_DestinationActor`))
      (`KismetSystemLibrary.K2_ClearAndInvalidateTimerHandle` (`self.TimerVar`))
      (switch `/Game/GameElements/Blueprints/Characters/E_CharacterID` (`/Game/GameElements/Blueprints/Characters/BP_PlayerCharacter_Master.CharacterID` _player_ref)
        (:`NewEnumerator2`
          (bind _asbp_character_chappucino (cast `/Game/GameElements/Blueprints/Characters/CharacterChildren/BP_Character_Chappucino` _player_ref))
          (if (`/Game/GameElements/Blueprints/Characters/CharacterChildren/BP_Character_Chappucino.IsCloud?` _asbp_character_chappucino)
            (`/Game/GameElements/Blueprints/Characters/BP_PlayerCharacter_Master.SpecialRequest` _asbp_character_chappucino 1.0)
            (`/Game/GameElements/Blueprints/Characters/BP_PlayerCharacter_Master.SpecialRequestComplete` _asbp_character_chappucino)
            (`KismetSystemLibrary.PrintString` "LEAVE" true true (struct :`G` 1.0 :`B` 0.069329 :`A` 1.0))))))))

(event `TriggerWind`
  (if (`self.Debug_Use_DestinationActor`)
    (set `self.Vec_Dest` (`self.K2_GetActorLocation` (`self.Destination_Bump`)))
    (set `self.Vec_Orig` (`self.K2_GetActorLocation`))
    (`Character.LaunchCharacter` (`self.Player_Ref`) (0.0 0.0 50.0) true true)
    (bind (_direction _newtrack_0) (`Timeline|Timeline` :!via `PlayFromStart`)
      (:`Update`
        (`self.K2_SetActorLocation` (`self.Player_Ref`) (`KismetMathLibrary.VLerp` (`self.Vec_Orig`) (`self.Vec_Dest`) _newtrack_0) false false)))
    (else
      (bind _returnvalue (`KismetSystemLibrary.K2_SetTimerDelegate` (delegate `PushTheChar`) 0.1 true))
      (set `self.TimerVar` _returnvalue))))

(event `PushTheChar`
  (switch `/Game/GameElements/Blueprints/Characters/E_CharacterID` (`/Game/GameElements/Blueprints/Characters/BP_PlayerCharacter_Master.CharacterID` (`self.Player_Ref`))
    (:`NewEnumerator1`
      (`Character.LaunchCharacter` (`self.Player_Ref`) (0.0 0.0 0.0) true true))
    (:`NewEnumerator2`
      (`Character.LaunchCharacter` (`self.Player_Ref`) (`self.LaunchForce`) true true))))

(fn `UserConstructionScript`)