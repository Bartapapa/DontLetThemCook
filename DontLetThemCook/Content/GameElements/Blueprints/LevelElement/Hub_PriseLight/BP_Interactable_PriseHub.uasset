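; Interactable hub plug (PriseHub) that performs a one-time plug-in movement when the player interacts with it.
; BeginPlay caches the DestinationActor's location, or prints a warning if none is set.
; InteractionEvent fires BranchementMovement once, where a timeline lerps rotation to DestRot and moves Y and Z on separate curve channels, keeping X fixed.
; When the timeline finishes, it ends the interaction through ACInteractible.
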(event `self.ReceiveBeginPlay`
  (bind _destinationactor (`self.DestinationActor`))
  (`parent.ReceiveBeginPlay`)
  (`/Engine/EditorBlueprintResources/StandardMacros.IsValid` _destinationactor
    (:`Is Valid`
      (set `self.Dest_Vec` (`self.K2_GetActorLocation` _destinationactor)))
    (:`Is Not Valid`
      (`KismetSystemLibrary.PrintString` "NOT SET DESTINATION SOAP"))))

(event `BranchementMovement`
  (bind (_dest_vec_x _dest_vec_y _dest_vec_z) (`KismetMathLibrary.BreakVector` (`self.Dest_Vec`)))
  (bind (_dest_vec_x_2 _dest_vec_y_2) (`KismetMathLibrary.BreakVector` (`self.Dest_Vec`)))
  (bind (_orig_vec_x _orig_vec_y) (`KismetMathLibrary.BreakVector` (`self.Orig_Vec`)))
  (bind (_orig_vec_x_2 _orig_vec_y_2 _orig_vec_z) (`KismetMathLibrary.BreakVector` (`self.Orig_Vec`)))
  (set `self.Orig_Rot` (`self.K2_GetActorRotation`))
  (set `self.Orig_Vec` (`self.K2_GetActorLocation`))
  (bind (_direction _newtrack_0 _newtrack_1) (`Timeline|Timeline` :!via `PlayFromStart`)
    (:`Update`
      (`self.K2_SetActorLocation` (`KismetMathLibrary.MakeVector` _orig_vec_x_2 (`KismetMathLibrary.Lerp` _orig_vec_y _dest_vec_y_2 (.x _newtrack_1)) (`KismetMathLibrary.Lerp` _orig_vec_z _dest_vec_z (.z _newtrack_1))))
      (`self.K2_SetActorRotation` (`KismetMathLibrary.RLerp` (`self.Orig_Rot`) (`self.Dest_Rot`) _newtrack_0)))
    (:`Finished`
      (`/Game/GameElements/Blueprints/Levels/AC_Interactible.EndInteract` (`self.AC_Interactible`)))))

(event `self.InteractionEvent`
  (`/Engine/EditorBlueprintResources/StandardMacros.DoOnce` false
    (:`Completed`
      (`self.BranchementMovement`))))

(fn `UserConstructionScript`
  (`parent.UserConstructionScript`))