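; BP_LightHub is a switchable point light level element for the hub that starts switched off when play begins.
; ActiveLight and DesactiveLight toggle IsActive, switching off by zeroing the attenuation radius and on by applying the configured radius, softness, indirect lighting, shadow and falloff settings.
; The construction script applies the same settings when IsActive is set and Inplay is false, previewing the lit state before play.
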(event `self.ReceiveBeginPlay`
  (set `self.Inplay` true)
  (`self.DesactiveLight`))

(event `ActiveLight`
  (bind _pointlight (`self.PointLight`))
  (set `self.is_Active` true)
  (`LocalLightComponent.SetAttenuationRadius` _pointlight (`self.AttenuationRadius`))
  (`PointLightComponent.SetSoftSourceRadius` _pointlight (`self.SoftSourceRadius`))
  (`LightComponent.SetIndirectLightingIntensity` _pointlight (`self.IndirectLightingIntensity`))
  (`LightComponentBase.SetCastShadows` _pointlight (`self.CastShadow`))
  (`PointLightComponent.SetLightFalloffExponent` _pointlight (`self.LightFalloffExponent`)))

(event `DesactiveLight`
  (set `self.is_Active` false)
  (`LocalLightComponent.SetAttenuationRadius` (`self.PointLight`) 0.0))

(fn `UserConstructionScript`
  (bind _pointlight (`self.PointLight`))
  (if (`self.Inplay`)
    _
    (elif (`self.is_Active`)
      (`LocalLightComponent.SetAttenuationRadius` _pointlight (`self.AttenuationRadius`))
      (`PointLightComponent.SetSoftSourceRadius` _pointlight (`self.SoftSourceRadius`))
      (`LightComponent.SetIndirectLightingIntensity` _pointlight (`self.IndirectLightingIntensity`))
      (`LightComponentBase.SetCastShadows` _pointlight (`self.CastShadow`))
      (`PointLightComponent.SetLightFalloffExponent` _pointlight (`self.LightFalloffExponent`)))))